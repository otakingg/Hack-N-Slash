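; Character component that toggles an aura effect while an activation key is held, or through Start and Stop events.
; BeginPlay pre-spawns optional ground and mesh-bound Niagara systems and creates a dynamic overlay material.
; Start and Stop toggle the Niagara systems, play optional sounds and camera shakes, and run a looping timer that fades the overlay.
; Zero-delay polling loops manage loop audio, sound resets and optional input freezing during fade-in.
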(event `self.ReceiveBeginPlay`
  (bind _skeletal_mesh (`self.Skeletal Mesh`))
  ;[0.4499 1 0.8278] Set References
  (bind _ascharacter (cast `Character` (`self.GetOwner`)))
  (set `self.As Character` _ascharacter)
  (set `self.Skeletal Mesh` (`Character.Mesh` _ascharacter))
  (set `self.IsActivated?` false)
  (set `self.TimerSpeed` (/ (`self.TimerSpeed`) 1000.0))
  ;[0.5651 0.5434 1] Set Niagara References
  (if (`self.Use Niagara "Ground"?`)
    (bind _returnvalue (`NiagaraFunctionLibrary.SpawnSystemAttached` (`self.Niagara "Ground"`) (`self.Skeletal Mesh`) "None" (0.0 0.0 0.0) (struct) "KeepRelativeOffset" false false "ManualRelease"))
    (set `self.Niagara Ground Start Spwaned` _returnvalue))
  (if (`self.Use Niagara "Ovrly"?`)
    (bind _returnvalue_2 (`NiagaraFunctionLibrary.SpawnSystemAttached` (`self.Niagara "Niagara "Ovrly""`) _skeletal_mesh "None" (0.0 0.0 0.0) (struct) "KeepRelativeOffset" false false "ManualRelease"))
    (set `self.Niagara"Ovrly"Spawned` _returnvalue_2)
    (`NiagaraFunctionLibrary.OverrideSystemUserVariableSkeletalMeshComponent` (`self.Niagara"Ovrly"Spawned`) "Skeletal Mesh" _skeletal_mesh))
  ;[0.9463 1 0.8527] Set Overlay Dynamic Material Instance
  (bind _returnvalue_3 (`KismetMaterialLibrary.CreateDynamicMaterialInstance` (`self.Overlay Material`)))
  (set `self.OverlayMaterialRef` _returnvalue_3))

(event `Play CameraShake-StartEffect`
  ;[0.1329 0 1] Camera Shake
  (if (`self.UseCameraShake?`)
    (`PlayerCameraManager.StartCameraShake` :`self` (`GameplayStatics.GetPlayerCameraManager` 0) :`ShakeClass` (`self.1-Camera Shake Start Effect`) :`Scale` (`self.1-Scale`))))

(event `Play CameraShake-StopEffect`
  ;[0.1329 0 1] Camera Shake
  (if (`self.UseCameraShake?`)
    (`PlayerCameraManager.StartCameraShake` :`self` (`GameplayStatics.GetPlayerCameraManager` 0) :`ShakeClass` (`self.2-Camera Shake Stop Effect`) :`Scale` (`self.2-Scale`))))

(event `Start Aura Effect`
  (bind _returnvalue (`GameplayStatics.GetPlayerController` 0))
  (bind _as_character (`self.As Character`))
  ;[1 0 0] Custom Events Start/Stop effect
  (if (`self.Use Niagara "Ground"?`) :!label _label
    (`self.Activate` (`self.Niagara Ground Start Spwaned`) false))
  (`self.Play CameraShake-StartEffect`)
  ;[0.3969 1 0.3036] System Activation
  (if (`self.Use Niagara "Ovrly"?`)
    (`self.Activate` (`self.Niagara"Ovrly"Spawned`) false))
  (`|ExecutionSequence`
    (:`then_0`
      (set `self.IsActivated?` true)
      (if (`self.Use Start Sound?`)
        (`|ExecutionSequence`
          (:`then_0`
            _)
          (:`then_1`
            ;[0 0.2882 1] Start & End Sounds
            (`/Engine/EditorBlueprintResources/StandardMacros.DoOnce` false :!label _label_2
              (:`Completed`
                (`GameplayStatics.SpawnSoundAtLocation` (`self.Start Sound`) (`SceneComponent.K2_GetComponentLocation` (`Character.Mesh` (`self.As Character`))) (struct) (`self.Start Volume`) 1.0 0.0 (`self.Attenuation Settings`) null)
                (if (`self.IsActivated?`) :!label _label_3
                  (`KismetSystemLibrary.Delay` 0.0)
                  (goto _label_3)
                  (else
                    (goto _label_2 :!via `Reset`))))))))
      (bind _returnvalue_2 (`KismetSystemLibrary.K2_SetTimerDelegate` (delegate `Time`) 0.001 true :!label _label_4))
      (set `self.Timer Handle` _returnvalue_2))
    (:`then_1`
      ;[1 0.4301 0] Freeze Controls
      (if (`self.Start Aura Freeze Input?`)
        (set `self.Freezeinputs` true)
        (`Actor.DisableInput` _as_character _returnvalue)
        (if (`self.Freezeinputs`) :!label _label_5
          (`KismetSystemLibrary.Delay` 0.0)
          (goto _label_5)
          (else
            (`KismetSystemLibrary.Delay` (`self.FreezeInputAdditionalDelay`))
            (`Actor.EnableInput` _as_character _returnvalue)))))))

(event `EnhancedInput|/Game/PlayerAuraEffect/Demo/ThirdPerson/Input/Actions/IA_Action`
  (params (ActionValue :type Boolean) (ElapsedSeconds :type "Float (double-precision)") (TriggeredSeconds :type "Float (double-precision)") (InputAction :type "InputAction Object Reference" :default "/Game/PlayerAuraEffect/Demo/ThirdPerson/Input/Actions/IA_Action.IA_Action"))
  ;[1 0.4328 0.8512 1 36] Key Selector:
  ; If you want to set another system based (for example) on a Player Input controller, delete "Set Key" content, and connect your own control logic ("Player Input Action" for example).
  ;;[0 1 0.9134] Enhanced Input example:
)

(event `Key|LeftShift`
  (params (Key :type "Key Structure"))
  ;[1 0.4328 0.8512 1 36] Key Selector:
  ; If you want to set another system based (for example) on a Player Input controller, delete "Set Key" content, and connect your own control logic ("Player Input Action" for example).
  ;;[0 1 0.9134] Other method:
  ;; A simple Key
)

(event `Key|AnyKey`
  (params (Key :type "Key Structure"))
  (bind (_activation_key_actionname _activation_key_bshift _activation_key_bctrl _activation_key_balt _activation_key_bcmd _activation_key_key) (break `InputActionKeyMapping` (`self.Activation Key`)))
  (bind _isactivated_ (`self.IsActivated?`))
  ;[1 0.4328 0.8512 1 36] Key Selector:
  ; If you want to set another system based (for example) on a Player Input controller, delete "Set Key" content, and connect your own control logic ("Player Input Action" for example).
  ;;[0 1 0.9134] Set Key Parameter:
  (:`Pressed`
    (if _isactivated_
      _
      (elif (== Key _activation_key_key)
        (goto _label))))
  (:`Released`
    (if _isactivated_
      (if (== Key _activation_key_key)
        (if (`self.Use Niagara "Ground"?`) :!label _label_6
          (`self.Deactivate` (`self.Niagara Ground Start Spwaned`)))
        (`self.Play CameraShake-StopEffect`)
        ;[0.3969 1 0.3036] System Activation
        (if (`self.Use Niagara "Ovrly"?`)
          (`self.Deactivate` (`self.Niagara"Ovrly"Spawned`)))
        (set `self.IsActivated?` false)
        (if (`self.Use End Sound?`)
          (`|ExecutionSequence`
            (:`then_0`
              (goto _label_4))
            (:`then_1`
              ;[0 0.2882 1] Start & End Sounds
              (`/Engine/EditorBlueprintResources/StandardMacros.DoOnce` false :!label _label_7
                (:`Completed`
                  (`GameplayStatics.SpawnSoundAtLocation` (`self.End Sound`) (`SceneComponent.K2_GetComponentLocation` (`Character.Mesh` (`self.As Character`))) (struct) (`self.End Volume`) 1.0 0.0 (`self.Attenuation Settings`) null)
                  (if (`self.IsActivated?`) :!label _label_8
                    (goto _label_7 :!via `Reset`)
                    (else
                      (`KismetSystemLibrary.Delay` 0.0)
                      (goto _label_8)))))))
          (else
            (goto _label_4)))))))

(event `Time`
  (bind _loopsoundref (`self.LoopSoundRef`))
  (if (`self.IsActivated?`)
    ;[1 0.4745 0.8193] Activate Overlay
    (`MeshComponent.SetOverlayMaterial` (`self.Skeletal Mesh`) (`self.OverlayMaterialRef`))
    (`|ExecutionSequence`
      (:`then_0`
        ;[0 0.2882 1] Loop Sound
        (`/Engine/EditorBlueprintResources/StandardMacros.DoOnce` false :!label _label_9
          (:`Completed`
            (if (`self.Use LoopSound?`)
              (bind _returnvalue (`GameplayStatics.SpawnSoundAtLocation` (`self.Loop Sound`) (`SceneComponent.K2_GetComponentLocation` (`Character.Mesh` (`self.As Character`))) (struct) (`self.Loop Volume`) 1.0 0.0 (`self.Attenuation Settings`) null))
              (set `self.LoopSoundRef` _returnvalue)
              (`AudioComponent.FadeIn` _loopsoundref (`self.Loop Fade in Duration`) 1.0 0.0 "Linear")
              (if (`self.IsActivated?`) :!label _label_10
                (`KismetSystemLibrary.Delay` 0.0)
                (goto _label_10)
                (else
                  (`AudioComponent.FadeOut` _loopsoundref (`self.Alpha`) 0.0 "Linear")
                  (goto _label_9 :!via `Reset`)))))))
      (:`then_1`
        (if (>= (`self.Alpha`) 1.0)
          (set `self.Alpha` 1.0)
          (set `self.Freezeinputs` false)
          (`KismetSystemLibrary.K2_ClearAndInvalidateTimerHandle` (`self.Timer Handle`))
          (else
            (set `self.Freezeinputs` true)
            (set `self.Alpha` (+ (`self.Alpha`) (`self.TimerSpeed`)))
            (`MaterialInstanceDynamic.SetScalarParameterValue` (`self.OverlayMaterialRef`) "Fade" (`self.Alpha`))))))
    (else
      ;[1 0.4745 0.8193] Deactivate Overlay
      (if (<= (`self.Alpha`) 0.0)
        (set `self.Alpha` 0.0)
        (`KismetSystemLibrary.K2_ClearAndInvalidateTimerHandle` (`self.Timer Handle`))
        (`MeshComponent.SetOverlayMaterial` (`self.Skeletal Mesh`) null)
        (else
          (set `self.Alpha` (- (`self.Alpha`) (`self.TimerSpeed`)))))
      (`MaterialInstanceDynamic.SetScalarParameterValue` (`self.OverlayMaterialRef`) "Fade" (`self.Alpha`)))))

(event `Stop Aura Effect`
  ;[1 0 0] Custom Events Start/Stop effect
  (goto _label_6))