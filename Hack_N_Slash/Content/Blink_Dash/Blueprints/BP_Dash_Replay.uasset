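; BP_Dash_Replay is a Blueprint that repeatedly replays a dash, likely as a looping demonstration of the Blink Dash effect.
; On BeginPlay it stores the capsule's world location and starts a looping timer with a period of TimeReplay.
; Each timeout calls DashStart on BPDash, then waits half that period before moving the capsule back to the stored location without sweep.
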(event `self.ReceiveBeginPlay`
  (bind _capsulecomponent (`self.CapsuleComponent`))
  (bind _returnvalue (`SceneComponent.K2_GetComponentLocation` _capsulecomponent))
  (set `self.Location` _returnvalue)
  (`SceneComponent.K2_SetWorldLocation` _capsulecomponent _returnvalue false false)
  (`KismetSystemLibrary.K2_SetTimer` null "Timeout" (`self.Time_Replay`) true))

(event `Timeout`
  (bind _time_replay (`self.Time_Replay`))
  (`/Game/Blink_Dash/Blueprints/BP_Dash.Dash Start` (`self.BP_Dash`))
  (`KismetSystemLibrary.Delay` (- _time_replay (/ _time_replay 2.0)))
  (`SceneComponent.K2_SetWorldLocation` (`self.CapsuleComponent`) (`self.Location`) false false))

(fn `UserConstructionScript`)