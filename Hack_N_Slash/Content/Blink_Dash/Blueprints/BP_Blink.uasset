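; BP_Blink gives its owning Character a short-range blink that moves it forward along its capsule's facing.
; BlinkStart stores a destination BlinkDistance ahead, spawns the Niagara effect at the capsule and starts a one-shot BlinkDelay timer.
; When the timer fires, BlinkEnd moves the capsule to the stored point with a sweep, so blocking geometry can cut the move short, then spawns the effect again on arrival.
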(event `self.ReceiveBeginPlay`
  (`|ExecutionSequence`
    (:`then_0`
      (bind _ascharacter (cast `Character` (`self.GetOwner`)))
      (set `self.As Character` _ascharacter))))

(event `Blink Start`
  (bind _capsulecomponent (`Character.CapsuleComponent` (`self.As Character`)))
  (bind _returnvalue (`SceneComponent.K2_GetComponentLocation` _capsulecomponent))
  (set `self.Blink Location` (+ _returnvalue (* (`SceneComponent.GetForwardVector` _capsulecomponent) (`self.Blink_Distance`))))
  (`NiagaraFunctionLibrary.SpawnSystemAtLocation` (`self.Blink_VFX`) _returnvalue (`SceneComponent.K2_GetComponentRotation` _capsulecomponent))
  (`KismetSystemLibrary.K2_SetTimerDelegate` (delegate `Blink End`) (`self.Blink Delay`)))

(event `Blink End`
  (`SceneComponent.K2_SetWorldLocation` (`Character.CapsuleComponent` (`self.As Character`)) (`self.Blink Location`) true false)
  (`NiagaraFunctionLibrary.SpawnSystemAtLocation` (`self.Blink_VFX`) (`SceneComponent.K2_GetComponentLocation` (`Character.CapsuleComponent` (`self.As Character`)))))