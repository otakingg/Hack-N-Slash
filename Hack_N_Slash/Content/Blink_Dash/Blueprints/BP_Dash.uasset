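; BP_Dash is a component that gives its owning Character a short forward dash with a Niagara effect.
; It caches the owner on BeginPlay, and DashStart saves the current velocity, then overrides it with the forward vector scaled by Distance.
; After a brief delay it deactivates the capsule-attached effect and restores the saved velocity.
; A CanDash flag blocks re-triggering until the dash ends.
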(event `self.ReceiveBeginPlay`
  (`|ExecutionSequence`
    (:`then_0`
      (bind _ascharacter (cast `Character` (`self.GetOwner`)))
      (set `self.As Character` _ascharacter))))

(event `Dash Start`
  (bind _capsulecomponent (`Character.CapsuleComponent` (`self.As Character`)))
  (if (`self.CanDash`)
    (set `self.CanDash` false)
    (set `self.OldVelocity` (`MovementComponent.Velocity` (`Character.CharacterMovement` (`self.As Character`))))
    (bind _returnvalue (`NiagaraFunctionLibrary.SpawnSystemAttached` (`self.Dash`) _capsulecomponent "None" (`SceneComponent.K2_GetComponentLocation` _capsulecomponent) (`KismetMathLibrary.MakeRotFromY` (`SceneComponent.GetForwardVector` _capsulecomponent)) "KeepWorldPosition"))
    (set `self.Dash_Spawn` _returnvalue)
    (set `MovementComponent.Velocity` (* (`Actor.GetActorForwardVector` (`self.As Character`)) (`self.Distance`)) (`Character.CharacterMovement` (`self.As Character`)))
    (`KismetSystemLibrary.Delay` 0.2)
    (`self.Deactivate` (`self.Dash_Spawn`))
    (set `MovementComponent.Velocity` (`self.OldVelocity`) (`Character.CharacterMovement` (`self.As Character`)))
    (set `self.CanDash` true)))