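; Elite enemy Delta, a dual-katana character built on a parent enemy class.
; Shortly after BeginPlay it spawns a katana for each hand and snaps it to that weapon socket on the mesh.
; Dash events play a sound and activate a VFX component, with an optional timer to delay its shutdown.
; The patrol route getter is an empty stub, and a brain-pause call is left unconnected.
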(event `self.ReceiveBeginPlay`
  (`parent.ReceiveBeginPlay`)
  (`KismetSystemLibrary.Delay` 0.5)
  (`|ExecutionSequence`
    (:`then_0`
      (bind _returnvalue (`|SpawnActorFromClass` "/Game/Hack-N-Slash/Enemies/Elites/Delta/Weapons/BP_Weapon_Delta_Katana.BP_Weapon_Delta_Katana_C" (`SceneComponent.GetSocketTransform` (`self.Mesh`) "WeaponBaseR_Socket" "RTS_World") "Undefined" "MultiplyWithRoot" self self))
      (`self.K2_AttachToComponent` _returnvalue (`self.Mesh`) "WeaponBaseR_Socket" "SnapToTarget" "SnapToTarget" "SnapToTarget" true))
    (:`then_1`
      (bind _returnvalue_2 (`|SpawnActorFromClass` "/Game/Hack-N-Slash/Enemies/Elites/Delta/Weapons/BP_Weapon_Delta_Katana.BP_Weapon_Delta_Katana_C" (`SceneComponent.GetSocketTransform` (`self.Mesh`) "WeaponBaseL_Socket" "RTS_World") "Undefined" "MultiplyWithRoot" self self))
      (`self.K2_AttachToComponent` _returnvalue_2 (`self.Mesh`) "WeaponBaseL_Socket" "SnapToTarget" "SnapToTarget" "SnapToTarget" true))))

(event `Start Dash FX`
  (`GameplayStatics.PlaySoundAtLocation` "/Game/Hack-N-Slash/Enemies/Elites/Delta/SFX/SQ_SFX_Delta_Dash.SQ_SFX_Delta_Dash" (`self.K2_GetActorLocation`) (struct) 1.0 1.0 0.0 null null null null)
  (bind _dash_vfx (`self.Dash VFX`)
    (:`then`
      (`ActorComponent.Activate` _dash_vfx true))
    (:`else`)))

(event `Stop Dash FX`
  (params (Delay :type "Float (double-precision)"))
  (bind _dash_vfx (`self.Dash VFX`)
    (:`then`
      (if (`ActorComponent.IsActive` _dash_vfx)
        (if (> Delay 0.0)
          (`KismetSystemLibrary.K2_SetTimerDelegate` (`|CreateDelegate` :!event `End Dash VFX`) Delay)
          (else
            (`ActorComponent.Deactivate` (`self.Dash VFX`))))))
    (:`else`)))

(event `End Dash VFX`
  (bind _dash_vfx (`self.Dash VFX`)
    (:`then`
      (`ActorComponent.Deactivate` _dash_vfx))
    (:`else`)))

(fn `GetPatrolRoute`
  (returns (`Patrol Route` :type "/Game/Hack-N-Slash/Utility/BP_PatrolRoute Object Reference"))
  (return null))

(fn `UserConstructionScript`
  (`parent.UserConstructionScript`))