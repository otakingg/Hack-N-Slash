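; Reactive enemy sequence for the elite Delta that air-dodges melee hits from an attacker it is facing.
; CanExecute also checks poise and sphere-traces behind Delta, away from the attacker, requiring a clear path with ground below the landing point.
; Execute turns Delta toward the attacker and plays the dodge montage with damage immunity, nullified reactions and pawn collision ignored.
; Completion or abort restores those states, with active-state checks guarding the steps.
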(event `self.Initialize`
  (params (InBrain :type "EnemyBrainComponent Object Reference"))
  ;[1 1 0 0.5] Initialize
  (`parent.Initialize` InBrain)
  (`/Engine/EditorBlueprintResources/StandardMacros.IsValid` InBrain
    (:`Is Valid`
      (bind _asbp_enemy_delta (cast `/Game/Hack-N-Slash/Enemies/Elites/Delta/BP_Enemy_Delta` (`ActorComponent.GetOwner` InBrain)))
      (set `self.Delta` _asbp_enemy_delta))))

(event `self.Execute`
  (params (HitData :type "AtkHitData Structure (by ref)"))
  ;[0 1 1 0.5] Execute
  (`self.Is Active?`
    (:`Yes`
      (`self.Ensure References`
        (:`Valid`
          (`EnemyController.ClearFocusHNS` (`EnemyBrainComponent.GetEnemyController` (`self.brain`)))
          (`self.Is Active?`
            (:`Yes`
              (`self.StartDodgeConditions`)
              (`self.Is Active?`
                (:`Yes`
                  (`Actor.K2_SetActorRotation` (`self.Delta`) (`KismetMathLibrary.MakeRotator` 0.0 0.0 (.yaw (`KismetMathLibrary.FindLookAtRotation` (`Actor.K2_GetActorLocation` (`self.Delta`)) (`Actor.K2_GetActorLocation` (`.damager` (break `AtkHitData` HitData)))))) false)
                  (`self.Is Active?`
                    (:`Yes`
                      (`|PlayMontage` (`Character.Mesh` (`self.Delta`)) (`self.Montage`)
                        (:`OnCompleted`
                          (`self.EndDodgeConditions`)
                          (`self.Finish`))
                        (:`OnInterrupted`
                          (`self.Is Active?`
                            (:`Yes`
                              (`self.Abort`))))))))))))
        (:`Invalid`
          (`self.Abort`))))))

(event `self.Abort`
  ;[1 0 0 0.5] Abort
  (`self.EndDodgeConditions`)
  (`parent.Abort`))

(fn `CanExecute`
  (params (HitData :type "AtkHitData Structure (by ref)"))
  (returns (ReturnValue :type Boolean))
  (bind (_attacker _damager _attackmotion _attackreaction _attacktype) (break `AtkHitData` (`local.HitData`)))
  (bind _returnvalue (`Actor.K2_GetActorLocation` (`self.Delta`)))
  (if (and (`parent.CanExecute` (`local.HitData`)) (`KismetSystemLibrary.IsValid` (`EnemyBrainComponent.GetEnemyController` (`self.brain`))) (`KismetSystemLibrary.IsValid` (`.TargetActor` (break `EnemyBlackboard` (`EnemyBrainComponent.blackboard` (`self.brain`))))) (`KismetSystemLibrary.IsValid` _damager) (`self.IsFacingActor` _damager) (`BlueprintGameplayTagLibrary.MatchesTag` _attacktype (struct :`TagName` "Attack.Type.Melee")) (`KismetSystemLibrary.IsValid` (`self.Delta`)) (`KismetSystemLibrary.IsValid` (`EnemyBase.combatResComp` (`self.Delta`))) (> (`CombatResolutionComponent.GetPoiseCalc` (`EnemyBase.combatResComp` (`self.Delta`))) -1) (`KismetSystemLibrary.IsValid` (`self.Montage`)))
    (bind (_outhit _returnvalue_2) (`KismetSystemLibrary.SphereTraceSingle` (`self.Delta`) (`Actor.K2_GetActorLocation` (`self.Delta`)) (+ _returnvalue (* (`KismetMathLibrary.GetForwardVector` (`KismetMathLibrary.MakeRotator` 0.0 0.0 (.yaw (`KismetMathLibrary.FindLookAtRotation` _returnvalue (`Actor.K2_GetActorLocation` (`.damager` (break `AtkHitData` (`local.HitData`)))))))) -1.0 300.0)) 25.0 "TraceTypeQuery1" false (`|MakeArray` (`self.Delta`) :!type "Actor Object Reference") (select `bool` (`self.bDebug`) :`true` "ForDuration" :!type "EDrawDebugTrace Enum")))
    (if _returnvalue_2
      (return false)
      (else
        (bind (_bblockinghit _binitialoverlap _time _distance _location _impactpoint _normal _impactnormal _physmat _hitactor _hitcomponent _hitbonename _bonename _hititem _elementindex _faceindex _tracestart _traceend) (`GameplayStatics.BreakHitResult` _outhit))
        (bind (_outhit_2 _returnvalue_3) (`KismetSystemLibrary.SphereTraceSingle` (`self.Delta`) _traceend (+ _traceend (0.0 0.0 -2000.0)) 25.0 "TraceTypeQuery1" false (`|MakeArray` (`self.Delta`) :!type "Actor Object Reference") (select `bool` (`self.bDebug`) :`true` "ForDuration" :!type "EDrawDebugTrace Enum")))
        (if _returnvalue_3
          (return true)
          (else
            (return false)))))
    (else
      (return false))))

(fn `EndDodgeConditions`
  (bind _delta (`self.Delta`)
    (:`then`
      (bind _statscomp (`EnemyBase.statsComp` _delta)
        (:`then`
          (`StatsComponent.SetDmgImmunity` _statscomp false))
        (:`else`
          _))
      (`self.Is Active?`
        (:`Yes`
          (bind _combatrescomp (`EnemyBase.combatResComp` (`self.Delta`))
            (:`then`
              (`CombatResolutionComponent.SetReactionOverride` _combatrescomp "None"))
            (:`else`
              _))
          (`self.Is Active?`
            (:`Yes`
              (bind _capsulecomponent (`Character.CapsuleComponent` (`self.Delta`))
                (:`then`
                  (`PrimitiveComponent.SetCollisionResponseToChannel` _capsulecomponent "ECC_Pawn" "ECR_Block"))
                (:`else`)))))))
    (:`else`)))

(fn `StartDodgeConditions`
  (bind _delta (`self.Delta`)
    (:`then`
      (`StatsComponent.SetDmgImmunity` (`EnemyBase.statsComp` _delta) true)
      (`self.Is Active?`
        (:`Yes`
          (`CombatResolutionComponent.SetReactionOverride` (`EnemyBase.combatResComp` (`self.Delta`)) "Nullify")
          (`self.Is Active?`
            (:`Yes`
              (`PrimitiveComponent.SetCollisionResponseToChannel` (`Character.CapsuleComponent` (`self.Delta`)) "ECC_Pawn" "ECR_Ignore"))))))
    (:`else`)))