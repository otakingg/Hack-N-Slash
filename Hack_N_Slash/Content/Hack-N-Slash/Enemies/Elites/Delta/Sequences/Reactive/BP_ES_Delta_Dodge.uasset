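; Reactive enemy sequence that makes the elite Delta dodge an incoming melee attack via a montage.
; It runs only if Delta faces the damager, passes a poise check, and sphere traces find a clear path away from the attacker with ground at its end.
; Execution nullifies hit reactions, grants damage immunity and turns Delta toward the damager before playing the montage.
; Finish and Abort clear both the reaction override and the immunity.
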(event `self.Initialize`
  (params (InBrain :type "EnemyBrainComponent Object Reference"))
  (`parent.Initialize` InBrain)
  (`/Engine/EditorBlueprintResources/StandardMacros.IsValid` InBrain
    (:`Is Valid`
      (bind _asbp_enemy_delta (cast `/Game/Hack-N-Slash/Enemies/Elites/Delta/BP_Enemy_Delta` (`ActorComponent.GetOwner` InBrain)))
      (bind _output_get (set `self.Delta` _asbp_enemy_delta))
      (set `self.Combat Res` (`Actor.GetComponentByClass` _output_get "/Script/Hack_N_Slash.CombatResolutionComponent"))
      (set `self.Stats` (`Actor.GetComponentByClass` (`self.Delta`) "/Script/Hack_N_Slash.StatsComponent")))))

(event `self.Execute`
  (params (HitData :type "AtkHitData Structure (by ref)"))
  (`self.Is Active?`
    (:`Yes`
      (`self.Ensure References`
        (:`Valid`
          (`CombatResolutionComponent.SetReactionOverride` (`self.Combat Res`) "Nullify")
          (`self.Is Active?`
            (:`Yes`
              (bind _stats (`self.Stats`)
                (:`then`
                  (`StatsComponent.SetDmgImmunity` _stats true)
                  (`self.Is Active?`
                    (:`Yes`
                      _)))
                (:`else`
                  _))
              (`Actor.K2_SetActorRotation` (`self.Delta`) (`KismetMathLibrary.FindLookAtRotation` (`Actor.K2_GetActorLocation` (`self.Delta`)) (`Actor.K2_GetActorLocation` (`.damager` (break `AtkHitData` HitData)))) false)
              (`self.Is Active?`
                (:`Yes`
                  (bind _mesh (`Character.Mesh` (`self.Delta`))
                    (:`then`
                      (`|PlayMontage` _mesh (`self.Montage`)
                        (:`OnCompleted`
                          (`self.Finish`))
                        (:`OnInterrupted`
                          (`self.Is Active?`
                            (:`Yes`
                              (`self.Abort`))))))
                    (:`else`)))))))))))

(event `self.Abort`
  (bind _combat_res (`self.Combat Res`)
    (:`then`
      (`CombatResolutionComponent.SetReactionOverride` _combat_res "None"))
    (:`else`
      _))
  (bind _stats (`self.Stats`)
    (:`then`
      (`StatsComponent.SetDmgImmunity` _stats false))
    (:`else`
      _))
  (`parent.Abort`))

(event `self.Finish`
  (bind _combat_res (`self.Combat Res`)
    (:`then`
      (`CombatResolutionComponent.SetReactionOverride` _combat_res "None"))
    (:`else`
      _))
  (bind _stats (`self.Stats`)
    (:`then`
      (`StatsComponent.SetDmgImmunity` _stats false))
    (:`else`
      _))
  (`parent.Finish`))

(fn `CanExecute`
  (params (HitData :type "AtkHitData Structure (by ref)"))
  (returns (ReturnValue :type Boolean))
  (bind (_attacker _damager _attackmotion _attackreaction _attacktype) (break `AtkHitData` (`local.HitData`)))
  (bind _returnvalue (`Actor.K2_GetActorLocation` (`self.Delta`)))
  (if (and (`parent.CanExecute` (`local.HitData`)) (`KismetSystemLibrary.IsValid` (`.TargetActor` (break `EnemyBlackboard` (`EnemyBrainComponent.blackboard` (`self.brain`))))) (`KismetSystemLibrary.IsValid` _damager) (`self.IsFacingActor` _damager) (`BlueprintGameplayTagLibrary.MatchesTag` _attacktype (struct :`TagName` "Attack.Type.Melee")) (`KismetSystemLibrary.IsValid` (`self.Delta`)) (`KismetSystemLibrary.IsValid` (`self.Combat Res`)) (> (`CombatResolutionComponent.GetPoiseCalc` (`self.Combat Res`)) -1) (`KismetSystemLibrary.IsValid` (`self.Montage`)))
    (bind (_outhit _returnvalue_2) (`KismetSystemLibrary.SphereTraceSingle` (`self.Delta`) (`Actor.K2_GetActorLocation` (`self.Delta`)) (+ _returnvalue (* (`KismetMathLibrary.GetForwardVector` (`KismetMathLibrary.FindLookAtRotation` _returnvalue (`Actor.K2_GetActorLocation` (`.damager` (break `AtkHitData` (`local.HitData`)))))) -1.0 300.0)) 25.0 "TraceTypeQuery1" false (`|MakeArray` (`self.Delta`) :!type "Actor Object Reference") (select `bool` (`self.bDebug`) :`true` "ForDuration" :!type "EDrawDebugTrace Enum")))
    (if _returnvalue_2
      (return false)
      (else
        (bind (_bblockinghit _binitialoverlap _time _distance _location _impactpoint _normal _impactnormal _physmat _hitactor _hitcomponent _hitbonename _bonename _hititem _elementindex _faceindex _tracestart _traceend) (`GameplayStatics.BreakHitResult` _outhit))
        (bind (_outhit_2 _returnvalue_3) (`KismetSystemLibrary.SphereTraceSingle` (`self.Delta`) _traceend (+ _traceend (0.0 0.0 -100.0)) 25.0 "TraceTypeQuery1" false (`|MakeArray` (`self.Delta`) :!type "Actor Object Reference") (select `bool` (`self.bDebug`) :`true` "ForDuration" :!type "EDrawDebugTrace Enum")))
        (if _returnvalue_3
          (return true)
          (else
            (return false)))))
    (else
      (return false))))