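; Reactive enemy sequence for the elite Delta that dodges an incoming melee hit, then follows up with an attack.
; It runs only when Delta faces the attacker, passes a poise check, and sphere traces find clear space and ground behind it.
; The dodge turns Delta toward the attacker and plays a montage with damage immunity and nullified hit reactions.
; Completion or abort restores both, and completion advances to the attack.
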(event `self.Initialize`
  (params (InBrain :type "EnemyBrainComponent Object Reference"))
  ;[1 1 0 0.5] Initialize
  (`parent.Initialize` InBrain)
  (`/Engine/EditorBlueprintResources/StandardMacros.IsValid` InBrain
    (:`Is Valid`
      (bind _asbp_enemy_delta (cast `/Game/Hack-N-Slash/Enemies/Elites/Delta/BP_Enemy_Delta` (`ActorComponent.GetOwner` InBrain)))
      (set `self.Delta` _asbp_enemy_delta))))

(event `self.Execute`
  (params (HitData :type "AtkHitData Structure (by ref)"))
  (bind _returnvalue (`EnemyBrainComponent.GetEnemyController` (`self.brain`)))
  ;[0 1 1 0.5] Execute
  (`self.Is Active?`
    (:`Yes`
      (`self.Ensure References`
        (:`Valid`
          (`/Engine/EditorBlueprintResources/StandardMacros.IsValid` _returnvalue
            (:`Is Valid`
              (`EnemyController.ClearFocusHNS` _returnvalue)
              (`self.Is Active?`
                (:`Yes`
                  _)))
            (:`Is Not Valid`
              _))
          (`CombatResolutionComponent.SetReactionOverride` (`EnemyBase.combatResComp` (`self.Delta`)) "Nullify")
          (`self.Is Active?`
            (:`Yes`
              (bind _statscomp (`EnemyBase.statsComp` (`self.Delta`))
                (:`then`
                  (`StatsComponent.SetDmgImmunity` _statscomp true)
                  (`self.Is Active?`
                    (:`Yes`
                      _)))
                (:`else`
                  _))
              (`Actor.K2_SetActorRotation` (`self.Delta`) (`KismetMathLibrary.FindLookAtRotation` (`Actor.K2_GetActorLocation` (`self.Delta`)) (`Actor.K2_GetActorLocation` (`.damager` (break `AtkHitData` HitData)))) false)
              (`self.Is Active?`
                (:`Yes`
                  (`|PlayMontage` (`Character.Mesh` (`self.Delta`)) (`self.Montage`)
                    (:`OnCompleted`
                      (`self.Is Active?`
                        (:`Yes`
                          (`self.EndImmunity`)
                          (`self.AdvanceSequence`))))
                    (:`OnInterrupted`
                      (`self.Is Active?`
                        (:`Yes`
                          (`self.Abort`))))))))))
        (:`Invalid`
          (`self.Abort`))))))

(event `self.AdvanceSequence`
  (`self.Is Active?`
    (:`Yes`
      (`self.Ensure References`
        (:`Valid`
          (bind _output_get (set `self.sequenceIndex` (+ (`self.sequenceIndex`) 1)))
          (switch `int` _output_get
            (:`Default`
              (`self.Finish` :!label _label))
            (:`2`
              (bind _returnvalue (`EnemyCombatComponent.Attack` (`EnemyBase.combatComp` (`self.Delta`)) (`self.Atk`)))
              (if (not _returnvalue)
                (`self.Abort`)))
            (:`3`
              (goto _label))))
        (:`Invalid`
          (`self.Abort`))))))

(event `self.Abort`
  ;[1 0 0 0.5] Abort
  (`self.EndImmunity`)
  (`parent.Abort`))

(fn `CanExecute`
  (params (HitData :type "AtkHitData Structure (by ref)"))
  (returns (ReturnValue :type Boolean))
  (bind (_attacker _damager _attackmotion _attackreaction _attacktype) (break `AtkHitData` (`local.HitData`)))
  (bind _returnvalue (`Actor.K2_GetActorLocation` (`self.Delta`)))
  (if (and (`parent.CanExecute` (`local.HitData`)) (`KismetSystemLibrary.IsValid` (`.TargetActor` (break `EnemyBlackboard` (`EnemyBrainComponent.blackboard` (`self.brain`))))) (`KismetSystemLibrary.IsValid` _damager) (`self.IsFacingActor` _damager) (`BlueprintGameplayTagLibrary.MatchesTag` _attacktype (struct :`TagName` "Attack.Type.Melee")) (`KismetSystemLibrary.IsValid` (`self.Delta`)) (`KismetSystemLibrary.IsValid` (`EnemyBase.combatResComp` (`self.Delta`))) (> (`CombatResolutionComponent.GetPoiseCalc` (`EnemyBase.combatResComp` (`self.Delta`))) -1) (`KismetSystemLibrary.IsValid` (`self.Montage`)) (`KismetSystemLibrary.IsValid` (`EnemyBase.combatComp` (`self.Delta`))))
    (bind (_outhit _returnvalue_2) (`KismetSystemLibrary.SphereTraceSingle` (`self.Delta`) (`Actor.K2_GetActorLocation` (`self.Delta`)) (+ _returnvalue (* (`KismetMathLibrary.GetForwardVector` (`KismetMathLibrary.FindLookAtRotation` _returnvalue (`Actor.K2_GetActorLocation` (`.damager` (break `AtkHitData` (`local.HitData`)))))) -1.0 300.0)) 25.0 "TraceTypeQuery1" false (`|MakeArray` (`self.Delta`) :!type "Actor Object Reference") (select `bool` (`self.bDebug`) :`true` "ForDuration" :!type "EDrawDebugTrace Enum")))
    (if _returnvalue_2
      (return false)
      (else
        (bind (_bblockinghit _binitialoverlap _time _distance _location _impactpoint _normal _impactnormal _physmat _hitactor _hitcomponent _hitbonename _bonename _hititem _elementindex _faceindex _tracestart _traceend) (`GameplayStatics.BreakHitResult` _outhit))
        (bind (_outhit_2 _returnvalue_3) (`KismetSystemLibrary.SphereTraceSingle` (`self.Delta`) _traceend (+ _traceend (0.0 0.0 -100.0)) 25.0 "TraceTypeQuery1" false (`|MakeArray` (`self.Delta`) :!type "Actor Object Reference") (select `bool` (`self.bDebug`) :`true` "ForDuration" :!type "EDrawDebugTrace Enum")))
        (if _returnvalue_3
          (return true)
          (else
            (return false)))))
    (else
      (return false))))

(fn `EndImmunity`
  (bind _delta (`self.Delta`)
    (:`then`
      (bind _statscomp (`EnemyBase.statsComp` _delta)
        (:`then`
          (`StatsComponent.SetDmgImmunity` _statscomp false))
        (:`else`
          _))
      (bind _combatrescomp (`EnemyBase.combatResComp` (`self.Delta`))
        (:`then`
          (`CombatResolutionComponent.SetReactionOverride` _combatrescomp "None"))
        (:`else`)))
    (:`else`)))