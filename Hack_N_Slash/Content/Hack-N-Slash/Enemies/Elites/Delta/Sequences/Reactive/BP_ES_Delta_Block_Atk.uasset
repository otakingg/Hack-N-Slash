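; Reactive enemy sequence for the Delta elite that blocks frontal, non-armor-breaking melee hits and retaliates with a revenge attack.
; Final hits build RevengeMeter, selecting block reaction montages; a full meter or any launcher triggers a counter on the attacker.
; AdvanceSequence then fires RevengeAtk if countering, otherwise finishes.
; A jump notify applies async root-motion force toward the target's velocity-predicted location, aborting if interrupted.
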(event `self.Initialize`
  (params (InBrain :type "EnemyBrainComponent Object Reference"))
  ;[1 1 0 0.5] Initialize
  (`parent.Initialize` InBrain)
  (`/Engine/EditorBlueprintResources/StandardMacros.IsValid` InBrain
    (:`Is Valid`
      (bind _asbp_enemy_delta (cast `/Game/Hack-N-Slash/Enemies/Elites/Delta/BP_Enemy_Delta` (`ActorComponent.GetOwner` InBrain)))
      (set `self.Delta` _asbp_enemy_delta))))

(event `self.Execute`
  (params (HitData :type "AtkHitData Structure (by ref)"))
  ;[0 1 1 0.5] Execute
  (`self.Is Active?`
    (:`Yes`
      (`self.Ensure References`
        (:`Valid`
          (bind _returnvalue (`EnemyCombatComponent.Block` (`EnemyBase.combatComp` (`self.Delta`))))
          (if (not _returnvalue)
            (`self.Finish`)
            (else
              (set `/Game/Hack-N-Slash/Enemies/Elites/Delta/BP_Enemy_Delta.Block Reaction` (`|GetArrayItem` (`self.BlockHitMonts`) (`self.revengeMeter`)) (`self.Delta`)))))
        (:`Invalid`
          (`self.Finish`))))))

(event `self.HandleReceiveHitPost`
  (params (HitData :type "AtkHitData Structure (by ref)"))
  (`self.Handle Block` HitData))

(event `self.AdvanceSequence`
  (`self.Is Active?`
    (:`Yes`
      (`self.Ensure References`
        (:`Valid`
          (`self.EarlyCounter?`
            (:`then`
              (bind _returnvalue (`EnemyCombatComponent.Attack` (`EnemyBase.combatComp` (`self.Delta`)) (`self.RevengeAtk`)))
              (if _returnvalue
                (set `self.revengeMeter` 0)
                (else
                  (`self.Abort`))))
            (:`else`
              (if (< (`self.revengeMeter`) (`self.maxRevenge`))
                (`self.Finish`)
                (else
                  (bind _returnvalue_2 (`EnemyCombatComponent.Attack` (`EnemyBase.combatComp` (`self.Delta`)) (`self.RevengeAtk`)))
                  (if _returnvalue_2
                    (set `self.revengeMeter` 0)
                    (else
                      (`self.Abort`))))))))
        (:`Invalid`
          (`self.Abort`))))))

(event `self.HandleAnimNotify`
  (params (NotifyTag :type "GameplayTag Structure (by ref)"))
  (bind _returnvalue (`Actor.K2_GetActorLocation` (`self.Delta`)))
  (bind _lococomp (`EnemyBase.locoComp` (`self.Delta`)))
  (bind _warploc (`LocomotionComponent.CalcWarpLocRot` (`EnemyBase.locoComp` (`self.Delta`)) (`self.Calc Target Location`) 100.0 0.0 true true false false))
  (`parent.HandleAnimNotify` NotifyTag)
  (`self.Is Active?`
    (:`Yes`
      (`self.Ensure References`
        (:`Valid`
          (`|SwitchGameplayTag` NotifyTag
            (:`NotifyEvent.EnemyBrain.Jump`
              (bind (_asynctaskproxy _rootmovement) (`AsyncRootMovement.AsyncRootMovement_JumpForce` (`self.Delta`) (`Character.CharacterMovement` (`self.Delta`)) (- _warploc _returnvalue) (`KismetMathLibrary.Vector_Distance` _warploc _returnvalue) 300.0 0.4 "SetVelocity")
                (:`then`
                  (`LocomotionComponent.AddRootMotionSource_BP` _lococomp _asynctaskproxy false))
                (:`OnComplete`
                  (`LocomotionComponent.OnRootMotionComplete` _lococomp _rootmovement))
                (:`OnInterrupted`
                  (`self.Is Active?`
                    (:`Yes`
                      (`self.Abort`))))))))
        (:`Invalid`
          (`self.Abort`))))))

(event `self.Abort`
  ;[1 0 0 0.5] Abort
  (set `self.EarlyCounter?` false)
  (set `self.revengeMeter` 0)
  (bind _delta (`self.Delta`)
    (:`then`
      (set `/Game/Hack-N-Slash/Enemies/Elites/Delta/BP_Enemy_Delta.Block Reaction` null _delta))
    (:`else`
      _))
  (`parent.Abort`))

(event `self.Finish`
  ;[0 1 0 0.5] Finish
  (set `self.EarlyCounter?` false)
  (set `self.revengeMeter` 0)
  (bind _delta (`self.Delta`)
    (:`then`
      (set `/Game/Hack-N-Slash/Enemies/Elites/Delta/BP_Enemy_Delta.Block Reaction` null _delta))
    (:`else`
      _))
  (`parent.Finish`))

(fn `Calc Target Location`
  (returns (`Jump Loc` :type "Vector Structure"))
  (locals (`Move Comp` :type "MovementComponent Object Reference") (`Target Velocity` :type "Vector Structure" :default (0.0 0.0 0.0)))
  (bind _returnvalue (`Actor.GetComponentByClass` (`.TargetActor` (break `EnemyBlackboard` (`EnemyBrainComponent.blackboard` (`self.brain`)))) "/Script/Engine.MovementComponent"))
  (`/Engine/EditorBlueprintResources/StandardMacros.IsValid` _returnvalue
    (:`Is Valid`
      (set `local.Target Velocity` (`MovementComponent.Velocity` _returnvalue)))
    (:`Is Not Valid`
      (set `local.Target Velocity` (0.0 0.0 0.0))))
  (return (+ (`Actor.K2_GetActorLocation` (`.TargetActor` (break `EnemyBlackboard` (`EnemyBrainComponent.blackboard` (`self.brain`))))) (* (`local.Target Velocity`) 0.25))))

(fn `CanExecute`
  (params (HitData :type "AtkHitData Structure (by ref)"))
  (returns (ReturnValue :type Boolean))
  (bind (_attacker _damager _attackmotion _attackreaction _attacktype _barmorbreaker) (break `AtkHitData` (`local.HitData`)))
  (return (and (`parent.CanExecute` HitData) (`KismetSystemLibrary.IsValid` (`.TargetActor` (break `EnemyBlackboard` (`EnemyBrainComponent.blackboard` (`self.brain`))))) (`KismetSystemLibrary.IsValid` (`self.Delta`)) (`KismetSystemLibrary.IsValid` (`EnemyBase.combatComp` (`self.Delta`))) (`KismetSystemLibrary.IsValid` (`EnemyBase.combatResComp` (`self.Delta`))) (> (`CombatResolutionComponent.GetPoiseCalc` (`EnemyBase.combatResComp` (`self.Delta`))) -1) (`self.IsFacingActor` _damager) (`BlueprintGameplayTagLibrary.MatchesTag` _attacktype (struct :`TagName` "Attack.Type.Melee")) (not _barmorbreaker) (`KismetSystemLibrary.IsValid` (`EnemyBase.locoComp` (`self.Delta`))))))

(fn `Handle Block`
  (params (AtkHitData :type "AtkHitData Structure (by ref)"))
  (`self.Is Active?`
    (:`Yes`
      (`self.Ensure References`
        (:`Valid`
          (if (`BlueprintGameplayTagLibrary.MatchesTag` (`.attackType` (break `AtkHitData` (`local.AtkHitData`))) (struct :`TagName` "Attack.Type.Melee"))
            (if (`BlueprintGameplayTagLibrary.MatchesTag` (`.attackMotion` (break `AtkHitData` (`local.AtkHitData`))) (struct :`TagName` "Attack.Motion.Launch"))
              (`BPFL_Combat.Counter` (`self.Delta`) (`.damager` (break `AtkHitData` (`local.AtkHitData`))) "Blocked")
              (set `self.EarlyCounter?` true)
              (`Character.PlayAnimMontage` (`self.Delta`) (`|GetArrayItem` (`self.BlockHitMonts`) (- (`KismetArrayLibrary.Array_Length` (`self.BlockHitMonts`)) 1)) 1.0 "None")
              (elif (or (`.bIsFinalHit` (break `AtkHitData` (`local.AtkHitData`))) (== (`self.revengeMeter`) (- (`self.maxRevenge`) 1)))
                (bind _output_get (set `self.revengeMeter` (`KismetMathLibrary.Clamp` (+ (`self.revengeMeter`) 1) 0 (`self.maxRevenge`))))
                (`self.Is Active?`
                  (:`Yes`
                    (if (>= _output_get (`self.maxRevenge`))
                      (set `/Game/Hack-N-Slash/Enemies/Elites/Delta/BP_Enemy_Delta.Block Reaction` null (`self.Delta`))
                      (`BPFL_Combat.Counter` (`self.Delta`) (`.damager` (break `AtkHitData` (`local.AtkHitData`))) "Blocked")
                      (else
                        (set `/Game/Hack-N-Slash/Enemies/Elites/Delta/BP_Enemy_Delta.Block Reaction` (`|GetArrayItem` (`self.BlockHitMonts`) (`self.revengeMeter`)) (`self.Delta`))))))))))
        (:`Invalid`
          (`self.Abort`))))))