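; Proactive AI sequence that makes the Delta elite enemy strafe at a slow walk while focused on its target.
; An EQS query favors farther or nearer spots depending on current target distance, picking randomly among the best-scoring results.
; EQS and move-completion callbacks advance a step index: move to the spot, then finish after a short random delay.
; It allows reactive interruption and aborts on invalid references or empty query results.
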(event `self.Initialize`
  (params (InBrain :type "EnemyBrainComponent Object Reference"))
  ;[1 1 0 0.5] Initialize
  (`parent.Initialize` InBrain)
  (bind _brain (`self.brain`)
    (:`then`
      (bind _asbp_enemy_delta (cast `/Game/Hack-N-Slash/Enemies/Elites/Delta/BP_Enemy_Delta` (`ActorComponent.GetOwner` _brain)))
      (set `self.Delta` _asbp_enemy_delta))
    (:`else`)))

(event `self.Execute`
  (bind _brain (`self.brain`))
  ;[0 1 1 0.5] Execute
  (`self.Is Active?`
    (:`Yes`
      (`self.EnsureReferences`
        (:`Is Valid`
          (set `self.bInterruptibleReactive` true)
          (`self.Is Active?`
            (:`Yes`
              (`EnemyController.SetFocusHNS` (`EnemyBrainComponent.GetEnemyController` _brain) (`.TargetActor` (break `EnemyBlackboard` (`EnemyBrainComponent.blackboard` _brain))))
              (`self.Is Active?`
                (:`Yes`
                  (`self.SetWalkSpeedAndAcceleration` 150.0 4000.0)
                  (`self.Is Active?`
                    (:`Yes`
                      (`self.FindStrafeLoc`))))))))
        (:`Is Not Valid`
          (`self.Abort`))))))

(event `self.HandleEQSFinished`
  (params (Result :type "EnvQueryResult Structure (by ref)"))
  (`self.AdvanceSequence`))

(event `self.HandleMoveCompleted`
  (params (RequestID :type Integer) (Result :type "EPathFollowingResult Enum" :default "Success"))
  (`self.AdvanceSequence`))

(event `self.AdvanceSequence`
  (`self.Is Active?`
    (:`Yes`
      (`self.EnsureReferences`
        (:`Is Valid`
          (bind _output_get (set `self.sequenceIndex` (+ (`self.sequenceIndex`) 1)))
          (switch `int` _output_get
            (:`Default`
              (`self.Finish`))
            (:`2`
              (bind _locsempty_ (`self.Move`))
              (if _locsempty_
                (`self.Abort`)))
            (:`3`
              (bind _returnvalue (`KismetSystemLibrary.K2_SetTimer` null "Finish" (`KismetMathLibrary.RandomFloatInRange` 0.0 2.0)))
              (set `self.TH_Finish` _returnvalue))))
        (:`Is Not Valid`
          (`self.Abort`))))))

(fn `CanExecute`
  (returns (ReturnValue :type Boolean))
  (bind _delta (`self.Delta`))
  (return (and (`parent.CanExecute`) (`KismetSystemLibrary.IsValid` (`EnemyBrainComponent.GetEnemyController` (`self.brain`))) (`KismetSystemLibrary.IsValid` _delta) (`KismetSystemLibrary.IsValid` (`Character.CharacterMovement` _delta)) (`KismetSystemLibrary.IsValid` (`EnemyBase.locoComp` _delta)) (`KismetSystemLibrary.IsValid` (`.TargetActor` (break `EnemyBlackboard` (`EnemyBrainComponent.blackboard` (`self.brain`))))))))

(fn `FindStrafeLoc`
  (locals (Params :type "Map of Name to Float (single-precision)"))
  (bind _params (`local.Params`))
  (bind _params_2 (`local.Params`))
  (if (<= (`KismetMathLibrary.Vector_Distance` (`Actor.K2_GetActorLocation` (`self.Delta`)) (`Actor.K2_GetActorLocation` (`.TargetActor` (break `EnemyBlackboard` (`EnemyBrainComponent.blackboard` (`self.brain`)))))) 500.0)
    (`BlueprintMapLibrary.Map_Add` _params_2 "Distance.Lesser.ScoringFactor")
    (`BlueprintMapLibrary.Map_Add` _params_2 "Distance.Greater.ScoringFactor" 1.0)
    (else
      (`BlueprintMapLibrary.Map_Add` _params "Distance.Lesser.ScoringFactor" 1.0)
      (`BlueprintMapLibrary.Map_Add` _params "Distance.Greater.ScoringFactor")))
  (`EnemyController.RunEQSQueryHNS` (`EnemyBrainComponent.GetEnemyController` (`self.brain`)) "/Game/Hack-N-Slash/EnvQuery/QuerySelf/EQ_Self_Strafe.EQ_Self_Strafe" (`local.Params`) "RandomBest5Pct"))

(fn `Move`
  (returns (`LocsEmpty?` :type Boolean))
  (bind (_targetactor _targetdistance _targetheightdifference _lastdamagesource _lastknownlocation _homelocation _lastattacktime _recenthits _eqs_actors _eqs_locs) (break `EnemyBlackboard` (`EnemyBrainComponent.blackboard` (`self.brain`))))
  (bind _returnvalue (`KismetArrayLibrary.Array_IsEmpty` _eqs_locs))
  (if (not _returnvalue)
    (`LocomotionComponent.MoveTo` (`EnemyBase.locoComp` (`self.Delta`)) null (`|GetArrayItem` _eqs_locs) 60.0))
  (return _returnvalue))

(fn `SetWalkSpeedAndAcceleration`
  (params (Speed :type "Float (double-precision)") (Acceleration :type "Float (double-precision)"))
  (bind _charactermovement (`Character.CharacterMovement` (`self.Delta`)))
  (set `CharacterMovementComponent.MaxWalkSpeed` Speed _charactermovement)
  (set `CharacterMovementComponent.MaxAcceleration` (`local.Acceleration`) _charactermovement))