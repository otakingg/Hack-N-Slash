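; Proactive enemy sequence that has the elite enemy Delta perform a back step when its target is close and roughly in front of it.
; On execution it clears the controller's focus, snaps Delta's yaw toward the blackboard target and plays a montage, presumably carrying the movement.
; An active-state check guards each step; montage completion finishes the sequence, while interruption aborts it if still active.
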(event `self.Initialize`
  (params (InBrain :type "EnemyBrainComponent Object Reference"))
  ;[1 1 0 0.5] Initialize
  (`parent.Initialize` InBrain)
  (bind _brain (`self.brain`)
    (:`then`
      (bind _asbp_enemy_delta (cast `/Game/Hack-N-Slash/Enemies/Elites/Delta/BP_Enemy_Delta` (`ActorComponent.GetOwner` _brain)))
      (set `self.Delta` _asbp_enemy_delta))
    (:`else`)))

(event `self.Execute`
  (bind (_returnvalue_roll _returnvalue_pitch _returnvalue_yaw) (`KismetMathLibrary.BreakRotator` (`KismetMathLibrary.FindLookAtRotation` (`Actor.K2_GetActorLocation` (`self.Delta`)) (`Actor.K2_GetActorLocation` (`.TargetActor` (break `EnemyBlackboard` (`EnemyBrainComponent.blackboard` (`self.brain`))))))))
  ;[0 1 1 0.5] Execute
  (`self.Is Active?`
    (:`Yes`
      (`EnemyController.ClearFocusHNS` (`EnemyBrainComponent.GetEnemyController` (`self.brain`)))
      (`self.Is Active?`
        (:`Yes`
          (`Actor.K2_SetActorRotation` (`self.Delta`) (`KismetMathLibrary.MakeRotator` 0.0 0.0 _returnvalue_yaw) false)
          (`self.Is Active?`
            (:`Yes`
              (`|PlayMontage` (`Character.Mesh` (`self.Delta`)) (`self.Montage`)
                (:`OnCompleted`
                  (`self.Finish`))
                (:`OnInterrupted`
                  (`self.Is Active?`
                    (:`Yes`
                      (`self.Abort`))))))))))))

(fn `CanExecute`
  (returns (ReturnValue :type Boolean))
  (bind _delta (`self.Delta`))
  (return (and (`parent.CanExecute`) (`KismetSystemLibrary.IsValid` (`EnemyBrainComponent.GetEnemyController` (`self.brain`))) (`KismetSystemLibrary.IsValid` _delta) (`KismetSystemLibrary.IsValid` (`Character.Mesh` _delta)) (`KismetSystemLibrary.IsValid` (`self.Montage`)) (`self.IsFacingActor` (`.TargetActor` (break `EnemyBlackboard` (`EnemyBrainComponent.blackboard` (`self.brain`))))) (<= (`.TargetDistance` (break `EnemyBlackboard` (`EnemyBrainComponent.blackboard` (`self.brain`)))) 400.0))))