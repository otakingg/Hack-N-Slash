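; Proactive sequence for the Delta elite enemy that closes in on its target when farther away than the desired radius.
; On execute it allows reactive interruption, focuses the target, sets walk speed and acceleration, and runs the approach EQS query.
; It moves to a random returned location, finishing on success and aborting on empty results or failed moves.
; Active-state checks guard each step.
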(event `self.Initialize`
  (params (InBrain :type "EnemyBrainComponent Object Reference"))
  ;[1 1 0 0.5] Initialize
  (`parent.Initialize` InBrain)
  (bind _brain (`self.brain`)
    (:`then`
      (bind _asbp_enemy_delta (cast `/Game/Hack-N-Slash/Enemies/Elites/Delta/BP_Enemy_Delta` (`ActorComponent.GetOwner` _brain)))
      (set `self.Delta` _asbp_enemy_delta))
    (:`else`)))

(event `self.Execute`
  (bind _brain (`self.brain`))
  ;[0 1 1 0.5] Execute
  (`self.Is Active?`
    (:`Yes`
      (set `self.bInterruptibleReactive` true)
      (`self.Is Active?`
        (:`Yes`
          (`EnemyController.SetFocusHNS` (`EnemyBrainComponent.GetEnemyController` _brain) (`.TargetActor` (break `EnemyBlackboard` (`EnemyBrainComponent.blackboard` _brain))))
          (`self.SetWalkSpeedAndAcceleration` 200.0 4000.0)
          (`self.FindApproachLoc`))))))

(event `self.HandleEQSFinished`
  (params (Result :type "EnvQueryResult Structure (by ref)"))
  (bind (_targetactor _targetdistance _targetheightdifference _lastdamagesource _lastknownlocation _homelocation _lastattacktime _recenthits _eqs_actors _eqs_locs) (break `EnemyBlackboard` (`EnemyBrainComponent.blackboard` (`self.brain`))))
  (`self.Is Active?`
    (:`Yes`
      (if (`KismetArrayLibrary.Array_IsEmpty` _eqs_locs)
        (`self.Abort`)
        (else
          (`LocomotionComponent.MoveTo` (`EnemyBase.locoComp` (`self.Delta`)) null (`|GetArrayItem` _eqs_locs (`KismetMathLibrary.RandomIntegerInRange` 0 (- (`KismetArrayLibrary.Array_Length` _eqs_locs) 1))) 50.0))))))

(event `self.HandleMoveCompleted`
  (params (RequestID :type Integer) (Result :type "EPathFollowingResult Enum" :default "Success"))
  (`self.Is Active?`
    (:`Yes`
      (switch `EPathFollowingResult` Result
        (:`Success`
          (`self.Finish`))
        (:`Blocked`
          (`self.Abort` :!label _label))
        (:`OffPath`
          (goto _label))
        (:`Aborted`
          (goto _label))
        (:`Invalid`
          (goto _label))))))

(fn `CanExecute`
  (returns (ReturnValue :type Boolean))
  (bind _delta (`self.Delta`))
  (return (and (`parent.CanExecute`) (`KismetSystemLibrary.IsValid` (`EnemyBrainComponent.GetEnemyController` (`self.brain`))) (`KismetSystemLibrary.IsValid` _delta) (`KismetSystemLibrary.IsValid` (`Character.CharacterMovement` _delta)) (`KismetSystemLibrary.IsValid` (`EnemyBase.locoComp` _delta)) (`KismetSystemLibrary.IsValid` (`.TargetActor` (break `EnemyBlackboard` (`EnemyBrainComponent.blackboard` (`self.brain`))))) (> (`self.GetTargetDistance`) (`self.Desired Radius`)))))

(fn `FindApproachLoc`
  (locals (Params :type "Map of Name to Float (single-precision)"))
  (`self.Is Active?`
    (:`Yes`
      (`EnemyController.RunEQSQueryHNS` (`EnemyBrainComponent.GetEnemyController` (`self.brain`)) "/Game/Hack-N-Slash/EnvQuery/QuerySelf/EQ_Self_Approach.EQ_Self_Approach" (`|MakeMap` "None" :!type "Name" :!valuetype "Float (single-precision)") "AllMatching"))))

(fn `SetWalkSpeedAndAcceleration`
  (params (Speed :type "Float (double-precision)") (Acceleration :type "Float (double-precision)"))
  (bind _charactermovement (`Character.CharacterMovement` (`self.Delta`)))
  (`self.Is Active?`
    (:`Yes`
      (set `CharacterMovementComponent.MaxWalkSpeed` (`local.Speed`) _charactermovement)
      (`self.Is Active?`
        (:`Yes`
          (set `CharacterMovementComponent.MaxAcceleration` (`local.Acceleration`) _charactermovement))))))