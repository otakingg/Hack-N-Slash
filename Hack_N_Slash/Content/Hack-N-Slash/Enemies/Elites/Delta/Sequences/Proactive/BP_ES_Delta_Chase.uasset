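; Proactive AI sequence for the Delta elite enemy that chases the blackboard target when it is farther than a desired radius.
; Execute marks the sequence interruptible by reactives, focuses the controller on the target, raises walk speed and acceleration, and starts a LocoComp move toward it.
; The move result finishes on success or aborts otherwise, and a five-second timer aborts chases that run too long.
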(event `self.Initialize`
  (params (InBrain :type "EnemyBrainComponent Object Reference"))
  ;[1 1 0 0.5] Initialize
  (`parent.Initialize` InBrain)
  (bind _brain (`self.brain`)
    (:`then`
      (bind _asbp_enemy_delta (cast `/Game/Hack-N-Slash/Enemies/Elites/Delta/BP_Enemy_Delta` (`ActorComponent.GetOwner` _brain)))
      (set `self.Delta` _asbp_enemy_delta))
    (:`else`)))

(event `self.Execute`
  (bind _brain (`self.brain`))
  ;[0 1 1 0.5] Execute
  (`self.Is Active?`
    (:`Yes`
      (set `self.bInterruptibleReactive` true)
      (`self.Is Active?`
        (:`Yes`
          (`EnemyController.SetFocusHNS` (`EnemyBrainComponent.GetEnemyController` _brain) (`.TargetActor` (break `EnemyBlackboard` (`EnemyBrainComponent.blackboard` _brain))))
          (`self.Is Active?`
            (:`Yes`
              (`self.SetWalkSpeedAndAcceleration` 650.0 4000.0)
              (`LocomotionComponent.MoveTo` (`EnemyBase.locoComp` (`self.Delta`)) (`.TargetActor` (break `EnemyBlackboard` (`EnemyBrainComponent.blackboard` (`self.brain`)))) (0.0 0.0 0.0) (`self.Desired Radius`))
              (`KismetSystemLibrary.K2_SetTimerDelegate` (delegate `Stop Chasing`) 5.0))))))))

(event `Stop Chasing`
  ;[0 1 1 0.5] Execute
  (`self.Is Active?`
    (:`Yes`
      (`self.Abort`))))

(event `self.HandleMoveCompleted`
  (params (RequestID :type Integer) (Result :type "EPathFollowingResult Enum" :default "Success"))
  (`self.Is Active?`
    (:`Yes`
      (switch `EPathFollowingResult` Result
        (:`Success`
          (`self.Finish`))
        (:`Blocked`
          (`self.Abort` :!label _label))
        (:`OffPath`
          (goto _label))
        (:`Aborted`
          (goto _label))
        (:`Invalid`
          (goto _label))))))

(fn `CanExecute`
  (returns (ReturnValue :type Boolean))
  (bind _delta (`self.Delta`))
  (return (and (`parent.CanExecute`) (`KismetSystemLibrary.IsValid` (`EnemyBrainComponent.GetEnemyController` (`self.brain`))) (`KismetSystemLibrary.IsValid` _delta) (`KismetSystemLibrary.IsValid` (`Character.CharacterMovement` _delta)) (`KismetSystemLibrary.IsValid` (`EnemyBase.locoComp` _delta)) (`KismetSystemLibrary.IsValid` (`.TargetActor` (break `EnemyBlackboard` (`EnemyBrainComponent.blackboard` (`self.brain`))))) (> (`self.GetTargetDistance`) (`self.Desired Radius`)))))

(fn `SetWalkSpeedAndAcceleration`
  (params (Speed :type "Float (double-precision)") (Acceleration :type "Float (double-precision)"))
  (bind _charactermovement (`Character.CharacterMovement` (`self.Delta`)))
  (set `CharacterMovementComponent.MaxWalkSpeed` Speed _charactermovement)
  (set `CharacterMovementComponent.MaxAcceleration` (`local.Acceleration`) _charactermovement))