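; Area-of-effect slash attack actor for the Delta elite enemy, built on a parent AOE class.
; On BeginPlay it builds armor-breaking stagger hit data, spawns a slash effect and the AOE, then triggers it.
; A looping timer repeats the blade whoosh sound.
; Each overlap copies the impact normal, point and location into the hit data and passes it to damage handling.
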(event `self.ReceiveBeginPlay`
  (`parent.ReceiveBeginPlay`)
  (set `self.Hit Data` (make `AtkHitData` (`self.GetInstigator`) self (struct :`TagName` "Attack.Motion.Stationary") "StaggerUpFront2" (struct :`TagName` "Attack.Type.AOE") true false _ 0.05 (`self.Damage`) (`self.Penetration`) (`self.Poise`) "Constant" "MaintainLastRootMotionVelocity" (0.0 0.0 0.0) 0.0 0.1 false (1.0 0.0 0.0) 10.0))
  (`NiagaraFunctionLibrary.SpawnSystemAtLocation` "/Game/NiagaraMagicalSlashes/Fx/Slashes/NS_Cut_Sl_07.NS_Cut_Sl_07" (`self.K2_GetActorLocation`))
  (`self.SpawnAOE`)
  (`GameplayStatics.PlaySoundAtLocation` "/Game/Hack-N-Slash/Audio/SFX/Whooshes/SQ_SFX_Blade_Whoosh_02.SQ_SFX_Blade_Whoosh_02" (`self.K2_GetActorLocation`) (struct) 1.0 1.0 0.0 null null null null)
  (`self.Trigger`)
  (`KismetSystemLibrary.K2_SetTimerDelegate` (delegate `Play Slash Sound`) 0.1 true))

(event `self.OnAOEOverlap`
  (params (Actor :type "Actor Object Reference") (HitResult :type "HitResult Structure (by ref)"))
  (bind (_bblockinghit _binitialoverlap _time _distance _location _impactpoint _normal _impactnormal) (`GameplayStatics.BreakHitResult` HitResult))
  (bind (_hit_data_attacker _hit_data_damager _hit_data_attackmotion _hit_data_attackreaction _hit_data_attacktype _hit_data_barmorbreaker _hit_data_biscounterfollowup _hit_data_elements _hit_data_aggrobuildup _hit_data_dmg _hit_data_penetration _hit_data_poise _hit_data_knockbacktype _hit_data_velocityonfinishmode _hit_data_velocityonfinish _hit_data_clampvelocityonfinish _hit_data_duration _hit_data_badditive _hit_data_localdir _hit_data_distance _hit_data_strengthovertime _hit_data_brestrictspeedtoexpected _hit_data_gbextrabounceheight _hit_data_bgbadditive _hit_data_gbsot _hit_data_gbcvof _hit_data_bkilled _hit_data_dmgdealt _hit_data_hitimpactnormal _hit_data_hitimpactpoint _hit_data_hitloc _hit_data_hitsfx _hit_data_hitvfx _hit_data_hitvfxscale _hit_data_resolvedreaction) (break `AtkHitData` (`self.Hit Data`)))
  (`parent.OnAOEOverlap` Actor HitResult)
  (bind _output_get (set `self.Hit Data` (make `AtkHitData` _hit_data_attacker _hit_data_damager _hit_data_attackmotion _hit_data_attackreaction _hit_data_attacktype _hit_data_barmorbreaker _hit_data_biscounterfollowup _hit_data_elements _hit_data_aggrobuildup _hit_data_dmg _hit_data_penetration _hit_data_poise _hit_data_knockbacktype _hit_data_velocityonfinishmode _hit_data_velocityonfinish _hit_data_clampvelocityonfinish _hit_data_duration _hit_data_badditive _hit_data_localdir _hit_data_distance _hit_data_strengthovertime _hit_data_brestrictspeedtoexpected _hit_data_gbextrabounceheight _hit_data_bgbadditive _hit_data_gbsot _hit_data_gbcvof _hit_data_bkilled _hit_data_dmgdealt _impactnormal _impactpoint _location _hit_data_hitsfx _hit_data_hitvfx _hit_data_hitvfxscale _hit_data_resolvedreaction)))
  (`self.HandleDamage` Actor _output_get))

(event `Play Slash Sound`
  (`GameplayStatics.PlaySoundAtLocation` "/Game/Hack-N-Slash/Audio/SFX/Whooshes/SQ_SFX_Blade_Whoosh_02.SQ_SFX_Blade_Whoosh_02" (`self.K2_GetActorLocation`) (struct) 1.0 1.0 0.0 null null null null))

(fn `UserConstructionScript`
  (`parent.UserConstructionScript`))