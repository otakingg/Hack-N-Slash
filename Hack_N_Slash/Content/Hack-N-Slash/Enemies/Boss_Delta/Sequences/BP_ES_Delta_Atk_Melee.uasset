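; Melee attack sequence for the Delta boss, available when its target is close and at similar height.
; Execute focuses the target, then attacks at once if within desired distance, otherwise speeds up and chases first, with a one-second timer that stops movement.
; Move completion clears the timer and triggers the attack through the combat component.
; Finish writes the current game time to the Brain's blackboard; a macro validates references before acting.
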(event `StopChasing`
  (`Controller.StopMovement` (`EnemyBrainComponent.GetEnemyController` (`self.brain`))))

(event `self.Execute`
  (bind _brain (`self.brain`))
  (bind _brain_2 (`self.brain`))
  (bind (_targetactor _targetdistance) (break `EnemyBlackboard` (`EnemyBrainComponent.blackboard` _brain)))
  (`self.EnsureReferences`
    (:`Is Valid`
      (set `self.bInterruptible` true)
      (`EnemyController.SetFocusHNS` (`EnemyBrainComponent.GetEnemyController` _brain) _targetactor)
      (if (> _targetdistance (`self.DesiredDistance`))
        (`self.SetWalkSpeedAndAcceleration` 1000.0 2048.0)
        (`LocomotionComponent.MoveTo` (`EnemyBrainComponent.GetLocoMotionComp` _brain_2) (`.TargetActor` (break `EnemyBlackboard` (`EnemyBrainComponent.blackboard` _brain_2))) (0.0 0.0 0.0) (`self.AcceptanceRadius`))
        (bind _returnvalue (`KismetSystemLibrary.K2_SetTimerDelegate` (delegate `StopChasing`) 1.0))
        (set `self.TH_Chase` _returnvalue)
        (else
          (`EnemyCombatComponent.Attack` (`EnemyBrainComponent.GetEnemyCombatComp` (`self.brain`)) (`self.Atk`) :!label _label))))
    (:`Is Not Valid`
      (`self.Finish`))))

(event `self.HandleMoveCompleted`
  (params (RequestID :type Integer) (Result :type "EPathFollowingResult Enum" :default "Success"))
  (`KismetSystemLibrary.K2_ClearTimer` null "StopChasing")
  (`self.EnsureReferences`
    (:`Is Valid`
      (goto _label))
    (:`Is Not Valid`
      (`self.Finish`))))

(event `self.AdvanceSequence`
  (`self.Finish`))

(event `self.Finish`
  (bind _brain (`self.brain`))
  (bind (_targetactor _targetdistance _targetheightdifference _lastknownlocation _lastdamagesource _homelocation _aggro _lastattacktime _eqs_actors _eqs_locs _blockedon _bforgottarget) (break `EnemyBlackboard` (`EnemyBrainComponent.blackboard` _brain)))
  (`/Engine/EditorBlueprintResources/StandardMacros.IsValid` _brain
    (:`Is Valid`
      (set `EnemyBrainComponent.blackboard` (make `EnemyBlackboard` _targetactor _lastknownlocation _lastdamagesource _homelocation _aggro (`KismetSystemLibrary.GetGameTimeInSeconds` self) _bforgottarget) _brain))
    (:`Is Not Valid`
      _))
  (`self.FinishHelper`))

(fn `CanExecute`
  (returns (ReturnValue :type Boolean))
  (bind _brain (`self.brain`))
  (bind (_targetactor _targetdistance _targetheightdifference) (break `EnemyBlackboard` (`EnemyBrainComponent.blackboard` _brain)))
  (return (and (`parent.CanExecute`) (`KismetSystemLibrary.IsValid` _targetactor) (<= _targetdistance 800.0) (<= (`KismetMathLibrary.Abs` _targetheightdifference) 75.0) (`KismetSystemLibrary.IsValid` (`EnemyBrainComponent.GetEnemyCombatComp` _brain)) (`KismetSystemLibrary.IsValid` (`EnemyBrainComponent.GetLocoMotionComp` _brain)))))