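; Boss Delta's proactive attack sequence for a giant AOE centered on the arena.
; After a warning montage with reaction immunity, it dashes hidden to the tagged center POI via async root motion, then attacks and spawns a warning AOE.
; Each AOE's destruction drives the next phase: Delta vanishes while the damage AOE runs, then reappears with an end montage.
; Active-state checks guard each step, and Abort restores visibility, collision and immunity.
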(event `self.Initialize`
  (params (InBrain :type "EnemyBrainComponent Object Reference"))
  (`parent.Initialize` InBrain)
  (bind _brain (`self.brain`)
    (:`then`
      (bind _returnvalue (`ActorComponent.GetOwner` _brain))
      (bind _asbp_enemy_delta (cast `/Game/Hack-N-Slash/Enemies/Boss_Delta/BP_Enemy_Delta` _returnvalue))
      (set `self.Delta` _asbp_enemy_delta)
      (set `self.MeshComp` (`Actor.GetComponentByClass` _returnvalue "/Script/Engine.SkeletalMeshComponent"))
      (set `self.EnemyCombat` (`Actor.GetComponentByClass` _returnvalue "/Script/Hack_N_Slash.EnemyCombatComponent"))
      (set `self.Locomotion` (`Actor.GetComponentByClass` _returnvalue "/Script/Hack_N_Slash.LocomotionComponent"))
      (set `self.Capsule` (`Actor.GetComponentByClass` _returnvalue "/Script/Engine.CapsuleComponent"))
      (set `self.CombatRes` (`Actor.GetComponentByClass` _returnvalue "/Script/Hack_N_Slash.CombatResolutionComponent"))
      (set `self.Movement` (`Actor.GetComponentByClass` _returnvalue "/Script/Engine.CharacterMovementComponent")))
    (:`else`)))

(event `self.Execute`
  (`self.Is Active?`
    (:`Yes`
      (`self.EnsureReferences`
        (:`Is Valid`
          (bind _outactors (`GameplayStatics.GetAllActorsOfClassWithTag` self "/Game/Hack-N-Slash/Utility/BP_POI.BP_POI_C" "Delta.ArenaCenter"))
          (`self.Is Active?`
            (:`Yes`
              (if (`KismetArrayLibrary.Array_IsEmpty` _outactors)
                (`self.Finish`)
                (else
                  (`self.Set Reaction Immunity` true)
                  (set `self.dashLoc` (`Actor.K2_GetActorLocation` (`|GetArrayItem` _outactors)))
                  (`self.Is Active?`
                    (:`Yes`
                      (`|PlayMontage` (`self.MeshComp`) "/Game/Hack-N-Slash/Animations/Delta/Miscellaneous/AM_Delta_GiantAOE_Warning.AM_Delta_GiantAOE_Warning"
                        (:`OnCompleted`
                          (`self.AdvanceSequence`))
                        (:`OnInterrupted`
                          (`self.Finish`))))))))))
        (:`Is Not Valid`
          (`self.Finish`))))))

(event `self.HandleMoveCompleted`
  (params (RequestID :type Integer) (Result :type "EPathFollowingResult Enum" :default "Success"))
  (`self.AdvanceSequence`))

(event `self.AdvanceSequence`
  (`self.Is Active?`
    (:`Yes`
      (`self.EnsureReferences`
        (:`Is Valid`
          (bind _output_get (set `self.sequenceIndex` (+ (`self.sequenceIndex`) 1)))
          (switch `int` _output_get
            (:`Default`
              (`self.Finish`))
            (:`2`
              ;[0 1 1 0.5] Dash To Arena Center
              (bind (_asynctaskproxy _rootmovement) (`AsyncRootMovement.AsyncRootMovement_MoveTo` self (`self.Movement`) (`Actor.K2_GetActorLocation` (`ActorComponent.GetOwner` (`self.brain`))) (`self.dashLoc`) (`self.CalcMoveToDuration`))
                (:`then`
                  (bind _output_get_2 (set `self.RMS_MovTo_Center` _asynctaskproxy))
                  (`LocomotionComponent.AddRootMotionSource_BP` (`self.Locomotion`) _output_get_2 false)
                  (`self.Is Active?`
                    (:`Yes`
                      (`self.SetMeshVisibility` false)
                      (`self.Is Active?`
                        (:`Yes`
                          (`self.SetCollChanlResp` "ECC_Pawn")
                          (`self.Is Active?`
                            (:`Yes`
                              (`/Game/Hack-N-Slash/Enemies/Boss_Delta/BP_Enemy_Delta.ActivateDashFX` (`self.Delta`)))))))))
                (:`OnComplete`
                  (bind _locomotion (`self.Locomotion`)
                    (:`then`
                      (`LocomotionComponent.OnRootMotionComplete` _locomotion _rootmovement))
                    (:`else`
                      _))
                  (set `self.RMS_MovTo_Center` null)
                  (`self.Is Active?`
                    (:`Yes`
                      (`self.SetMeshVisibility` true)
                      (`self.Is Active?`
                        (:`Yes`
                          (`self.SetCollChanlResp` "ECC_Pawn" "ECR_Block")
                          (`self.Is Active?`
                            (:`Yes`
                              (bind _delta (`self.Delta`)
                                (:`then`
                                  (`/Game/Hack-N-Slash/Enemies/Boss_Delta/BP_Enemy_Delta.DeacticateDashVFX` _delta 0.5))
                                (:`else`
                                  _))
                              (`self.AdvanceSequence`))))))))
                (:`OnFail`
                  (set `self.RMS_MovTo_Center` null)
                  (`self.Set Reaction Immunity` false)
                  (`self.Finish`))
                (:`OnInterrupted`
                  (set `self.RMS_MovTo_Center` null)
                  (`self.Is Active?`
                    (:`Yes`
                      (bind _brain (`self.brain`)
                        (:`then`
                          (`EnemyBrainComponent.RemoveActiveSequence` _brain)
                          (`self.Abort`))
                        (:`else`)))))))
            (:`3`
              ;[1 0 0 0.5] Attack
              (bind _returnvalue (`EnemyCombatComponent.Attack` (`self.EnemyCombat`) (`self.Atk`)))
              (`self.Is Active?`
                (:`Yes`
                  (if _returnvalue
                    (bind _aoe_warning (`/Game/Hack-N-Slash/Enemies/Boss_Delta/BP_Enemy_Delta.SpawnGiantAOEWarning` (`self.Delta`)))
                    (bind _output_get_3 (set `self.AOE Warning` _aoe_warning))
                    (`self.Is Active?`
                      (:`Yes`
                        (`/Engine/EditorBlueprintResources/StandardMacros.IsValid` _output_get_3
                          (:`Is Valid`
                            (add `Actor.OnDestroyed` (`self.AOE Warning`) (delegate `Warning AOE Destroyed`)))
                          (:`Is Not Valid`
                            (`self.Finish`)))))
                    (else
                      (`self.Finish`))))))))
        (:`Is Not Valid`
          (`self.Finish`))))))

(event `Warning AOE Destroyed`
  (params (DestroyedActor :type "Actor Object Reference"))
  ;[1 0 0 0.5] Attack
  (`self.Is Active?`
    (:`Yes`
      (`self.SetCollChanlResp` "ECC_GameTraceChannel1")
      (`self.Is Active?`
        (:`Yes`
          (`self.SetCollChanlResp` "ECC_Pawn")
          (`self.Is Active?`
            (:`Yes`
              (`self.SetMeshVisibility` false)
              (`self.Is Active?`
                (:`Yes`
                  (bind _delta (`self.Delta`)
                    (:`then`
                      (bind _aoe_atk (`/Game/Hack-N-Slash/Enemies/Boss_Delta/BP_Enemy_Delta.SpawnGiantAOEAtk` _delta))
                      (`self.Is Active?`
                        (:`Yes`
                          (`/Engine/EditorBlueprintResources/StandardMacros.IsValid` _aoe_atk
                            (:`Is Valid`
                              (add `Actor.OnDestroyed` _aoe_atk (delegate `Atk AOE Destroyed`)))
                            (:`Is Not Valid`
                              (`self.Finish`))))))
                    (:`else`
                      (`self.Finish`))))))))))))

(event `self.Abort`
  (`parent.Abort`)
  (`self.ClearRootMotSrc` (`self.RMS_MovTo_Center`))
  (bind _aoe_warning (`self.AOE Warning`)
    (:`then`
      (`Actor.K2_DestroyActor` _aoe_warning))
    (:`else`
      _))
  (`self.SetMeshVisibility` true)
  (`self.SetCollChanlResp` "ECC_Pawn" "ECR_Block")
  (`self.SetCollChanlResp` "ECC_GameTraceChannel1" "ECR_Block")
  (`self.Set Reaction Immunity` false)
  (bind _delta (`self.Delta`)
    (:`then`
      (`/Game/Hack-N-Slash/Enemies/Boss_Delta/BP_Enemy_Delta.DeacticateDashVFX` _delta 0.0))
    (:`else`)))

(event `Atk AOE Destroyed`
  (params (DestroyedActor :type "Actor Object Reference"))
  ;[1 0 0 0.5] Attack
  (`self.Is Active?`
    (:`Yes`
      (`self.MeshComp`
        (:`then`
          (`self.SetMeshVisibility` true)
          (`self.Is Active?`
            (:`Yes`
              (`self.SetCollChanlResp` "ECC_Pawn" "ECR_Block")
              (`self.Is Active?`
                (:`Yes`
                  (`self.SetCollChanlResp` "ECC_GameTraceChannel1" "ECR_Block")
                  (`self.Is Active?`
                    (:`Yes`
                      (`self.Set Reaction Immunity` false)
                      (`self.Is Active?`
                        (:`Yes`
                          (`|PlayMontage` (`self.MeshComp`) (`.montage` (break `EnemyAtkData` (`self.Atk`))) 1.0 0.0 "End"
                            (:`OnCompleted`
                              _)
                            (:`OnInterrupted`
                              _))
                          (`self.AdvanceSequence`))))))))))
        (:`else`
          (`self.Finish`))))))

(event `self.Finish`
  (bind (_blackboard_targetactor _blackboard_targetdistance _blackboard_targetheightdifference _blackboard_lastdamagesource _blackboard_lastknownlocation _blackboard_homelocation _blackboard_lastattacktime _blackboard_recenthits _blackboard_eqs_actors _blackboard_eqs_locs _blackboard_blockedon _blackboard_bforgottarget) (break `EnemyBlackboard` (`EnemyBrainComponent.blackboard` (`self.brain`))))
  (`self.Is Active?`
    (:`Yes`
      (set `EnemyBrainComponent.blackboard` (make `EnemyBlackboard` _blackboard_targetactor _blackboard_targetdistance _blackboard_targetheightdifference _blackboard_lastdamagesource _blackboard_lastknownlocation _blackboard_homelocation (`KismetSystemLibrary.GetGameTimeInSeconds` self) _blackboard_recenthits _blackboard_eqs_actors _blackboard_eqs_locs _blackboard_blockedon _blackboard_bforgottarget) (`self.brain`))
      (`parent.Finish`))))

(fn `CalcMoveToDuration`
  (returns (Duration :type "Float (double-precision)"))
  (return (`KismetMathLibrary.FClamp` (/ (`KismetMathLibrary.Vector_Distance` (`Actor.K2_GetActorLocation` (`ActorComponent.GetOwner` (`self.brain`))) (`self.dashLoc`)) 5000.0) 0.1 0.5)))

(fn `CanExecute`
  (returns (ReturnValue :type Boolean))
  (return (and (`parent.CanExecute`) (`KismetSystemLibrary.IsValid` (`.TargetActor` (break `EnemyBlackboard` (`EnemyBrainComponent.blackboard` (`self.brain`))))) (`KismetSystemLibrary.IsValid` (`self.MeshComp`)) (`KismetSystemLibrary.IsValid` (`self.Capsule`)) (`KismetSystemLibrary.IsValid` (`self.Locomotion`)) (`KismetSystemLibrary.IsValid` (`self.EnemyCombat`)) (`KismetSystemLibrary.IsValid` (`self.CombatRes`)) (`KismetSystemLibrary.IsValid` (`self.Movement`)))))

(fn `ClearRootMotSrc`
  (params (RootMotSrc :type "AsyncRootMovement Object Reference"))
  (bind _locomotion (`self.Locomotion`)
    (:`then`
      (`LocomotionComponent.ClearRootMotionSource` _locomotion RootMotSrc))
    (:`else`)))

(fn `Set Reaction Immunity`
  (params (`bImmune?` :type Boolean :default false))
  (bind _combatres (`self.CombatRes`)
    (:`then`
      (`CombatResolutionComponent.SetImmunity` _combatres `bImmune?`))
    (:`else`)))

(fn `SetCollChanlResp`
  (params (Channel :type "ECollisionChannel Enum" :default "ECC_WorldStatic") (Response :type "ECollisionResponse Enum" :default "ECR_Ignore"))
  (bind _capsule (`self.Capsule`)
    (:`then`
      (`PrimitiveComponent.SetCollisionResponseToChannel` _capsule (`local.Channel`) (`local.Response`)))
    (:`else`)))

(fn `SetMeshVisibility`
  (params (`Visible?` :type Boolean))
  (bind _meshcomp (`self.MeshComp`)
    (:`then`
      (`SceneComponent.SetVisibility` _meshcomp `Visible?` true))
    (:`else`)))