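; Proactive enemy sequence that repositions the Delta boss with a fast, invisible dash.
; An EQS query picks the destination, flipping its distance scoring to favor far spots when the target is close and near spots when far.
; An async root-motion move carries Delta there with mesh hidden, Pawn collision ignored and dash VFX active.
; On arrival it restores these, then becomes interruptible and finishes after a short random delay; Abort also restores state.
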(event `self.Initialize`
  (params (InBrain :type "EnemyBrainComponent Object Reference"))
  (bind _delta (`self.Delta`))
  (`parent.Initialize` InBrain)
  (bind _brain (`self.brain`)
    (:`then`
      (bind _asbp_enemy_delta (cast `/Game/Hack-N-Slash/Enemies/Boss_Delta/BP_Enemy_Delta` (`ActorComponent.GetOwner` _brain)))
      (bind _output_get (set `self.Delta` _asbp_enemy_delta))
      (`/Engine/EditorBlueprintResources/StandardMacros.IsValid` _output_get
        (:`Is Valid`
          (set `self.Movement` (`Actor.GetComponentByClass` _output_get "/Script/Engine.CharacterMovementComponent"))
          (set `self.MeshComp` (`Actor.GetComponentByClass` _output_get "/Script/Engine.SkeletalMeshComponent"))
          (set `self.Locomotion` (`Actor.GetComponentByClass` _delta "/Script/Hack_N_Slash.LocomotionComponent"))
          (set `self.Capsule` (`Actor.GetComponentByClass` _delta "/Script/Engine.CapsuleComponent")))))
    (:`else`)))

(event `self.Execute`
  (bind _brain (`self.brain`))
  (`self.Is Active?`
    (:`Yes`
      (`self.EnsureReferences`
        (:`Is Valid`
          (`EnemyController.SetFocusHNS` (`EnemyBrainComponent.GetEnemyController` _brain) (`.TargetActor` (break `EnemyBlackboard` (`EnemyBrainComponent.blackboard` _brain))))
          (`self.Is Active?`
            (:`Yes`
              (`self.FindReposLoc`))))
        (:`Is Not Valid`
          (`self.Finish`))))))

(event `self.HandleEQSFinished`
  (params (Result :type "EnvQueryResult Structure (by ref)"))
  (`self.AdvanceSequence`))

(event `self.AdvanceSequence`
  (`self.Is Active?`
    (:`Yes`
      (`self.EnsureReferences`
        (:`Is Valid`
          (bind _output_get (set `self.sequenceIndex` (+ (`self.sequenceIndex`) 1)))
          (switch `int` _output_get
            (:`Default`
              (`self.Finish`))
            (:`2`
              (if (`KismetArrayLibrary.Array_IsEmpty` (`.EQS_Locs` (break `EnemyBlackboard` (`EnemyBrainComponent.blackboard` (`self.brain`)))))
                (`KismetSystemLibrary.PrintString` null "Enemy Delta Sequence: Reposition: Move Location invalid")
                (`self.Finish`)
                (else
                  (bind (_asynctaskproxy _rootmovement) (`AsyncRootMovement.AsyncRootMovement_MoveTo` self (`self.Movement`) (`Actor.K2_GetActorLocation` (`ActorComponent.GetOwner` (`self.brain`))) (`|GetArrayItem` (`.EQS_Locs` (break `EnemyBlackboard` (`EnemyBrainComponent.blackboard` (`self.brain`))))) (`self.CalcMoveToDuration`))
                    (:`then`
                      (bind _output_get_2 (set `self.RMS_MovTo_Rep` _asynctaskproxy))
                      (`LocomotionComponent.AddRootMotionSource_BP` (`self.Locomotion`) _output_get_2 false)
                      (`self.Is Active?`
                        (:`Yes`
                          (`self.SetMeshVisibility` false)
                          (`self.Is Active?`
                            (:`Yes`
                              (`self.SetCollChanlResp` "ECC_Pawn")
                              (`self.Is Active?`
                                (:`Yes`
                                  (`/Game/Hack-N-Slash/Enemies/Boss_Delta/BP_Enemy_Delta.ActivateDashFX` (`self.Delta`)))))))))
                    (:`OnComplete`
                      (bind _locomotion (`self.Locomotion`)
                        (:`then`
                          (`LocomotionComponent.OnRootMotionComplete` _locomotion _rootmovement))
                        (:`else`
                          _))
                      (set `self.RMS_MovTo_Rep` null)
                      (`self.Is Active?`
                        (:`Yes`
                          (`self.SetMeshVisibility` true)
                          (`self.Is Active?`
                            (:`Yes`
                              (`self.SetCollChanlResp` "ECC_Pawn" "ECR_Block")
                              (`self.Is Active?`
                                (:`Yes`
                                  (bind _delta (`self.Delta`)
                                    (:`then`
                                      (`/Game/Hack-N-Slash/Enemies/Boss_Delta/BP_Enemy_Delta.DeacticateDashVFX` _delta 0.5))
                                    (:`else`
                                      _))
                                  (`self.AdvanceSequence`))))))))
                    (:`OnFail`
                      (set `self.RMS_MovTo_Rep` null)
                      (`self.Finish`))
                    (:`OnInterrupted`
                      (set `self.RMS_MovTo_Rep` null)
                      (`self.Is Active?`
                        (:`Yes`
                          (bind _brain (`self.brain`)
                            (:`then`
                              (`EnemyBrainComponent.RemoveActiveSequence` _brain false)
                              (`self.Abort`))
                            (:`else`)))))))))
            (:`3`
              (set `self.bInterruptible` true)
              (bind _returnvalue (`KismetSystemLibrary.K2_SetTimer` null "Finish" (`KismetMathLibrary.RandomFloatInRange` 1.0 1.5)))
              (set `self.TH_Finish` _returnvalue))))
        (:`Is Not Valid`
          (`self.Finish`))))))

(event `self.Abort`
  (`parent.Abort`)
  (`self.ClearRootMotSrc` (`self.RMS_MovTo_Rep`))
  (`self.SetMeshVisibility` true)
  (`self.SetCollChanlResp` "ECC_Pawn" "ECR_Block")
  (bind _delta (`self.Delta`)
    (:`then`
      (`/Game/Hack-N-Slash/Enemies/Boss_Delta/BP_Enemy_Delta.DeacticateDashVFX` _delta 0.0))
    (:`else`)))

(fn `CalcMoveToDuration`
  (returns (Duration :type "Float (double-precision)"))
  (bind _brain (`self.brain`))
  (return (`KismetMathLibrary.FClamp` (/ (`KismetMathLibrary.Vector_Distance` (`Actor.K2_GetActorLocation` (`ActorComponent.GetOwner` _brain)) (`|GetArrayItem` (`.EQS_Locs` (break `EnemyBlackboard` (`EnemyBrainComponent.blackboard` _brain))))) 5000.0) 0.1 0.5)))

(fn `CanExecute`
  (returns (ReturnValue :type Boolean))
  (bind (_targetactor _targetdistance _targetheightdifference _lastknownlocation _lastdamagesource _homelocation _aggro _lastattacktime) (break `EnemyBlackboard` (`EnemyBrainComponent.blackboard` (`self.brain`))))
  (return (and (`parent.CanExecute`) (`KismetSystemLibrary.IsValid` _targetactor) (>= _lastattacktime 0.0) (`KismetSystemLibrary.IsValid` (`self.Movement`)) (`KismetSystemLibrary.IsValid` (`self.Locomotion`)) (`KismetSystemLibrary.IsValid` (`self.MeshComp`)) (`KismetSystemLibrary.IsValid` (`self.Capsule`)))))

(fn `ClearRootMotSrc`
  (params (RootMotSrc :type "AsyncRootMovement Object Reference"))
  (bind _locomotion (`self.Locomotion`)
    (:`then`
      (`LocomotionComponent.ClearRootMotionSource` _locomotion RootMotSrc))
    (:`else`)))

(fn `FindReposLoc`
  (locals (params :type "Map of Name to Float (single-precision)"))
  (if (<= (`.TargetDistance` (break `EnemyBlackboard` (`EnemyBrainComponent.blackboard` (`self.brain`)))) 300.0)
    (`BlueprintMapLibrary.Map_Add` (`local.params`) "Distance.ToTarget.ScoringFactor" 1.0)
    (else
      (`BlueprintMapLibrary.Map_Add` (`local.params`) "Distance.ToTarget.ScoringFactor" -1.0)))
  (`EnemyController.RunEQSQueryHNS` (`EnemyBrainComponent.GetEnemyController` (`self.brain`)) "/Game/Hack-N-Slash/EnvQuery/QueryTarget/EQ_Target_FarIfTargetClose_CloseIfTargetFar.EQ_Target_FarIfTargetClose_CloseIfTargetFar" (`local.params`) "RandomBest5Pct"))

(fn `SetCollChanlResp`
  (params (Channel :type "ECollisionChannel Enum" :default "ECC_WorldStatic") (Response :type "ECollisionResponse Enum" :default "ECR_Ignore"))
  (bind _capsule (`self.Capsule`)
    (:`then`
      (`PrimitiveComponent.SetCollisionResponseToChannel` _capsule (`local.Channel`) (`local.Response`)))
    (:`else`)))

(fn `SetMeshVisibility`
  (params (`Visible?` :type Boolean))
  (bind _meshcomp (`self.MeshComp`)
    (:`then`
      (`SceneComponent.SetVisibility` _meshcomp (`local.Visible?`) true))
    (:`else`)))