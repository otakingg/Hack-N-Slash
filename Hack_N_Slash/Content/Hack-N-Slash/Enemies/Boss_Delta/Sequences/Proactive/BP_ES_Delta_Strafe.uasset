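; Proactive, interruptible enemy sequence that makes the Delta boss strafe at slow walk speed while focused on its target.
; An EQS query picks the strafe spot, with scoring flipped by target distance to favor farther points when close and nearer ones when far.
; Query and move completion events advance the steps: move via the Locomotion component, then finish after a short random delay, ending early if no location is found.
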(event `self.Initialize`
  (params (InBrain :type "EnemyBrainComponent Object Reference"))
  (`parent.Initialize` InBrain)
  (bind _brain (`self.brain`)
    (:`then`
      (bind _returnvalue (`ActorComponent.GetOwner` _brain))
      (`/Engine/EditorBlueprintResources/StandardMacros.IsValid` _returnvalue
        (:`Is Valid`
          (set `self.Movement` (`Actor.GetComponentByClass` _returnvalue "/Script/Engine.CharacterMovementComponent"))
          (set `self.Locomotion` (`Actor.GetComponentByClass` _returnvalue "/Script/Hack_N_Slash.LocomotionComponent")))))
    (:`else`)))

(event `self.Execute`
  (bind _brain (`self.brain`))
  (`self.Is Active?`
    (:`Yes`
      (`self.EnsureReferences`
        (:`Is Valid`
          (set `self.bInterruptible` true)
          (`self.Is Active?`
            (:`Yes`
              (`EnemyController.SetFocusHNS` (`EnemyBrainComponent.GetEnemyController` _brain) (`.TargetActor` (break `EnemyBlackboard` (`EnemyBrainComponent.blackboard` _brain))))
              (`self.Is Active?`
                (:`Yes`
                  (`self.SetWalkSpeedAndAcceleration` 150.0 4000.0)
                  (`self.Is Active?`
                    (:`Yes`
                      (`self.FindStrafeLoc`))))))))
        (:`Is Not Valid`
          (`self.Finish`))))))

(event `self.HandleEQSFinished`
  (params (Result :type "EnvQueryResult Structure (by ref)"))
  (`self.AdvanceSequence`))

(event `self.HandleMoveCompleted`
  (params (RequestID :type Integer) (Result :type "EPathFollowingResult Enum" :default "Success"))
  (`self.AdvanceSequence`))

(event `self.AdvanceSequence`
  (`self.Is Active?`
    (:`Yes`
      (`self.EnsureReferences`
        (:`Is Valid`
          (bind _output_get (set `self.sequenceIndex` (+ (`self.sequenceIndex`) 1)))
          (switch `int` _output_get
            (:`Default`
              (`self.Finish`))
            (:`2`
              (bind _locsempty_ (`self.Move`))
              (if _locsempty_
                (`self.Finish`)))
            (:`3`
              (bind _returnvalue (`KismetSystemLibrary.K2_SetTimer` null "Finish" (`KismetMathLibrary.RandomFloatInRange` 0.0 2.0)))
              (set `self.TH_Finish` _returnvalue))))
        (:`Is Not Valid`
          (`self.Finish`))))))

(fn `CanExecute`
  (returns (ReturnValue :type Boolean))
  (return (and (`parent.CanExecute`) (`KismetSystemLibrary.IsValid` (`self.Movement`)) (`KismetSystemLibrary.IsValid` (`self.Locomotion`)) (`KismetSystemLibrary.IsValid` (`.TargetActor` (break `EnemyBlackboard` (`EnemyBrainComponent.blackboard` (`self.brain`))))))))

(fn `FindStrafeLoc`
  (locals (Params :type "Map of Name to Float (single-precision)"))
  (bind _params (`local.Params`))
  (bind _params_2 (`local.Params`))
  (bind (_blackboard_targetactor _blackboard_targetdistance) (break `EnemyBlackboard` (`EnemyBrainComponent.blackboard` (`self.brain`))))
  (if (<= _blackboard_targetdistance 500.0)
    (`BlueprintMapLibrary.Map_Add` _params_2 "Distance.Lesser.ScoringFactor")
    (`BlueprintMapLibrary.Map_Add` _params_2 "Distance.Greater.ScoringFactor" 1.0)
    (else
      (`BlueprintMapLibrary.Map_Add` _params "Distance.Lesser.ScoringFactor" 1.0)
      (`BlueprintMapLibrary.Map_Add` _params "Distance.Greater.ScoringFactor")))
  (`EnemyController.RunEQSQueryHNS` (`EnemyBrainComponent.GetEnemyController` (`self.brain`)) "/Game/Hack-N-Slash/EnvQuery/QuerySelf/EQ_Self_Strafe.EQ_Self_Strafe" (`local.Params`) "RandomBest5Pct"))

(fn `Move`
  (returns (`LocsEmpty?` :type Boolean))
  (bind (_targetactor _targetdistance _targetheightdifference _lastknownlocation _lastdamagesource _homelocation _lastattacktime _recenthits _eqs_actors _eqs_locs) (break `EnemyBlackboard` (`EnemyBrainComponent.blackboard` (`self.brain`))))
  (bind _returnvalue (`KismetArrayLibrary.Array_IsEmpty` _eqs_locs))
  (if (not _returnvalue)
    (`LocomotionComponent.MoveTo` (`self.Locomotion`) null (`|GetArrayItem` _eqs_locs) 60.0))
  (return _returnvalue))

(fn `SetWalkSpeedAndAcceleration`
  (params (Speed :type "Float (double-precision)") (Acceleration :type "Float (double-precision)"))
  (bind _movement (`self.Movement`)
    (:`then`
      (set `CharacterMovementComponent.MaxWalkSpeed` (`local.Speed`) _movement)
      (set `CharacterMovementComponent.MaxAcceleration` (`local.Acceleration`) _movement))
    (:`else`)))