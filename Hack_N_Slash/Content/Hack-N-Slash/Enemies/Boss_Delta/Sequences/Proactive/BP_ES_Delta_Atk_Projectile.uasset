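; Proactive enemy sequence for the Delta boss that performs a projectile attack at long range.
; It can run only when the Brain has a target at or beyond a minimum distance and an EnemyCombat component is cached from the owner.
; Execute checks references, marks itself reactive-interruptible and triggers the attack, finishing early if either step fails.
; AdvanceSequence stamps the current game time into the Brain's Blackboard, then finishes the sequence.
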(event `self.Initialize`
  (params (InBrain :type "EnemyBrainComponent Object Reference"))
  (`parent.Initialize` InBrain)
  (bind _brain (`self.brain`)
    (:`then`
      (bind _returnvalue (`ActorComponent.GetOwner` _brain))
      (`/Engine/EditorBlueprintResources/StandardMacros.IsValid` _returnvalue
        (:`Is Valid`
          (set `self.EnemyCombat` (`Actor.GetComponentByClass` _returnvalue "/Script/Hack_N_Slash.EnemyCombatComponent")))))
    (:`else`)))

(event `self.Execute`
  (`self.Is Active?`
    (:`Yes`
      (`self.EnsureReferences`
        (:`Is Valid`
          (set `self.bInterruptibleReactive` true)
          (`self.Is Active?`
            (:`Yes`
              (bind _returnvalue (`EnemyCombatComponent.Attack` (`self.EnemyCombat`) (`self.Atk`)))
              (if (not _returnvalue)
                (`self.Finish`)))))
        (:`Is Not Valid`
          (`self.Finish`))))))

(event `self.AdvanceSequence`
  (bind _brain (`self.brain`))
  (bind (_targetactor _targetdistance _targetheightdifference _lastdamagesource _lastknownlocation _homelocation _lastattacktime _recenthits _eqs_actors _eqs_locs _blockedon _bforgottarget) (break `EnemyBlackboard` (`EnemyBrainComponent.blackboard` _brain)))
  (`self.Is Active?`
    (:`Yes`
      (`/Engine/EditorBlueprintResources/StandardMacros.IsValid` _brain
        (:`Is Valid`
          (set `EnemyBrainComponent.blackboard` (make `EnemyBlackboard` _targetactor _targetdistance _targetheightdifference _lastdamagesource _lastknownlocation _homelocation (`KismetSystemLibrary.GetGameTimeInSeconds` self) _recenthits _eqs_actors _eqs_locs _blockedon _bforgottarget) (`self.brain`)))
        (:`Is Not Valid`
          _))
      (`self.Is Active?`
        (:`Yes`
          (`self.Finish`))))))

(fn `CanExecute`
  (returns (ReturnValue :type Boolean))
  (bind (_targetactor _targetdistance) (break `EnemyBlackboard` (`EnemyBrainComponent.blackboard` (`self.brain`))))
  (return (and (`parent.CanExecute`) (`KismetSystemLibrary.IsValid` _targetactor) (>= _targetdistance 1000.0) (`KismetSystemLibrary.IsValid` (`self.EnemyCombat`)))))