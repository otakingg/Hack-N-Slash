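; Proactive enemy sequence for the Delta boss's melee attack, runnable when the target is close and at similar height.
; Focuses the target, then attacks at once if within desired distance, otherwise raises walk speed and chases, with a timer capping the run.
; Move completion triggers the attack, with active-state and reference checks guarding the steps.
; A failed attack or sequence advance finishes it, writing game time to the Brain's blackboard.
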(event `self.Initialize`
  (params (InBrain :type "EnemyBrainComponent Object Reference"))
  (`parent.Initialize` InBrain)
  (bind _brain (`self.brain`)
    (:`then`
      (bind _returnvalue (`ActorComponent.GetOwner` _brain))
      (`/Engine/EditorBlueprintResources/StandardMacros.IsValid` _returnvalue
        (:`Is Valid`
          (set `self.Movement` (`Actor.GetComponentByClass` _returnvalue "/Script/Engine.CharacterMovementComponent"))
          (set `self.Locomotion` (`Actor.GetComponentByClass` _returnvalue "/Script/Hack_N_Slash.LocomotionComponent"))
          (set `self.EnemyCombat` (`Actor.GetComponentByClass` _returnvalue "/Script/Hack_N_Slash.EnemyCombatComponent")))))
    (:`else`)))

(event `self.Execute`
  (bind _brain (`self.brain`))
  (bind (_targetactor _targetdistance) (break `EnemyBlackboard` (`EnemyBrainComponent.blackboard` _brain)))
  (`self.Is Active?`
    (:`Yes`
      (`self.EnsureReferences`
        (:`Is Valid`
          (set `self.bInterruptible` true)
          (`self.Is Active?`
            (:`Yes`
              (`EnemyController.SetFocusHNS` (`EnemyBrainComponent.GetEnemyController` _brain) _targetactor)
              (`self.Is Active?`
                (:`Yes`
                  (if (> _targetdistance (`self.DesiredDistance`))
                    (`self.SetWalkSpeedAndAcceleration` 1000.0 2048.0)
                    (`self.Is Active?`
                      (:`Yes`
                        (`LocomotionComponent.MoveTo` (`self.Locomotion`) (`.TargetActor` (break `EnemyBlackboard` (`EnemyBrainComponent.blackboard` (`self.brain`)))) (0.0 0.0 0.0) (`self.AcceptanceRadius`))
                        (`self.Is Active?`
                          (:`Yes`
                            (bind _returnvalue (`KismetSystemLibrary.K2_SetTimerDelegate` (delegate `StopChasing`) 1.0))
                            (set `self.TH_Chase` _returnvalue)))))
                    (else
                      (bind _returnvalue_2 (`EnemyCombatComponent.Attack` (`self.EnemyCombat`) (`self.Atk`) :!label _label))
                      (if (not _returnvalue_2)
                        (`self.Finish`)))))))))
        (:`Is Not Valid`
          (`self.Finish`))))))

(event `StopChasing`
  (`self.Is Active?`
    (:`Yes`
      (`Controller.StopMovement` (`EnemyBrainComponent.GetEnemyController` (`self.brain`))))))

(event `self.HandleMoveCompleted`
  (params (RequestID :type Integer) (Result :type "EPathFollowingResult Enum" :default "Success"))
  (`KismetSystemLibrary.K2_ClearTimer` null "StopChasing")
  (`self.Is Active?`
    (:`Yes`
      (`self.EnsureReferences`
        (:`Is Valid`
          (goto _label))
        (:`Is Not Valid`
          (`self.Finish`))))))

(event `self.AdvanceSequence`
  (`self.Finish`))

(event `self.Finish`
  (bind _brain (`self.brain`))
  (bind (_targetactor _targetdistance _targetheightdifference _lastknownlocation _lastdamagesource _homelocation _lastattacktime _recenthits _eqs_actors _eqs_locs _blockedon _bforgottarget) (break `EnemyBlackboard` (`EnemyBrainComponent.blackboard` _brain)))
  (`/Engine/EditorBlueprintResources/StandardMacros.IsValid` _brain
    (:`Is Valid`
      (set `EnemyBrainComponent.blackboard` (make `EnemyBlackboard` _targetactor _lastknownlocation _lastdamagesource _homelocation (`KismetSystemLibrary.GetGameTimeInSeconds` self) _recenthits _bforgottarget) (`self.brain`))
      (`parent.Finish`))))

(fn `CanExecute`
  (returns (ReturnValue :type Boolean))
  (bind (_targetactor _targetdistance _targetheightdifference) (break `EnemyBlackboard` (`EnemyBrainComponent.blackboard` (`self.brain`))))
  (return (and (`parent.CanExecute`) (`KismetSystemLibrary.IsValid` _targetactor) (<= _targetdistance 800.0) (<= (`KismetMathLibrary.Abs` _targetheightdifference) 75.0) (`KismetSystemLibrary.IsValid` (`self.Movement`)) (`KismetSystemLibrary.IsValid` (`self.Locomotion`)) (`KismetSystemLibrary.IsValid` (`self.EnemyCombat`)))))

(fn `SetWalkSpeedAndAcceleration`
  (params (Speed :type "Float (double-precision)") (Acceleration :type "Float (double-precision)"))
  (bind _movement (`self.Movement`)
    (:`then`
      (set `CharacterMovementComponent.MaxWalkSpeed` (`local.Speed`) _movement)
      (set `CharacterMovementComponent.MaxAcceleration` (`local.Acceleration`) _movement))
    (:`else`)))