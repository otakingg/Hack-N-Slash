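; Enemy brain attack sequence for the Delta boss that closes the gap by dashing toward and past its target by an offset.
; Execute starts the attack, and its Dash anim notify triggers FindDashLoc, which steps capsule-widths along the path checking obstacles and ground.
; An async root motion source moves the boss over a distance-scaled, clamped duration, ignoring Pawn collision until completion.
; Finishing timestamps the Blackboard, while Abort clears the root motion.
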(event `self.Initialize`
  (params (InBrain :type "EnemyBrainComponent Object Reference"))
  (`parent.Initialize` InBrain)
  (bind _brain (`self.brain`)
    (:`then`
      (bind _returnvalue (`ActorComponent.GetOwner` _brain))
      (`/Engine/EditorBlueprintResources/StandardMacros.IsValid` _returnvalue
        (:`Is Valid`
          (set `self.Movement` (`Actor.GetComponentByClass` _returnvalue "/Script/Engine.CharacterMovementComponent"))
          (set `self.MeshComp` (`Actor.GetComponentByClass` _returnvalue "/Script/Engine.SkeletalMeshComponent"))
          (set `self.EnemyCombat` (`Actor.GetComponentByClass` _returnvalue "/Script/Hack_N_Slash.EnemyCombatComponent"))
          (set `self.Capsule` (`Actor.GetComponentByClass` _returnvalue "/Script/Engine.CapsuleComponent"))
          (set `self.Locomotion` (`Actor.GetComponentByClass` _returnvalue "/Script/Hack_N_Slash.LocomotionComponent")))))
    (:`else`)))

(event `self.Execute`
  (`self.Is Active?`
    (:`Yes`
      (`self.EnsureReferences`
        (:`Is Valid`
          (bind _returnvalue (`EnemyCombatComponent.Attack` (`self.EnemyCombat`) (`self.Atk`)))
          (if (not _returnvalue)
            (`self.Finish`)))
        (:`Is Not Valid`
          (`self.Finish`))))))

(event `self.HandleAnimNotify`
  (params (NotifyTag :type "GameplayTag Structure (by ref)"))
  (`parent.HandleAnimNotify` NotifyTag)
  (`self.Is Active?`
    (:`Yes`
      (`self.EnsureReferences`
        (:`Is Valid`
          (`|SwitchGameplayTag` NotifyTag
            (:`NotifyEvent.EnemyBrain.Dash`
              (bind _output_get (set `self.startLoc` (`Actor.K2_GetActorLocation` (`ActorComponent.GetOwner` (`self.brain`)))))
              (bind _output_get_2 (set `self.dashLoc` (`self.FindDashLoc` _output_get)))
              (`self.Is Active?`
                (:`Yes`
                  (if (== _output_get_2 (`self.startLoc`) :`ErrorTolerance` 100.0)
                    (`KismetSystemLibrary.PrintString` self "Delta Gap Closer: Dash Loc is nearly equal to start loc")
                    (`self.Finish`)
                    (else
                      (bind (_asynctaskproxy _rootmovement) (`AsyncRootMovement.AsyncRootMovement_MoveTo` self (`self.Movement`) (`self.startLoc`) (`self.dashLoc`) (`KismetMathLibrary.FClamp` (/ (`KismetMathLibrary.Vector_Distance` (`self.dashLoc`) (`self.startLoc`)) 5000.0) 0.1 0.5))
                        (:`then`
                          (bind _output_get_3 (set `self.RMS_MovTo_GC` _asynctaskproxy))
                          (`LocomotionComponent.AddRootMotionSource_BP` (`self.Locomotion`) _output_get_3 false)
                          (`self.Is Active?`
                            (:`Yes`
                              (`self.SetCollChanlResp` "ECC_Pawn"))))
                        (:`OnComplete`
                          (bind _locomotion (`self.Locomotion`)
                            (:`then`
                              (`LocomotionComponent.OnRootMotionComplete` _locomotion _rootmovement))
                            (:`else`
                              _))
                          (set `self.RMS_MovTo_GC` null)
                          (`self.Is Active?`
                            (:`Yes`
                              (`self.SetCollChanlResp` "ECC_Pawn" "ECR_Block"))))
                        (:`OnFail`
                          (set `self.RMS_MovTo_GC` null)
                          (`self.Finish`))
                        (:`OnInterrupted`
                          (set `self.RMS_MovTo_GC` null)
                          (`self.Is Active?`
                            (:`Yes`
                              (bind _brain (`self.brain`)
                                (:`then`
                                  (`EnemyBrainComponent.RemoveActiveSequence` _brain)
                                  (`self.Abort`))
                                (:`else`)))))))))))))
        (:`Is Not Valid`
          (`self.Finish`))))))

(event `self.AdvanceSequence`
  (bind _brain (`self.brain`))
  (bind (_targetactor _targetdistance _targetheightdifference _lastdamagesource _lastknownlocation _homelocation _lastattacktime _recenthits _eqs_actors _eqs_locs _blockedon _bforgottarget) (break `EnemyBlackboard` (`EnemyBrainComponent.blackboard` _brain)))
  (`/Engine/EditorBlueprintResources/StandardMacros.IsValid` _brain
    (:`Is Valid`
      (set `EnemyBrainComponent.blackboard` (make `EnemyBlackboard` _targetactor -1.0 0.0 _lastdamagesource _lastknownlocation _homelocation (`KismetSystemLibrary.GetGameTimeInSeconds` self) _recenthits _ _ false _bforgottarget) _brain))
    (:`Is Not Valid`
      _))
  (`self.Finish`))

(event `self.Abort`
  (`parent.Abort`)
  (`self.ClearRootMotSrc` (`self.RMS_MovTo_GC`)))

(event `self.Finish`
  (bind (_blackboard_targetactor _blackboard_targetdistance _blackboard_targetheightdifference _blackboard_lastdamagesource _blackboard_lastknownlocation _blackboard_homelocation _blackboard_lastattacktime _blackboard_recenthits _blackboard_eqs_actors _blackboard_eqs_locs _blackboard_blockedon _blackboard_bforgottarget) (break `EnemyBlackboard` (`EnemyBrainComponent.blackboard` (`self.brain`))))
  (`self.Is Active?`
    (:`Yes`
      (set `EnemyBrainComponent.blackboard` (make `EnemyBlackboard` _blackboard_targetactor _blackboard_targetdistance _blackboard_targetheightdifference _blackboard_lastdamagesource _blackboard_lastknownlocation _blackboard_homelocation (`KismetSystemLibrary.GetGameTimeInSeconds` self) _blackboard_recenthits _blackboard_eqs_actors _blackboard_eqs_locs _blackboard_blockedon _blackboard_bforgottarget) (`self.brain`))
      (`parent.Finish`))))

(fn `CanExecute`
  (returns (ReturnValue :type Boolean))
  (return (and (`parent.CanExecute`) (`KismetSystemLibrary.IsValid` (`.TargetActor` (break `EnemyBlackboard` (`EnemyBrainComponent.blackboard` (`self.brain`))))) (`KismetSystemLibrary.IsValid` (`self.Movement`)) (`KismetSystemLibrary.IsValid` (`self.Locomotion`)) (`KismetSystemLibrary.IsValid` (`self.MeshComp`)) (`KismetSystemLibrary.IsValid` (`self.Capsule`)) (`KismetSystemLibrary.IsValid` (`self.EnemyCombat`)))))

(fn `ClearRootMotSrc`
  (params (RootMotSrc :type "AsyncRootMovement Object Reference"))
  (bind _locomotion (`self.Locomotion`)
    (:`then`
      (`LocomotionComponent.ClearRootMotionSource` _locomotion RootMotSrc))
    (:`else`)))

(fn `FindDashLoc`
  (params (startLoc :type "Vector Structure"))
  (returns (dashLoc :type "Vector Structure"))
  (locals (diameter :type "Float (single-precision)" :default 0.0) (capsueCount :type Integer) (desiredLoc :type "Vector Structure") (bestLoc :type "Vector Structure") (dashDir :type "Vector Structure" :default (0.0 0.0 0.0)) (testLoc :type "Vector Structure"))
  (bind _testloc (`local.testLoc`))
  (bind _brain (`self.brain`))
  (bind (_outradius _outhalfheight) (`CapsuleComponent.GetUnscaledCapsuleSize` (`self.Capsule`)))
  (bind _returnvalue (`Actor.K2_GetActorLocation` (`.TargetActor` (break `EnemyBlackboard` (`EnemyBrainComponent.blackboard` _brain)))))
  (bind _returnvalue_2 (`KismetMathLibrary.Normal` (- _returnvalue (`local.startLoc`))))
  (set `local.bestLoc` startLoc)
  (set `local.diameter` (* (`CapsuleComponent.CapsuleRadius` (`self.Capsule`)) 2.0))
  (set `local.dashDir` _returnvalue_2)
  (set `local.desiredLoc` (+ _returnvalue (* _returnvalue_2 (`self.dashLocOffset`))))
  (bind _output_get (set `local.capsueCount` (/ (`KismetMathLibrary.Vector_Distance` (`local.desiredLoc`) (`local.startLoc`)) (`local.diameter`))))
  (for _ (range (+ _output_get 1))
    (bind _output_get_2 (set `local.testLoc` (+ (`local.bestLoc`) (* (`local.dashDir`) (`local.diameter`)))))
    (bind _outhits (`KismetSystemLibrary.CapsuleTraceMultiForObjects` self _output_get_2 _output_get_2 _outradius _outhalfheight (`|MakeArray` "ObjectTypeQuery1" "ObjectTypeQuery2" "ObjectTypeQuery5" "ObjectTypeQuery6" :!type "EObjectTypeQuery Enum") false (`|MakeArray` (`ActorComponent.GetOwner` _brain) (`.TargetActor` (break `EnemyBlackboard` (`EnemyBrainComponent.blackboard` (`self.brain`))))) (select `bool` (`self.bDebug`) :`true` "ForDuration" :!type "EDrawDebugTrace Enum") true (struct :`R` 1.0 :`A` 1.0) (struct :`G` 1.0 :`A` 1.0) 3.0))
    (if (`self.IsValidDashLoc` _outhits (`local.testLoc`))
      (set `local.bestLoc` _testloc)
      (else
        (return _testloc))))
  (return (`local.bestLoc`)))

(fn `IsValidDashLoc`
  (params (Hits :type "Array of HitResult Structure") (Location :type "Vector Structure"))
  (returns (`Valid?` :type Boolean))
  (bind (_outradius _outhalfheight) (`CapsuleComponent.GetUnscaledCapsuleSize` (`self.Capsule`)))
  (bind (_outhit _returnvalue) (`KismetSystemLibrary.SphereTraceSingle` self Location (- Location (`KismetMathLibrary.MakeVector` 0.0 0.0 (+ _outhalfheight 200.0))) _outradius "TraceTypeQuery1" false (`|MakeArray` (`ActorComponent.GetOwner` (`self.brain`))) (select `bool` (`self.bDebug`) :`true` "ForDuration" :!type "EDrawDebugTrace Enum") true (struct :`R` 1.0 :`A` 1.0) (struct :`G` 1.0 :`A` 1.0) 3.0))
  (if _returnvalue
    (for _array_element (`local.Hits`)
      (if (`|EnumEquality` (`PrimitiveComponent.GetCollisionResponseToChannel` (`.HitComponent` (`GameplayStatics.BreakHitResult` _array_element)) "ECC_Pawn") "ECR_Block")
        (return false)))
    (return true)
    (else
      (return false))))

(fn `SetCollChanlResp`
  (params (Channel :type "ECollisionChannel Enum" :default "ECC_WorldStatic") (Response :type "ECollisionResponse Enum" :default "ECR_Ignore"))
  (bind _capsule (`self.Capsule`)
    (:`then`
      (`PrimitiveComponent.SetCollisionResponseToChannel` _capsule (`local.Channel`) (`local.Response`)))
    (:`else`)))