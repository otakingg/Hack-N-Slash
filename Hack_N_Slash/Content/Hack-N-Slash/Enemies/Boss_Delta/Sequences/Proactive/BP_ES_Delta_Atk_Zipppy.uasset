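; Proactive attack sequence for the Delta boss that zips around its target in three rapid dashes, then strikes with a close or far attack chosen by distance.
; An indexed state machine chains EQS location queries, root-motion moves and short random pauses, with EQS scoring flipped by target distance.
; During each dash the mesh is hidden, pawn collision is ignored and dash VFX play; Abort restores all three.
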(event `self.Initialize`
  (params (InBrain :type "EnemyBrainComponent Object Reference"))
  (`parent.Initialize` InBrain)
  (bind _brain (`self.brain`)
    (:`then`
      (bind _asbp_enemy_delta (cast `/Game/Hack-N-Slash/Enemies/Boss_Delta/BP_Enemy_Delta` (`ActorComponent.GetOwner` _brain)))
      (set `self.Delta` _asbp_enemy_delta))
    (:`else`)))

(event `self.Execute`
  (bind _brain (`self.brain`))
  (`self.Is Active?`
    (:`Yes`
      (`self.EnsureReferences`
        (:`Is Valid`
          (`EnemyController.SetFocusHNS` (`EnemyBrainComponent.GetEnemyController` _brain) (`.TargetActor` (break `EnemyBlackboard` (`EnemyBrainComponent.blackboard` _brain))))
          (`self.Is Active?`
            (:`Yes`
              (`self.FindDashLoc`))))
        (:`Is Not Valid`
          (`self.Finish`))))))

(event `self.HandleEQSFinished`
  (params (Result :type "EnvQueryResult Structure (by ref)"))
  (`self.AdvanceSequence`))

(event `self.AdvanceSequence`
  (bind _brain (`self.brain`))
  (bind _brain_2 (`self.brain`))
  (bind _returnvalue (`EnemyBrainComponent.GetLocoMotionComp` (`self.brain`)))
  (`self.Is Active?`
    (:`Yes`
      (`self.EnsureReferences`
        (:`Is Valid`
          (bind _output_get (set `self.sequenceIndex` (+ (`self.sequenceIndex`) 1)))
          (switch `int` _output_get
            (:`Default`
              (`self.Finish`))
            (:`2`
              (if (`KismetArrayLibrary.Array_IsEmpty` (`.EQS_Locs` (break `EnemyBlackboard` (`EnemyBrainComponent.blackboard` (`self.brain`))))) :!label _label
                (`KismetSystemLibrary.PrintString` null "Enemy Delta Sequence: Reposition: Move Location invalid")
                (`self.Finish`)
                (else
                  (bind (_asynctaskproxy _rootmovement) (`AsyncRootMovement.AsyncRootMovement_MoveTo` self (`EnemyBrainComponent.GetCharacterMovement` (`self.brain`)) (`Actor.K2_GetActorLocation` (`ActorComponent.GetOwner` (`self.brain`))) (`|GetArrayItem` (`.EQS_Locs` (break `EnemyBlackboard` (`EnemyBrainComponent.blackboard` (`self.brain`))))) (`KismetMathLibrary.FClamp` (/ (`KismetMathLibrary.Vector_Distance` (`Actor.K2_GetActorLocation` (`ActorComponent.GetOwner` _brain)) (`|GetArrayItem` (`.EQS_Locs` (break `EnemyBlackboard` (`EnemyBrainComponent.blackboard` _brain))))) 5000.0) 0.1 0.5))
                    (:`then`
                      (`/Engine/EditorBlueprintResources/StandardMacros.IsValid` _asynctaskproxy
                        (:`Is Valid`
                          (`LocomotionComponent.AddRootMotionSource` (`EnemyBrainComponent.GetLocoMotionComp` (`self.brain`)) _asynctaskproxy false)
                          (`self.Is Active?`
                            (:`Yes`
                              (`self.SetMeshVisibility` false)
                              (`self.Is Active?`
                                (:`Yes`
                                  (`self.SetCollChanlResp` "ECC_Pawn")
                                  (`self.Is Active?`
                                    (:`Yes`
                                      (`/Game/Hack-N-Slash/Enemies/Boss_Delta/BP_Enemy_Delta.ActivateDashFX` (`self.Delta`)))))))))
                        (:`Is Not Valid`
                          (`self.Finish`))))
                    (:`OnComplete`
                      (`/Engine/EditorBlueprintResources/StandardMacros.IsValid` _returnvalue
                        (:`Is Valid`
                          (`LocomotionComponent.OnRootMotionComplete` _returnvalue _rootmovement))
                        (:`Is Not Valid`
                          _))
                      (`self.Is Active?`
                        (:`Yes`
                          (`self.SetMeshVisibility` true)
                          (`self.Is Active?`
                            (:`Yes`
                              (`self.SetCollChanlResp` "ECC_Pawn" "ECR_Block")
                              (`self.Is Active?`
                                (:`Yes`
                                  (bind _delta (`self.Delta`)
                                    (:`then`
                                      (`/Game/Hack-N-Slash/Enemies/Boss_Delta/BP_Enemy_Delta.DeacticateDashVFX` _delta (`KismetMathLibrary.SelectFloat` 0.5 0.0 (>= (`self.sequenceIndex`) 8))))
                                    (:`else`
                                      _))
                                  (`self.AdvanceSequence`))))))))
                    (:`OnFail`
                      (`self.Finish`))))))
            (:`3`
              (`self.SetCollChanlResp` "ECC_Pawn" "ECR_Block" :!label _label_2)
              (`self.Is Active?`
                (:`Yes`
                  (bind _returnvalue_2 (`KismetSystemLibrary.K2_SetTimer` null "AdvanceSequence" (`KismetMathLibrary.RandomFloatInRange` 0.25 0.5)))
                  (set `self.TH_AdvSeq` _returnvalue_2))))
            (:`4`
              (`self.FindDashLoc` :!label _label_3))
            (:`5`
              (goto _label))
            (:`6`
              (goto _label_2))
            (:`7`
              (goto _label_3))
            (:`8`
              (goto _label))
            (:`9`
              (`AIController.K2_ClearFocus` (`EnemyBrainComponent.GetEnemyController` _brain_2))
              (`self.Is Active?`
                (:`Yes`
                  (bind _returnvalue_3 (`EnemyCombatComponent.Attack` (`EnemyBrainComponent.GetEnemyCombatComp` _brain_2) (select `bool` (> (`self.GetTargetDistance`) 600.0) :`false` (`self.atkClose`) :`true` (`self.atkFar`))))
                  (if (not _returnvalue_3)
                    (`self.Is Active?`
                      (:`Yes`
                        (`self.Finish`)))))))))
        (:`Is Not Valid`
          (`self.Finish`))))))

(event `self.Abort`
  (`parent.Abort`)
  (`self.SetMeshVisibility` true)
  (`self.SetCollChanlResp` "ECC_Pawn" "ECR_Block")
  (bind _delta (`self.Delta`)
    (:`then`
      (`/Game/Hack-N-Slash/Enemies/Boss_Delta/BP_Enemy_Delta.DeacticateDashVFX` _delta 0.0))
    (:`else`)))

(event `self.Finish`
  (bind _brain (`self.brain`))
  (bind (_targetactor _targetdistance _targetheightdifference _lastknownlocation _lastdamagesource _homelocation _aggro _lastattacktime _eqs_actors _eqs_locs _blockedon _bforgottarget) (break `EnemyBlackboard` (`EnemyBrainComponent.blackboard` _brain)))
  (`self.Is Active?`
    (:`Yes`
      (`/Engine/EditorBlueprintResources/StandardMacros.IsValid` _brain
        (:`Is Valid`
          (set `EnemyBrainComponent.blackboard` (make `EnemyBlackboard` _targetactor _lastknownlocation _lastdamagesource _homelocation _aggro (`KismetSystemLibrary.GetGameTimeInSeconds` self) _bforgottarget) (`self.brain`))
          (`parent.Finish`))))))

(fn `CanExecute`
  (returns (ReturnValue :type Boolean))
  (bind _brain (`self.brain`))
  (bind (_targetactor _targetdistance _targetheightdifference _lastknownlocation _lastdamagesource _homelocation _aggro _lastattacktime) (break `EnemyBlackboard` (`EnemyBrainComponent.blackboard` _brain)))
  (return (and (`parent.CanExecute`) (`KismetSystemLibrary.IsValid` _targetactor) (>= _lastattacktime 0.0) (`KismetSystemLibrary.IsValid` (`EnemyBrainComponent.GetEnemyCombatComp` _brain)))))

(fn `FindDashLoc`
  (locals (params :type "Map of Name to Float (single-precision)"))
  (if (<= (`.TargetDistance` (break `EnemyBlackboard` (`EnemyBrainComponent.blackboard` (`self.brain`)))) 300.0)
    (`BlueprintMapLibrary.Map_Add` (`local.params`) "Distance.ToTarget.ScoringFactor" 1.0)
    (else
      (`BlueprintMapLibrary.Map_Add` (`local.params`) "Distance.ToTarget.ScoringFactor" -1.0)))
  (`EnemyController.RunEQSQueryHNS` (`EnemyBrainComponent.GetEnemyController` (`self.brain`)) "/Game/Hack-N-Slash/EnvQuery/QueryTarget/EQ_Target_FarIfTargetClose_CloseIfTargetFar.EQ_Target_FarIfTargetClose_CloseIfTargetFar" (`local.params`) "RandomBest5Pct"))

(fn `SetCollChanlResp`
  (params (Channel :type "ECollisionChannel Enum" :default "ECC_WorldStatic") (Response :type "ECollisionResponse Enum" :default "ECR_Ignore"))
  (bind _brain (`self.brain`)
    (:`then`
      (bind _returnvalue (`EnemyBrainComponent.GetCapsule` _brain))
      (`/Engine/EditorBlueprintResources/StandardMacros.IsValid` _returnvalue
        (:`Is Valid`
          (`PrimitiveComponent.SetCollisionResponseToChannel` _returnvalue (`local.Channel`) (`local.Response`)))))
    (:`else`)))

(fn `SetMeshVisibility`
  (params (`Visible?` :type Boolean))
  (bind _brain (`self.brain`)
    (:`then`
      (bind _returnvalue (`EnemyBrainComponent.GetMesh` _brain))
      (`/Engine/EditorBlueprintResources/StandardMacros.IsValid` _returnvalue
        (:`Is Valid`
          (`SceneComponent.SetVisibility` _returnvalue (`local.Visible?`) true))))
    (:`else`)))