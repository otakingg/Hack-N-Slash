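; Boss Delta enemy sequence that triggers a projectile attack on the current target.
; It can execute only when the parent check passes and the blackboard's target is valid and at least a set minimum distance away.
; Execution validates brain, owner, movement, controller, state machine and target, then requests the attack from the state machine, or finishes if any is missing.
; Advancing the sequence writes the current game time to the blackboard and finishes.
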(event `self.Execute`
  (`self.EnsureReferences`
    (:`Is Valid`
      (`StateMachineComponent.RequestAttackEnemy` (`EnemyBrainComponent.GetStateMachine` (`self.GetBrain`)) (`self.Atk`)))
    (:`Is Not Valid`
      (`self.Finish`))))

(event `self.AdvanceSequence`
  (bind _returnvalue (`self.GetBrain`))
  (bind (_blackboard_targetactor _blackboard_targetdistance _blackboard_targetheightdifference _blackboard_lastknownlocation _blackboard_lastdamagesource _blackboard_homelocation _blackboard_aggro _blackboard_lastattacktime _blackboard_eqs_actors _blackboard_eqs_locs _blackboard_bforgottarget _blackboard_bstaggered) (break `EnemyBlackboard` (`EnemyBrainComponent.blackboard` _returnvalue)))
  (`/Engine/EditorBlueprintResources/StandardMacros.IsValid` _returnvalue
    (:`Is Valid`
      (set `EnemyBrainComponent.blackboard` (make `EnemyBlackboard` _blackboard_targetactor _blackboard_lastknownlocation _blackboard_lastdamagesource _blackboard_homelocation _blackboard_aggro (`KismetSystemLibrary.GetGameTimeInSeconds` self) _blackboard_bforgottarget _blackboard_bstaggered) _returnvalue))
    (:`Is Not Valid`
      _))
  (`self.Finish`))

(fn `CanExecute`
  (returns (ReturnValue :type Boolean))
  (bind (_blackboard_targetactor _blackboard_targetdistance) (break `EnemyBlackboard` (`EnemyBrainComponent.blackboard` (`self.GetBrain`))))
  (return (and (`parent.CanExecute`) (`KismetSystemLibrary.IsValid` _blackboard_targetactor) (>= _blackboard_targetdistance 700.0))))