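; Boss Delta enemy sequence for the giant AOE attack, requiring a valid target and combat component.
; It finds the tagged arena-center POI and plays a montage, whose completion advances an indexed step machine.
; The steps dash the boss there via async root-movement with distance-based, clamped duration, ignoring Pawn collision, then trigger the attack through the combat component.
; Finishing writes the current game time to the Brain's blackboard.
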(event `self.Execute`
  (`self.EnsureReferences`
    (:`Is Valid`
      (bind _outactors (`GameplayStatics.GetAllActorsOfClassWithTag` self "/Game/Hack-N-Slash/Utility/BP_POI.BP_POI_C" "Delta.ArenaCenter"))
      (if (`KismetArrayLibrary.Array_IsEmpty` _outactors)
        (`self.Finish`)
        (else
          (set `self.dashLoc` (`Actor.K2_GetActorLocation` (`|GetArrayItem` _outactors)))
          (`|PlayMontage` (`EnemyBrainComponent.GetMesh` (`self.brain`))
            (:`OnCompleted`
              (`self.AdvanceSequence`))
            (:`OnInterrupted`
              (`self.Finish`))))))
    (:`Is Not Valid`
      (`self.Finish`))))

(event `self.HandleMoveCompleted`
  (params (RequestID :type Integer) (Result :type "EPathFollowingResult Enum" :default "Success"))
  (`self.AdvanceSequence`))

(event `self.AdvanceSequence`
  (bind _brain (`self.brain`))
  (bind _returnvalue (`EnemyBrainComponent.GetCapsule` (`self.brain`)))
  (bind _returnvalue_2 (`Actor.K2_GetActorLocation` (`ActorComponent.GetOwner` _brain)))
  (`self.EnsureReferences`
    (:`Is Valid`
      (bind _output_get (set `self.sequenceIndex` (+ (`self.sequenceIndex`) 1)))
      (switch `int` _output_get
        (:`Default`
          (`self.Finish`))
        (:`2`
          (bind _asynctaskproxy (`AsyncRootMovement.AsyncRootMovement_MoveTo` self (`EnemyBrainComponent.GetCharacterMovement` _brain) _returnvalue_2 (`self.dashLoc`) (`KismetMathLibrary.FClamp` (/ (`KismetMathLibrary.Vector_Distance` _returnvalue_2 (`self.dashLoc`)) 5000.0) 0.1 0.5))
            (:`then`
              (`/Engine/EditorBlueprintResources/StandardMacros.IsValid` _asynctaskproxy
                (:`Is Valid`
                  (`PrimitiveComponent.SetCollisionResponseToChannel` _returnvalue "ECC_Pawn" "ECR_Ignore"))
                (:`Is Not Valid`
                  (`self.Finish`))))
            (:`OnComplete`
              (`PrimitiveComponent.SetCollisionResponseToChannel` _returnvalue "ECC_Pawn" "ECR_Block")
              (`self.AdvanceSequence`))
            (:`OnFail`
              (`self.Finish`))
            (:`OnInterrupted`
              (`PrimitiveComponent.SetCollisionResponseToChannel` (`EnemyBrainComponent.GetCapsule` (`self.brain`)) "ECC_Pawn" "ECR_Block")
              (`self.Finish`))))
        (:`3`
          (`EnemyCombatComponent.Attack` (`EnemyBrainComponent.GetEnemyCombatComp` (`self.brain`)) (`self.Atk`)))))
    (:`Is Not Valid`
      (`self.Finish`))))

(event `self.Finish`
  (bind _brain (`self.brain`))
  (bind (_blackboard_targetactor _blackboard_targetdistance _blackboard_targetheightdifference _blackboard_lastknownlocation _blackboard_lastdamagesource _blackboard_homelocation _blackboard_aggro _blackboard_lastattacktime _blackboard_consecutivesequenceuses _blackboard_eqs_actors _blackboard_eqs_locs _blackboard_blockedon _blackboard_bforgottarget) (break `EnemyBlackboard` (`EnemyBrainComponent.blackboard` _brain)))
  (`/Engine/EditorBlueprintResources/StandardMacros.IsValid` _brain
    (:`Is Valid`
      (set `EnemyBrainComponent.blackboard` (make `EnemyBlackboard` _blackboard_targetactor _blackboard_lastknownlocation _blackboard_lastdamagesource _blackboard_homelocation _blackboard_aggro (`KismetSystemLibrary.GetGameTimeInSeconds` self) _blackboard_bforgottarget) _brain))
    (:`Is Not Valid`
      _))
  (`self.FinishHelper`))

(fn `CanExecute`
  (returns (ReturnValue :type Boolean))
  (bind _brain (`self.brain`))
  (return (and (`parent.CanExecute`) (`KismetSystemLibrary.IsValid` (`.TargetActor` (break `EnemyBlackboard` (`EnemyBrainComponent.blackboard` _brain)))) (`KismetSystemLibrary.IsValid` (`EnemyBrainComponent.GetEnemyCombatComp` _brain)))))