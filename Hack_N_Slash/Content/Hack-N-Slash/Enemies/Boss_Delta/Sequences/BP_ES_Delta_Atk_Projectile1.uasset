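; Boss Delta enemy sequence for the Projectile1 attack, which makes room by dashing when the target is close.
; Beyond a distance threshold it requests the attack immediately and flags the sequence to finish on the next advance.
; Otherwise it focuses the target and runs an EQS query, then successive advances request a high-speed move to the first result and the attack.
; Brain, state machine, controller and target are validated first, finishing the sequence if any is missing.
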(event `self.Execute`
  (bind _returnvalue (`self.GetBrain`))
  (bind _returnvalue_2 (`self.GetBrain`))
  (bind _blackboard_targetactor (break `EnemyBlackboard` (`EnemyBrainComponent.blackboard` _returnvalue_2)))
  (bind _blackboard_targetactor_2 (break `EnemyBlackboard` (`EnemyBrainComponent.blackboard` _returnvalue)))
  (`self.EnsureReferences`
    (:`Is Valid`
      (if (> (`KismetMathLibrary.Vector_Distance` (`Actor.K2_GetActorLocation` (`ActorComponent.GetOwner` _returnvalue_2)) (`Actor.K2_GetActorLocation` _blackboard_targetactor)) 500.0)
        (set `self.bInterruptible` false)
        (`StateMachineComponent.RequestAttackEnemy` (`EnemyBrainComponent.GetStateMachine` (`self.GetBrain`)) (`self.Atk`))
        (set `self.FinishEarly?` true)
        (else
          (`self.FindDashLoc`)
          (`EnemyController.SetFocusHNS` (`EnemyBrainComponent.GetEnemyController` _returnvalue) _blackboard_targetactor_2))))
    (:`Is Not Valid`
      (`self.Finish`))))

(event `self.AdvanceSequence`
  (`self.EnsureReferences`
    (:`Is Valid`
      (`self.FinishEarly?`
        (:`then`
          (set `self.FinishEarly?` false)
          (`self.Finish`))
        (:`else`
          (bind _output_get (set `self.sequenceIndex` (+ (`self.sequenceIndex`) 1)))
          (switch `int` _output_get
            (:`Default`
              (`self.Finish`))
            (:`2`
              (set `self.bInterruptible` false)
              (`self.SetWalkSpeedAndAcceleration` 9000.0 10000.0)
              (bind _dashlocvalid_ (`self.Dash`))
              (if (not _dashlocvalid_)
                (`self.Finish`)))
            (:`3`
              (`StateMachineComponent.RequestAttackEnemy` (`EnemyBrainComponent.GetStateMachine` (`self.GetBrain`)) (`self.Atk`)))))))
    (:`Is Not Valid`
      (`self.Finish`))))

(fn `Dash`
  (returns (`DashLocValid?` :type Boolean))
  (bind _returnvalue (`self.GetBrain`))
  (bind (_targetactor _lastknownlocation _lastdamagesource _homelocation _eqs_actors _eqs_locs) (break `EnemyBlackboard` (`EnemyBrainComponent.blackboard` _returnvalue)))
  (`StateMachineComponent.RequestMoveTo` (`EnemyBrainComponent.GetStateMachine` _returnvalue) null (`|GetArrayItem` _eqs_locs) 100.0)
  (return (`KismetArrayLibrary.Array_IsEmpty` _eqs_locs)))

(fn `FindDashLoc`
  (`EnemyController.RunEQSQueryHNS` (`EnemyBrainComponent.GetEnemyController` (`self.GetBrain`)) null (`|MakeMap` "None" :!type "Name" :!valuetype "Float (single-precision)") "RandomBest5Pct"))