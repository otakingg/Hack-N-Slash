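; Boss Delta enemy attack sequence that zips the boss through up to three high-speed dashes while focused on its target, then requests a close or far attack by distance.
; An indexed AdvanceSequence cycles EQS query, move and random timed pause.
; The query's scoring parameters flip with target distance, favoring far spots when close and close spots when far.
; Finish clears focus, resets the sequence and starts any cooldown.
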(event `self.Execute`
  (bind _returnvalue (`self.GetBrain`))
  (bind _blackboard_targetactor (break `EnemyBlackboard` (`EnemyBrainComponent.blackboard` _returnvalue)))
  (`self.EnsureReferences`
    (:`Is Valid`
      (set `self.bInterruptible` false)
      (`self.FindDashLoc`)
      (`EnemyController.SetFocusHNS` (`EnemyBrainComponent.GetEnemyController` _returnvalue) _blackboard_targetactor)
      (`self.SetWalkSpeedAndAcceleration` 9000.0 10000.0))
    (:`Is Not Valid`
      (`self.Finish`))))

(event `self.AdvanceSequence`
  (bind _returnvalue (`self.GetBrain`))
  (bind (_blackboard_targetactor _blackboard_targetdistance) (break `EnemyBlackboard` (`EnemyBrainComponent.blackboard` (`self.GetBrain`))))
  (`self.EnsureReferences`
    (:`Is Valid`
      (`PrimitiveComponent.SetCollisionResponseToChannel` (`EnemyBrainComponent.GetCapsuleComponent` (`self.GetBrain`)) "ECC_Pawn" "ECR_Block")
      (bind _output_get (set `self.sequenceIndex` (+ (`self.sequenceIndex`) 1)))
      (switch `int` _output_get
        (:`Default`
          (`self.Finish`))
        (:`2`
          (bind _dashlocvalid_ (`self.Dash` :!label _label))
          (if _dashlocvalid_
            (`PrimitiveComponent.SetCollisionResponseToChannel` (`EnemyBrainComponent.GetCapsuleComponent` (`self.GetBrain`)) "ECC_Pawn" "ECR_Ignore")
            (else
              (`self.Finish`))))
        (:`3`
          (bind _returnvalue_2 (`KismetSystemLibrary.K2_SetTimer` null "Advance Sequence" (`KismetMathLibrary.RandomFloatInRange` 0.2 1.0) :!label _label_2))
          (set `self.TH_AdvSeq` _returnvalue_2))
        (:`4`
          (`self.FindDashLoc` :!label _label_3))
        (:`5`
          (goto _label))
        (:`6`
          (goto _label_2))
        (:`7`
          (goto _label_3))
        (:`8`
          (goto _label))
        (:`9`
          (`AIController.K2_ClearFocus` (`EnemyBrainComponent.GetEnemyController` _returnvalue))
          (`StateMachineComponent.RequestAttackEnemy` (`EnemyBrainComponent.GetStateMachine` _returnvalue) (select `bool` (> _blackboard_targetdistance 300.0) :`false` (`self.atkClose`) :`true` (`self.atkFar`))))))
    (:`Is Not Valid`
      (`self.Finish`))))

(event `self.Finish`
  (`self.EnsureReferences`
    (:`Is Valid`
      (`AIController.K2_ClearFocus` (`EnemyBrainComponent.GetEnemyController` (`self.GetBrain`))))
    (:`Is Not Valid`
      _))
  (`KismetSystemLibrary.K2_ClearAndInvalidateTimerHandle` self (`self.TH_AdvSeq`))
  (if (> (`self.cooldown`) 0.0)
    (set `self.bOnCooldown` true)
    (`KismetSystemLibrary.K2_ClearAndInvalidateTimerHandle` self (`self.TH_Cooldown`))
    (bind _returnvalue (`KismetSystemLibrary.K2_SetTimer` self "EndCooldown" (`self.cooldown`)))
    (set `self.TH_Cooldown` _returnvalue))
  (set `self.sequenceIndex` 1)
  (set `self.bInterruptible` true))

(fn `Dash`
  (returns (`dashLocValid?` :type Boolean))
  (bind _returnvalue (`self.GetBrain`))
  (bind (_targetactor _targetdistance _lastknownlocation _lastdamagesource _homelocation _aggro _eqs_actors _eqs_locs) (break `EnemyBlackboard` (`EnemyBrainComponent.blackboard` _returnvalue)))
  (`StateMachineComponent.RequestMoveTo` (`EnemyBrainComponent.GetStateMachine` _returnvalue) null (`|GetArrayItem` _eqs_locs) 100.0)
  (return (`KismetArrayLibrary.Array_IsEmpty` _eqs_locs)))

(fn `FindDashLoc`
  (locals (params :type "Map of Name to Float (single-precision)"))
  (bind _params (`local.params`))
  (bind _params_2 (`local.params`))
  (bind (_blackboard_targetactor _blackboard_targetdistance) (break `EnemyBlackboard` (`EnemyBrainComponent.blackboard` (`self.GetBrain`))))
  (if (<= _blackboard_targetdistance 500.0)
    (`BlueprintMapLibrary.Map_Add` _params_2 "Distance.Lesser.ScoringFactor")
    (`BlueprintMapLibrary.Map_Add` _params_2 "Distance.Greater.ScoringFactor" 1.0)
    (else
      (`BlueprintMapLibrary.Map_Add` _params "Distance.Lesser.ScoringFactor" 1.0)
      (`BlueprintMapLibrary.Map_Add` _params "Distance.Greater.ScoringFactor")))
  (`EnemyController.RunEQSQueryHNS` (`EnemyBrainComponent.GetEnemyController` (`self.GetBrain`)) "/Game/Hack-N-Slash/Enemies/EnvQuery/QueryTarget/EQ_FarIfTargetClose_CloseIfTargetFar.EQ_FarIfTargetClose_CloseIfTargetFar" (`local.params`) "RandomBest25Pct"))