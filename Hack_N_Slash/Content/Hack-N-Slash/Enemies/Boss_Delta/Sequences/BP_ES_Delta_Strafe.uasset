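; Boss Delta's Strafe enemy sequence, which repositions the boss at a set walk speed while keeping focus on its target.
; An EQS query picks the spot, flipping its distance scoring depending on whether the target is near or far.
; EQS and move-completion callbacks advance the steps from query to move to a short random wait.
; Finish then starts any cooldown and removes the sequence from the enemy's brain.
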(event `self.Execute`
  (bind _returnvalue (`self.GetBrain`))
  (bind _blackboard_targetactor (break `EnemyBlackboard` (`EnemyBrainComponent.blackboard` _returnvalue)))
  (`self.EnsureReferences`
    (:`Is Valid`
      (set `self.bInterruptible` true)
      (`EnemyController.SetFocusHNS` (`EnemyBrainComponent.GetEnemyController` _returnvalue) _blackboard_targetactor)
      (`self.SetWalkSpeedAndAcceleration` 150.0 4000.0)
      (`self.FindStrafeLoc`))
    (:`Is Not Valid`
      (`self.Finish`))))

(event `self.HandleEQSFinished`
  (params (Result :type "EnvQueryResult Structure (by ref)"))
  (`self.AdvanceSequence`))

(event `self.HandleMoveCompleted`
  (params (RequestID :type Integer) (Result :type "EPathFollowingResult Enum" :default "Success"))
  (`self.AdvanceSequence`))

(event `self.AdvanceSequence`
  (`self.EnsureReferences`
    (:`Is Valid`
      (bind _output_get (set `self.sequenceIndex` (+ (`self.sequenceIndex`) 1)))
      (switch `int` _output_get
        (:`2`
          (bind _locsempty_ (`self.Move`))
          (if _locsempty_
            (`KismetSystemLibrary.PrintString` null "Enemy Delta Sequence: Strafe: Move Location invalid")
            (`self.Finish`)))
        (:`3`
          (bind _returnvalue (`KismetSystemLibrary.K2_SetTimer` null "Finish" (`KismetMathLibrary.RandomFloatInRange` 0.0 2.0)))
          (set `self.TH_Finish` _returnvalue)
          (`KismetSystemLibrary.PrintString` null "Enemy Delta Strafe: Waiting"))))
    (:`Is Not Valid`
      (`self.Finish`))))

(event `self.Finish`
  (`/Engine/EditorBlueprintResources/StandardMacros.IsValid` (`self.GetBrain`)
    (:`Is Valid`
      (`KismetSystemLibrary.K2_ClearTimer` null "Finish")
      (if (> (`self.cooldown`) 0.0)
        (set `self.bOnCooldown` true)
        (`KismetSystemLibrary.K2_ClearTimer` null "EndCooldown")
        (bind _returnvalue (`KismetSystemLibrary.K2_SetTimer` null "EndCooldown" (`self.cooldown`)))
        (set `self.TH_Cooldown` _returnvalue))
      (set `self.sequenceIndex` 1)
      (set `self.bInterruptible` false)
      (`EnemyBrainComponent.RemoveActiveSequence` (`self.GetBrain`)))))

(fn `CanExecute`
  (returns (ReturnValue :type Boolean))
  (bind _blackboard_targetactor (break `EnemyBlackboard` (`EnemyBrainComponent.blackboard` (`self.GetBrain`))))
  (return (and (`parent.CanExecute`) (`KismetSystemLibrary.IsValid` _blackboard_targetactor))))

(fn `FindStrafeLoc`
  (locals (Params :type "Map of Name to Float (single-precision)"))
  (bind _params (`local.Params`))
  (bind _params_2 (`local.Params`))
  (bind (_blackboard_targetactor _blackboard_targetdistance) (break `EnemyBlackboard` (`EnemyBrainComponent.blackboard` (`self.GetBrain`))))
  (if (<= _blackboard_targetdistance 500.0)
    (`BlueprintMapLibrary.Map_Add` _params_2 "Distance.Lesser.ScoringFactor")
    (`BlueprintMapLibrary.Map_Add` _params_2 "Distance.Greater.ScoringFactor" 1.0)
    (else
      (`BlueprintMapLibrary.Map_Add` _params "Distance.Lesser.ScoringFactor" 1.0)
      (`BlueprintMapLibrary.Map_Add` _params "Distance.Greater.ScoringFactor")))
  (`EnemyController.RunEQSQueryHNS` (`EnemyBrainComponent.GetEnemyController` (`self.GetBrain`)) "/Game/Hack-N-Slash/Enemies/EnvQuery/QuerySelf/EQ_StrafeSelf.EQ_StrafeSelf" (`local.Params`) "RandomBest5Pct"))

(fn `Move`
  (returns (`LocsEmpty?` :type Boolean))
  (bind _returnvalue (`self.GetBrain`))
  (bind (_targetactor _targetdistance _lastknownlocation _lastdamagesource _homelocation _aggro _timesincelastattack _eqs_actors _eqs_locs) (break `EnemyBlackboard` (`EnemyBrainComponent.blackboard` _returnvalue)))
  (bind _returnvalue_2 (`KismetArrayLibrary.Array_IsEmpty` _eqs_locs))
  (if (not _returnvalue_2)
    (`StateMachineComponent.RequestMoveTo` (`EnemyBrainComponent.GetStateMachine` _returnvalue) null (`|GetArrayItem` _eqs_locs) 10.0))
  (return _returnvalue_2))