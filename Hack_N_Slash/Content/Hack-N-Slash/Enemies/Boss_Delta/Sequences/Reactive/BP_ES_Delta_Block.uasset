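; Reactive enemy sequence that makes the Delta boss block melee hits and retaliate with a revenge attack.
; It runs only with a target, sufficient poise, the boss facing the damager, and no armor breaker.
; Melee hits during the block raise a revenge meter that selects the boss's block-hit montage.
; On advance, a full meter triggers the revenge attack; otherwise the sequence finishes, resetting meter and montage.
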(event `self.Initialize`
  (params (InBrain :type "EnemyBrainComponent Object Reference"))
  (bind _returnvalue (`ActorComponent.GetOwner` InBrain))
  (`parent.Initialize` InBrain)
  (`/Engine/EditorBlueprintResources/StandardMacros.IsValid` InBrain
    (:`Is Valid`
      (bind _asbp_enemy_delta (cast `/Game/Hack-N-Slash/Enemies/Boss_Delta/BP_Enemy_Delta` _returnvalue))
      (set `self.Delta` _asbp_enemy_delta)
      (set `self.EnemyCombat` (`Actor.GetComponentByClass` _returnvalue "/Script/Hack_N_Slash.EnemyCombatComponent"))
      (set `self.CombatRes` (`Actor.GetComponentByClass` _returnvalue "/Script/Hack_N_Slash.CombatResolutionComponent")))))

(event `self.Execute`
  (`self.Is Active?`
    (:`Yes`
      (`self.Ensure References`
        (:`Valid`
          (bind _returnvalue (`EnemyCombatComponent.Block` (`self.EnemyCombat`)))
          (`self.Is Active?`
            (:`Yes`
              (if (not _returnvalue)
                (`self.Finish`)
                (else
                  (set `/Game/Hack-N-Slash/Enemies/Boss_Delta/BP_Enemy_Delta.blockHitMont` (`|GetArrayItem` (`self.BlockHitMonts`) (`self.revengeMeter`)) (`self.Delta`)))))))
        (:`Invalid`
          (`self.Finish`))))))

(event `self.HandleReceiveHitPost`
  (params (HitData :type "AtkHitData Structure (by ref)"))
  (`self.Is Active?`
    (:`Yes`
      (`self.Ensure References`
        (:`Valid`
          (if (`BlueprintGameplayTagLibrary.MatchesTag` (`.attackType` (break `AtkHitData` HitData)) (struct :`TagName` "Attack.Type.Melee"))
            (bind _output_get (set `self.revengeMeter` (`KismetMathLibrary.Clamp` (+ (`self.revengeMeter`) 1) 0 (`self.maxRevenge`))))
            (`self.Is Active?`
              (:`Yes`
                (if (>= _output_get (`self.maxRevenge`))
                  (set `/Game/Hack-N-Slash/Enemies/Boss_Delta/BP_Enemy_Delta.blockHitMont` null (`self.Delta`))
                  (else
                    (set `/Game/Hack-N-Slash/Enemies/Boss_Delta/BP_Enemy_Delta.blockHitMont` (`|GetArrayItem` (`self.BlockHitMonts`) (`self.revengeMeter`)) (`self.Delta`))))))))))))

(event `self.AdvanceSequence`
  (`self.Is Active?`
    (:`Yes`
      (`self.Ensure References`
        (:`Valid`
          (if (< (`self.revengeMeter`) (`self.maxRevenge`))
            (`self.Finish`)
            (else
              (bind _returnvalue (`EnemyCombatComponent.Attack` (`self.EnemyCombat`) (`self.RevengeAtk`)))
              (if _returnvalue
                (set `self.revengeMeter` 0)
                (else
                  (`self.Finish`))))))))))

(event `self.Abort`
  (`parent.Abort`)
  (set `self.revengeMeter` 0 :!label _label)
  (bind _delta (`self.Delta`)
    (:`then`
      (set `/Game/Hack-N-Slash/Enemies/Boss_Delta/BP_Enemy_Delta.blockHitMont` null _delta))
    (:`else`
      _))
  (`parent.Finish`))

(event `self.Finish`
  (goto _label))

(fn `CanExecute`
  (params (HitData :type "AtkHitData Structure (by ref)"))
  (returns (ReturnValue :type Boolean))
  (bind (_attacker _damager _attackmotion _attackreaction _attacktype _barmorbreaker) (break `AtkHitData` (`local.HitData`)))
  (return (and (`parent.CanExecute` HitData) (`KismetSystemLibrary.IsValid` (`.TargetActor` (break `EnemyBlackboard` (`EnemyBrainComponent.blackboard` (`self.brain`))))) (`KismetSystemLibrary.IsValid` (`self.EnemyCombat`)) (`KismetSystemLibrary.IsValid` (`self.CombatRes`)) (> (`CombatResolutionComponent.GetPoiseCalc` (`self.CombatRes`)) -1) (`self.IsFacingTarget` _damager) (`BlueprintGameplayTagLibrary.MatchesTag` _attacktype (struct :`TagName` "Attack.Type.Melee")) (not _barmorbreaker))))