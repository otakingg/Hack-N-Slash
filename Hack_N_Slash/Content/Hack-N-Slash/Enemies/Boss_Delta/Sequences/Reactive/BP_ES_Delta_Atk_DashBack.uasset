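; Reactive enemy sequence for boss Delta that answers a frontal melee hit (dash, leap or stationary) with a back dash and counterattack.
; An EQS query picks the spot, then async root motion moves Delta there hidden, damage-immune and ignoring pawns, with dash FX.
; On arrival it restores that state and attacks, with a jump anim notify adding a forward root-motion leap scaled to target distance.
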(event `self.Initialize`
  (params (InBrain :type "EnemyBrainComponent Object Reference"))
  (`parent.Initialize` InBrain)
  (bind _brain (`self.brain`)
    (:`then`
      (bind _asbp_enemy_delta (cast `/Game/Hack-N-Slash/Enemies/Boss_Delta/BP_Enemy_Delta` (`ActorComponent.GetOwner` _brain)))
      (set `self.Delta` _asbp_enemy_delta))
    (:`else`)))

(event `self.Execute`
  (`self.Is Active?`
    (:`Yes`
      (`self.EnsureReferences`
        (:`Is Valid`
          (`self.SetPoiseCalc` 10)
          (`self.Is Active?`
            (:`Yes`
              (`self.SetDmgImmunity` true)
              (`self.Is Active?`
                (:`Yes`
                  (`EnemyController.ClearFocusHNS` (`EnemyBrainComponent.GetEnemyController` (`self.brain`)))
                  (`self.Is Active?`
                    (:`Yes`
                      (`self.FaceTarget`)
                      (`self.Is Active?`
                        (:`Yes`
                          (`self.FindDashLoc`))))))))))
        (:`Is Not Valid`
          (`self.Finish`))))))

(event `self.HandleEQSFinished`
  (params (Result :type "EnvQueryResult Structure (by ref)"))
  (`self.AdvanceSequence`))

(event `self.AdvanceSequence`
  (bind _returnvalue (`EnemyBrainComponent.GetLocoMotionComp` (`self.brain`)))
  (`self.Is Active?`
    (:`Yes`
      (`self.EnsureReferences`
        (:`Is Valid`
          (bind _output_get (set `self.sequenceIndex` (+ (`self.sequenceIndex`) 1)))
          (switch `int` _output_get
            (:`Default`
              (`self.Finish`))
            (:`2`
              (if (`KismetArrayLibrary.Array_IsEmpty` (`.EQS_Locs` (break `EnemyBlackboard` (`EnemyBrainComponent.blackboard` (`self.brain`)))))
                (`KismetSystemLibrary.PrintString` null "Enemy Delta Sequence: Dash Back Atk: Move Location invalid")
                (`self.SetPoiseCalc` 0)
                (`self.SetDmgImmunity` false)
                (`self.Finish`)
                (else
                  (bind (_asynctaskproxy _rootmovement) (`AsyncRootMovement.AsyncRootMovement_MoveTo` self (`EnemyBrainComponent.GetCharacterMovement` (`self.brain`)) (`Actor.K2_GetActorLocation` (`ActorComponent.GetOwner` (`self.brain`))) (`|GetArrayItem` (`.EQS_Locs` (break `EnemyBlackboard` (`EnemyBrainComponent.blackboard` (`self.brain`))))) (`KismetMathLibrary.FClamp` (/ (`KismetMathLibrary.Vector_Distance` (`Actor.K2_GetActorLocation` (`ActorComponent.GetOwner` (`self.brain`))) (`|GetArrayItem` (`.EQS_Locs` (break `EnemyBlackboard` (`EnemyBrainComponent.blackboard` (`self.brain`)))))) 5000.0) 0.1 0.5))
                    (:`then`
                      (`/Engine/EditorBlueprintResources/StandardMacros.IsValid` _asynctaskproxy
                        (:`Is Valid`
                          (bind _output_get_2 (set `self.RMS_MovTo_Back` _asynctaskproxy))
                          (`LocomotionComponent.AddRootMotionSource` (`EnemyBrainComponent.GetLocoMotionComp` (`self.brain`)) _output_get_2 false)
                          (`self.Is Active?`
                            (:`Yes`
                              (`self.SetMeshVisibility` false)
                              (`self.Is Active?`
                                (:`Yes`
                                  (`self.SetCollChanlResp` "ECC_Pawn")
                                  (`self.Is Active?`
                                    (:`Yes`
                                      (bind _delta (`self.Delta`)
                                        (:`then`
                                          (`/Game/Hack-N-Slash/Enemies/Boss_Delta/BP_Enemy_Delta.ActivateDashFX` _delta))
                                        (:`else`)))))))))
                        (:`Is Not Valid`
                          (`self.Finish`))))
                    (:`OnComplete`
                      (`/Engine/EditorBlueprintResources/StandardMacros.IsValid` _returnvalue
                        (:`Is Valid`
                          (`LocomotionComponent.OnRootMotionComplete` _returnvalue _rootmovement)
                          (set `self.RMS_MovTo_Back` null)
                          (`self.Is Active?`
                            (:`Yes`
                              (`self.SetMeshVisibility` true)
                              (`self.Is Active?`
                                (:`Yes`
                                  (`self.SetCollChanlResp` "ECC_Pawn" "ECR_Block")
                                  (`self.Is Active?`
                                    (:`Yes`
                                      (`self.SetPoiseCalc` 0)
                                      (`self.Is Active?`
                                        (:`Yes`
                                          (`self.SetDmgImmunity` false)
                                          (`self.Is Active?`
                                            (:`Yes`
                                              (bind _delta_2 (`self.Delta`)
                                                (:`then`
                                                  (`/Game/Hack-N-Slash/Enemies/Boss_Delta/BP_Enemy_Delta.DeacticateDashVFX` _delta_2 0.5))
                                                (:`else`
                                                  _))
                                              (`self.AdvanceSequence`))))))))))))))
                    (:`OnFail`
                      (set `self.RMS_MovTo_Back` null)
                      (`self.SetMeshVisibility` true)
                      (`self.SetCollChanlResp` "ECC_Pawn" "ECR_Block")
                      (`self.SetPoiseCalc` 0)
                      (`self.SetDmgImmunity` false)
                      (bind _delta_3 (`self.Delta`)
                        (:`then`
                          (`/Game/Hack-N-Slash/Enemies/Boss_Delta/BP_Enemy_Delta.DeacticateDashVFX` _delta_3 0.0)
                          (`self.Finish`))
                        (:`else`)))
                    (:`OnInterrupted`
                      (set `self.RMS_MovTo_Back` null)
                      (`self.Is Active?`
                        (:`Yes`
                          (bind _brain (`self.brain`)
                            (:`then`
                              (`EnemyBrainComponent.RemoveActiveSequence` _brain false)
                              (`self.Abort`))
                            (:`else`)))))))))
            (:`3`
              (bind _returnvalue_2 (`EnemyCombatComponent.Attack` (`EnemyBrainComponent.GetEnemyCombatComp` (`self.brain`)) (`self.Atk`)))
              (if (not _returnvalue_2)
                (`self.Finish`)))))
        (:`Is Not Valid`
          (`self.Finish`))))))

(event `self.HandleAnimNotify`
  (params (NotifyTag :type "GameplayTag Structure (by ref)"))
  (bind _returnvalue (`EnemyBrainComponent.GetLocoMotionComp` (`self.brain`)))
  (`parent.HandleAnimNotify` NotifyTag)
  (`self.Is Active?`
    (:`Yes`
      (if (`BlueprintGameplayTagLibrary.MatchesTag` NotifyTag (struct :`TagName` "NotifyEvent.EnemyBrain.Jump") true)
        (bind (_asynctaskproxy _rootmovement) (`AsyncRootMovement.AsyncRootMovement_JumpForce` self (`EnemyBrainComponent.GetCharacterMovement` (`self.brain`)) (`Actor.GetActorForwardVector` (`ActorComponent.GetOwner` (`self.brain`))) (`KismetMathLibrary.FClamp` (`self.GetJumpDistance`) 300.0 800.0) 400.0)
          (:`then`
            (`/Engine/EditorBlueprintResources/StandardMacros.IsValid` _asynctaskproxy
              (:`Is Valid`
                (`LocomotionComponent.AddRootMotionSource` _returnvalue _asynctaskproxy true))))
          (:`OnComplete`
            (`/Engine/EditorBlueprintResources/StandardMacros.IsValid` _returnvalue
              (:`Is Valid`
                (`LocomotionComponent.OnRootMotionComplete` _returnvalue _rootmovement)))))))))

(event `self.Abort`
  (`parent.Abort`)
  (`self.ClearRootMotSrc` (`self.RMS_MovTo_Back`)))

(event `self.Finish`
  (bind _brain (`self.brain`))
  (bind (_targetactor _targetdistance _targetheightdifference _lastknownlocation _lastdamagesource _homelocation _aggro _lastattacktime _eqs_actors _eqs_locs _blockedon _bforgottarget) (break `EnemyBlackboard` (`EnemyBrainComponent.blackboard` _brain)))
  (`self.Is Active?`
    (:`Yes`
      (`/Engine/EditorBlueprintResources/StandardMacros.IsValid` _brain
        (:`Is Valid`
          (set `EnemyBrainComponent.blackboard` (make `EnemyBlackboard` _targetactor _lastknownlocation _lastdamagesource _homelocation _aggro (`KismetSystemLibrary.GetGameTimeInSeconds` self) _bforgottarget) (`self.brain`))
          (`parent.Finish`))))))

(fn `CanExecute`
  (params (HitData :type "AtkHitData Structure (by ref)"))
  (returns (ReturnValue :type Boolean))
  (locals (Distance :type "Float (double-precision)" :default 0.0))
  (bind _brain (`self.brain`))
  (`/Engine/EditorBlueprintResources/StandardMacros.IsValid` (`.damager` (break `AtkHitData` (`local.HitData`)))
    (:`Is Valid`
      (if (and (`parent.CanExecute` (`local.HitData`)) (`KismetSystemLibrary.IsValid` (`.TargetActor` (break `EnemyBlackboard` (`EnemyBrainComponent.blackboard` _brain)))) (`KismetSystemLibrary.IsValid` (`EnemyBrainComponent.GetEnemyCombatComp` _brain)) (`KismetSystemLibrary.IsValid` (`EnemyBrainComponent.GetLocoMotionComp` _brain)) (`KismetSystemLibrary.IsValid` (`EnemyBrainComponent.GetCombatResComp` _brain)) (not (< (`CombatResolutionComponent.GetPoiseCalc` (`EnemyBrainComponent.GetCombatResComp` _brain)) 0)) (`self.IsFacingTarget` (`.damager` (break `AtkHitData` (`local.HitData`))) 0.7))
        (`|SwitchGameplayTag` (`.attackType` (break `AtkHitData` (`local.HitData`)))
          (:`Default`
            _)
          (:`Attack.Type.AOE`
            _)
          (:`Attack.Type.Melee`
            (`|SwitchGameplayTag` (`.attackMotion` (break `AtkHitData` (`local.HitData`)))
              (:`Default`
                _)
              (:`Attack.Motion.Dash`
                (return true))
              (:`Attack.Motion.Leap`
                (return true))
              (:`Attack.Motion.Stationary`
                (return true))
              (:`Attack.Motion.Teleport`
                _))
            (return false))
          (:`Attack.Type.Projectile`
            _))
        (return false)
        (else
          (return false))))
    (:`Is Not Valid`
      (return false))))

(fn `ClearRootMotSrc`
  (params (RootMotSrc :type "AsyncRootMovement Object Reference"))
  (bind _brain (`self.brain`)
    (:`then`
      (bind _returnvalue (`EnemyBrainComponent.GetLocoMotionComp` _brain))
      (`/Engine/EditorBlueprintResources/StandardMacros.IsValid` _returnvalue
        (:`Is Valid`
          (`LocomotionComponent.ClearRootMotionSource` _returnvalue (`local.RootMotSrc`)))))
    (:`else`)))

(fn `FaceTarget`
  (bind _returnvalue (`ActorComponent.GetOwner` (`self.brain`)))
  (bind _brain (`self.brain`)
    (:`then`
      (bind _targetactor (break `EnemyBlackboard` (`EnemyBrainComponent.blackboard` _brain)))
      (`/Engine/EditorBlueprintResources/StandardMacros.IsValid` _targetactor
        (:`Is Valid`
          (`/Engine/EditorBlueprintResources/StandardMacros.IsValid` _returnvalue
            (:`Is Valid`
              (`Actor.K2_SetActorRotation` (`ActorComponent.GetOwner` (`self.brain`)) (`KismetMathLibrary.MakeRotator` 0.0 0.0 (.yaw (`KismetMathLibrary.FindLookAtRotation` (`Actor.K2_GetActorLocation` _returnvalue) (`Actor.K2_GetActorLocation` _targetactor)))) false))))))
    (:`else`)))

(fn `FindDashLoc`
  (`EnemyController.RunEQSQueryHNS` (`EnemyBrainComponent.GetEnemyController` (`self.brain`)) "/Game/Hack-N-Slash/EnvQuery/QuerySelf/EQ_Self_GetBack.EQ_Self_GetBack" (`|MakeMap`) "RandomBest25Pct"))

(fn `GetJumpDistance`
  (returns (Distance :type "Float (double-precision)"))
  (bind _brain (`self.brain`))
  (return (`KismetMathLibrary.Vector_Distance` (`LocomotionComponent.CalcWarpLocRot` (`EnemyBrainComponent.GetLocoMotionComp` _brain) (`.TargetActor` (break `EnemyBlackboard` (`EnemyBrainComponent.blackboard` _brain))) 0.0 0.0 0.0 true true false false) (`Actor.K2_GetActorLocation` (`ActorComponent.GetOwner` (`self.brain`))))))

(fn `SetCollChanlResp`
  (params (Channel :type "ECollisionChannel Enum" :default "ECC_WorldStatic") (Response :type "ECollisionResponse Enum" :default "ECR_Ignore"))
  (bind _brain (`self.brain`)
    (:`then`
      (bind _returnvalue (`EnemyBrainComponent.GetCapsule` _brain))
      (`/Engine/EditorBlueprintResources/StandardMacros.IsValid` _returnvalue
        (:`Is Valid`
          (`PrimitiveComponent.SetCollisionResponseToChannel` _returnvalue (`local.Channel`) (`local.Response`)))))
    (:`else`)))

(fn `SetDmgImmunity`
  (params (`Immune?` :type Boolean))
  (bind _returnvalue (`EnemyBrainComponent.GetStatsComp` (`self.brain`)))
  (`/Engine/EditorBlueprintResources/StandardMacros.IsValid` _returnvalue
    (:`Is Valid`
      (`StatsComponent.SetDmgImmunity` _returnvalue `Immune?`))))

(fn `SetMeshVisibility`
  (params (`Visible?` :type Boolean))
  (bind _brain (`self.brain`)
    (:`then`
      (bind _returnvalue (`EnemyBrainComponent.GetMesh` _brain))
      (`/Engine/EditorBlueprintResources/StandardMacros.IsValid` _returnvalue
        (:`Is Valid`
          (`SceneComponent.SetVisibility` _returnvalue (`local.Visible?`) true))))
    (:`else`)))

(fn `SetPoiseCalc`
  (params (Poise :type Integer))
  (bind _returnvalue (`EnemyBrainComponent.GetCombatResComp` (`self.brain`)))
  (`/Engine/EditorBlueprintResources/StandardMacros.IsValid` _returnvalue
    (:`Is Valid`
      (`CombatResolutionComponent.SetPoiseCalc` _returnvalue Poise))))