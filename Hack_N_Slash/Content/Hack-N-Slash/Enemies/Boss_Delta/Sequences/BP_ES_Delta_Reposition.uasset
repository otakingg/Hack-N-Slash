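; Boss Delta enemy sequence that quickly dashes the boss to a new position relative to its target.
; An EQS query, weighted by target distance, favors far spots when the target is close and near spots when it is far.
; The finished query triggers a short async root-motion move with Pawn collision ignored, then a brief random wait before finishing.
; Invalid references, missing locations or failed moves end the sequence early.
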(event `self.Execute`
  (bind _returnvalue (`self.GetBrain`))
  (bind _blackboard_targetactor (break `EnemyBlackboard` (`EnemyBrainComponent.blackboard` _returnvalue)))
  (`self.EnsureReferences`
    (:`Is Valid`
      (`EnemyController.SetFocusHNS` (`EnemyBrainComponent.GetEnemyController` _returnvalue) _blackboard_targetactor)
      (`self.FindReposLoc`))
    (:`Is Not Valid`
      (`self.Finish`))))

(event `self.HandleEQSFinished`
  (params (Result :type "EnvQueryResult Structure (by ref)"))
  (`self.AdvanceSequence`))

(event `self.AdvanceSequence`
  (bind _returnvalue (`self.GetBrain`))
  (bind _returnvalue_2 (`EnemyBrainComponent.GetCapsuleComponent` (`self.GetBrain`)))
  (bind _returnvalue_3 (`Actor.K2_GetActorLocation` (`ActorComponent.GetOwner` _returnvalue)))
  (bind _output (`|GetArrayItem` (`.EQS_Locs` (break `EnemyBlackboard` (`EnemyBrainComponent.blackboard` _returnvalue)))))
  (`self.EnsureReferences`
    (:`Is Valid`
      (bind _output_get (set `self.sequenceIndex` (+ (`self.sequenceIndex`) 1)))
      (switch `int` _output_get
        (:`Default`
          (`self.Finish`))
        (:`2`
          (if (`KismetArrayLibrary.Array_IsEmpty` (`.EQS_Locs` (break `EnemyBlackboard` (`EnemyBrainComponent.blackboard` _returnvalue))))
            (`KismetSystemLibrary.PrintString` null "Enemy Delta Sequence: Reposition: Move Location invalid")
            (`self.Finish`)
            (else
              (bind _asynctaskproxy (`AsyncRootMovement.AsyncRootMovement_MoveTo` self (`EnemyBrainComponent.GetCharacterMovement` _returnvalue) _returnvalue_3 _output (`KismetMathLibrary.FClamp` (/ (`KismetMathLibrary.Vector_Distance` _returnvalue_3 _output) 5000.0) 0.1 0.5))
                (:`then`
                  (`/Engine/EditorBlueprintResources/StandardMacros.IsValid` _asynctaskproxy
                    (:`Is Valid`
                      (`PrimitiveComponent.SetCollisionResponseToChannel` _returnvalue_2 "ECC_Pawn" "ECR_Ignore"))
                    (:`Is Not Valid`
                      (`self.Finish`))))
                (:`OnComplete`
                  (`PrimitiveComponent.SetCollisionResponseToChannel` _returnvalue_2 "ECC_Pawn" "ECR_Block")
                  (`self.AdvanceSequence`))
                (:`OnFail`
                  (`self.Finish`))
                (:`OnInterrupted`
                  (`PrimitiveComponent.SetCollisionResponseToChannel` (`EnemyBrainComponent.GetCapsuleComponent` (`self.GetBrain`)) "ECC_Pawn" "ECR_Block")
                  (`self.Finish`))))))
        (:`3`
          (bind _returnvalue_4 (`KismetSystemLibrary.K2_SetTimer` null "Finish" (`KismetMathLibrary.RandomFloatInRange` 1.0 1.5)))
          (set `self.TH_Finish` _returnvalue_4)
          (`KismetSystemLibrary.PrintString` null "Enemy Delta Reposition: Waiting"))))
    (:`Is Not Valid`
      (`self.Finish`))))

(fn `CanExecute`
  (returns (ReturnValue :type Boolean))
  (bind _blackboard_targetactor (break `EnemyBlackboard` (`EnemyBrainComponent.blackboard` (`self.GetBrain`))))
  (return (and (`parent.CanExecute`) (`KismetSystemLibrary.IsValid` _blackboard_targetactor))))

(fn `FindReposLoc`
  (locals (params :type "Map of Name to Float (single-precision)"))
  (bind _params (`local.params`))
  (bind _params_2 (`local.params`))
  (bind (_blackboard_targetactor _blackboard_targetdistance) (break `EnemyBlackboard` (`EnemyBrainComponent.blackboard` (`self.GetBrain`))))
  (if (<= _blackboard_targetdistance 500.0)
    (`BlueprintMapLibrary.Map_Add` _params_2 "Distance.Lesser.ScoringFactor")
    (`BlueprintMapLibrary.Map_Add` _params_2 "Distance.Greater.ScoringFactor" 1.0)
    (else
      (`BlueprintMapLibrary.Map_Add` _params "Distance.Lesser.ScoringFactor" 1.0)
      (`BlueprintMapLibrary.Map_Add` _params "Distance.Greater.ScoringFactor")))
  (`EnemyController.RunEQSQueryHNS` (`EnemyBrainComponent.GetEnemyController` (`self.GetBrain`)) "/Game/Hack-N-Slash/Enemies/EnvQuery/QueryTarget/EQ_FarIfTargetClose_CloseIfTargetFar.EQ_FarIfTargetClose_CloseIfTargetFar" (`local.params`) "RandomBest25Pct"))