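; Boss Delta's gap-closer attack sequence, which dashes the boss toward its blackboard target.
; Execute focuses the target and requests the attack, then anim notifies toggle focus, trigger the dash and end the sequence.
; FindDashLoc steps capsule-width probes toward an offset from the target, keeping the furthest unblocked spot with ground beneath.
; An async root-movement move, timed by distance, performs the dash while the capsule ignores Pawn collision.
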(event `self.Execute`
  (bind _returnvalue (`self.GetBrain`))
  (bind _blackboard_targetactor (break `EnemyBlackboard` (`EnemyBrainComponent.blackboard` _returnvalue)))
  (`self.EnsureReferences`
    (:`Is Valid`
      (`EnemyController.SetFocusHNS` (`EnemyBrainComponent.GetEnemyController` _returnvalue) _blackboard_targetactor)
      (`StateMachineComponent.RequestAttackEnemy` (`EnemyBrainComponent.GetStateMachine` (`self.GetBrain`)) (`self.Atk`)))
    (:`Is Not Valid`
      (`self.Finish`))))

(event `self.HandleAnimNotify`
  (params (NotifyTag :type "GameplayTag Structure"))
  (bind _returnvalue (`self.GetBrain`))
  (bind _returnvalue_2 (`EnemyBrainComponent.GetEnemyController` _returnvalue))
  (bind _returnvalue_3 (`EnemyBrainComponent.GetCapsuleComponent` (`self.GetBrain`)))
  (bind _blackboard_targetactor (break `EnemyBlackboard` (`EnemyBrainComponent.blackboard` _returnvalue)))
  (`|SwitchGameplayTag` NotifyTag
    (:`Notify.EnemyBrain.ClearFocus`
      (`AIController.K2_ClearFocus` _returnvalue_2))
    (:`Notify.EnemyBrain.SetFocus`
      (`EnemyController.SetFocusHNS` _returnvalue_2 _blackboard_targetactor))
    (:`Notify.EnemyBrain.Dash`
      (`self.EnsureReferences`
        (:`Is Valid`
          (bind _output_get (set `self.startLoc` (`Actor.K2_GetActorLocation` (`ActorComponent.GetOwner` _returnvalue))))
          (bind _output_get_2 (set `self.dashLoc` (`self.FindDashLoc` _output_get)))
          (if (== _output_get_2 (`self.startLoc`) :`ErrorTolerance` 100.0)
            (`KismetSystemLibrary.PrintString` self "Delta Gap Closer: Dash Loc is nearly equal to start loc")
            (`self.Finish`)
            (else
              (bind _asynctaskproxy (`AsyncRootMovement.AsyncRootMovement_MoveTo` self (`EnemyBrainComponent.GetCharacterMovement` (`self.GetBrain`)) (`self.startLoc`) (`self.dashLoc`) (`KismetMathLibrary.FClamp` (/ (`KismetMathLibrary.Vector_Distance` (`self.dashLoc`) (`self.startLoc`)) 5000.0) 0.1 0.5))
                (:`then`
                  (`/Engine/EditorBlueprintResources/StandardMacros.IsValid` _asynctaskproxy
                    (:`Is Valid`
                      (`PrimitiveComponent.SetCollisionResponseToChannel` _returnvalue_3 "ECC_Pawn" "ECR_Ignore"))
                    (:`Is Not Valid`
                      (`self.Finish`))))
                (:`OnComplete`
                  (`PrimitiveComponent.SetCollisionResponseToChannel` _returnvalue_3 "ECC_Pawn" "ECR_Block"))
                (:`OnFail`
                  (`self.Finish`))
                (:`OnInterrupted`
                  (`PrimitiveComponent.SetCollisionResponseToChannel` (`EnemyBrainComponent.GetCapsuleComponent` (`self.GetBrain`)) "ECC_Pawn" "ECR_Block")
                  (`self.Finish`))))))
        (:`Is Not Valid`
          (`self.Finish`))))
    (:`Notify.EnemyBrain.AdvanceSequence`
      (`self.AdvanceSequence`))))

(event `self.AdvanceSequence`
  (`self.Finish`))

(fn `CanExecute`
  (returns (ReturnValue :type Boolean))
  (bind _blackboard_targetactor (break `EnemyBlackboard` (`EnemyBrainComponent.blackboard` (`self.GetBrain`))))
  (return (and (`parent.CanExecute`) (`KismetSystemLibrary.IsValid` _blackboard_targetactor))))

(fn `FindDashLoc`
  (params (startLoc :type "Vector Structure"))
  (returns (dashLoc :type "Vector Structure"))
  (locals (diameter :type "Float (single-precision)" :default 0.0) (capsueCount :type Integer) (desiredLoc :type "Vector Structure") (bestLoc :type "Vector Structure") (dashDir :type "Vector Structure" :default (0.0 0.0 0.0)) (testLoc :type "Vector Structure"))
  (bind _returnvalue (`self.GetBrain`))
  (bind _blackboard_targetactor (break `EnemyBlackboard` (`EnemyBrainComponent.blackboard` _returnvalue)))
  (bind _returnvalue_2 (`Actor.K2_GetActorLocation` _blackboard_targetactor))
  (bind (_outradius _outhalfheight) (`CapsuleComponent.GetUnscaledCapsuleSize` (`EnemyBrainComponent.GetCapsuleComponent` (`self.GetBrain`))))
  (bind _returnvalue_3 (`KismetMathLibrary.Normal` (- _returnvalue_2 (`local.startLoc`))))
  (set `local.bestLoc` startLoc)
  (set `local.diameter` (* (`CapsuleComponent.CapsuleRadius` (`EnemyBrainComponent.GetCapsuleComponent` _returnvalue)) 2.0))
  (set `local.dashDir` _returnvalue_3)
  (set `local.desiredLoc` (+ _returnvalue_2 (* _returnvalue_3 (`self.dashLocOffset`))))
  (bind _output_get (set `local.capsueCount` (/ (`KismetMathLibrary.Vector_Distance` (`local.desiredLoc`) (`local.startLoc`)) (`local.diameter`))))
  (for _ (range (+ _output_get 1))
    (bind _output_get_2 (set `local.testLoc` (+ (`local.bestLoc`) (* (`local.dashDir`) (`local.diameter`)))))
    (bind _outhits (`KismetSystemLibrary.CapsuleTraceMultiForObjects` self _output_get_2 _output_get_2 _outradius _outhalfheight (`|MakeArray` "ObjectTypeQuery1" "ObjectTypeQuery2" "ObjectTypeQuery5" "ObjectTypeQuery6" :!type "EObjectTypeQuery Enum") false (`|MakeArray` (`ActorComponent.GetOwner` _returnvalue)) (select `bool` (`self.bDebug`) :`true` "ForDuration" :!type "EDrawDebugTrace Enum") true (struct :`R` 1.0 :`A` 1.0) (struct :`G` 1.0 :`A` 1.0) 3.0))
    (if (`self.IsValidDashLoc` _outhits (`local.testLoc`))
      (set `local.bestLoc` (`local.testLoc`))))
  (return (`local.bestLoc`)))

(fn `IsValidDashLoc`
  (params (Hits :type "Array of HitResult Structure") (Location :type "Vector Structure"))
  (returns (`Valid?` :type Boolean))
  (bind (_outradius _outhalfheight) (`CapsuleComponent.GetUnscaledCapsuleSize` (`EnemyBrainComponent.GetCapsuleComponent` (`self.GetBrain`))))
  (bind (_outhit _returnvalue) (`KismetSystemLibrary.SphereTraceSingle` self Location (- Location (`KismetMathLibrary.MakeVector` 0.0 0.0 (+ _outhalfheight 200.0))) _outradius "TraceTypeQuery1" false (`|MakeArray` (`ActorComponent.GetOwner` (`self.GetBrain`))) (select `bool` (`self.bDebug`) :`true` "ForDuration" :!type "EDrawDebugTrace Enum") true (struct :`R` 1.0 :`A` 1.0) (struct :`G` 1.0 :`A` 1.0) 3.0))
  (if _returnvalue
    (for _array_element (`local.Hits`)
      (if (`|EnumEquality` (`PrimitiveComponent.GetCollisionResponseToChannel` (`.HitComponent` (`GameplayStatics.BreakHitResult` _array_element)) "ECC_Pawn") "ECR_Block")
        (return false)))
    (return true)
    (else
      (return false))))