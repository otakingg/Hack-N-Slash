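; Enemy sequence for the Delta boss that dashes back from a target at close range, then requests an attack.
; It focuses the target and runs the EQ_GetBack EQS query to pick a landing spot.
; An async root-movement dash, timed by distance, hides the mesh, ignores Pawn collision and plays dash VFX.
; Completion restores these and hands off to the state machine's attack, while failures or interruptions finish the sequence.
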(event `self.Initialize`
  (params (InBrain :type "EnemyBrainComponent Object Reference"))
  (set `self.brain` InBrain)
  (if (and (`self.bStartOnCooldown`) (> (`self.cooldown`) 0.0))
    (set `self.bOnCooldown` true)
    (bind _returnvalue (`KismetSystemLibrary.K2_SetTimer` null "EndCooldown" (`self.cooldown`)))
    (set `self.TH_Cooldown` _returnvalue))
  (bind _brain (`self.brain`)
    (:`then`
      (bind _asbp_enemy_delta (cast `/Game/Hack-N-Slash/Enemies/Boss_Delta/BP_Enemy_Delta` (`ActorComponent.GetOwner` _brain)))
      (set `self.Delta` _asbp_enemy_delta))
    (:`else`)))

(event `self.Execute`
  (bind _returnvalue (`self.GetBrain`))
  (bind _blackboard_targetactor (break `EnemyBlackboard` (`EnemyBrainComponent.blackboard` _returnvalue)))
  (`self.EnsureReferences`
    (:`Is Valid`
      (`EnemyController.SetFocusHNS` (`EnemyBrainComponent.GetEnemyController` _returnvalue) _blackboard_targetactor)
      (`self.FindDashLoc`))
    (:`Is Not Valid`
      (`self.Finish`))))

(event `self.HandleEQSFinished`
  (params (Result :type "EnvQueryResult Structure (by ref)"))
  (`self.AdvanceSequence`))

(event `self.AdvanceSequence`
  (bind _returnvalue (`self.GetBrain`))
  (bind _returnvalue_2 (`self.GetBrain`))
  (bind _returnvalue_3 (`self.GetBrain`))
  (bind _returnvalue_4 (`EnemyBrainComponent.GetMeshComp` _returnvalue_3))
  (bind _returnvalue_5 (`EnemyBrainComponent.GetCapsuleComponent` _returnvalue_3))
  (bind _returnvalue_6 (`Actor.K2_GetActorLocation` (`ActorComponent.GetOwner` _returnvalue)))
  (bind _output (`|GetArrayItem` (`.EQS_Locs` (break `EnemyBlackboard` (`EnemyBrainComponent.blackboard` _returnvalue)))))
  (`self.EnsureReferences`
    (:`Is Valid`
      (bind _output_get (set `self.sequenceIndex` (+ (`self.sequenceIndex`) 1)))
      (switch `int` _output_get
        (:`Default`
          (`self.Finish`))
        (:`2`
          (if (`KismetArrayLibrary.Array_IsEmpty` (`.EQS_Locs` (break `EnemyBlackboard` (`EnemyBrainComponent.blackboard` _returnvalue))))
            (`KismetSystemLibrary.PrintString` null "Enemy Delta Sequence: Reposition: Move Location invalid")
            (`self.Finish`)
            (else
              (bind _asynctaskproxy (`AsyncRootMovement.AsyncRootMovement_MoveTo` self (`EnemyBrainComponent.GetCharacterMovement` _returnvalue) _returnvalue_6 _output (`KismetMathLibrary.FClamp` (/ (`KismetMathLibrary.Vector_Distance` _returnvalue_6 _output) 5000.0) 0.1 0.5))
                (:`then`
                  (`/Engine/EditorBlueprintResources/StandardMacros.IsValid` _asynctaskproxy
                    (:`Is Valid`
                      (`SceneComponent.SetVisibility` _returnvalue_4 false true)
                      (`PrimitiveComponent.SetCollisionResponseToChannel` _returnvalue_5 "ECC_Pawn" "ECR_Ignore")
                      (bind _delta (`self.Delta`)
                        (:`then`
                          (`/Game/Hack-N-Slash/Enemies/Boss_Delta/BP_Enemy_Delta.ActivateDashVFX` _delta))
                        (:`else`)))
                    (:`Is Not Valid`
                      (`self.Finish`))))
                (:`OnComplete`
                  (`SceneComponent.SetVisibility` _returnvalue_4 true true)
                  (`PrimitiveComponent.SetCollisionResponseToChannel` _returnvalue_5 "ECC_Pawn" "ECR_Block")
                  (bind _delta_2 (`self.Delta`)
                    (:`then`
                      (`/Game/Hack-N-Slash/Enemies/Boss_Delta/BP_Enemy_Delta.DeacticateDashVFX` _delta_2 0.5))
                    (:`else`
                      _))
                  (`self.AdvanceSequence`))
                (:`OnFail`
                  (`self.Finish`))
                (:`OnInterrupted`
                  (`SceneComponent.SetVisibility` (`EnemyBrainComponent.GetMeshComp` _returnvalue_2) true true)
                  (`PrimitiveComponent.SetCollisionResponseToChannel` (`EnemyBrainComponent.GetCapsuleComponent` _returnvalue_2) "ECC_Pawn" "ECR_Block")
                  (bind _delta_3 (`self.Delta`)
                    (:`then`
                      (`/Game/Hack-N-Slash/Enemies/Boss_Delta/BP_Enemy_Delta.DeacticateDashVFX` _delta_3 0.5))
                    (:`else`
                      _))
                  (`self.Finish`))))))
        (:`3`
          (`AIController.K2_ClearFocus` (`EnemyBrainComponent.GetEnemyController` _returnvalue))
          (`StateMachineComponent.RequestAttackEnemy` (`EnemyBrainComponent.GetStateMachine` _returnvalue) (`self.Atk`)))))
    (:`Is Not Valid`
      (`self.Finish`))))

(event `self.Finish`
  (bind _returnvalue (`self.GetBrain`))
  (bind (_blackboard_targetactor _blackboard_targetdistance _blackboard_targetheightdifference _blackboard_lastknownlocation _blackboard_lastdamagesource _blackboard_homelocation _blackboard_aggro _blackboard_lastattacktime _blackboard_eqs_actors _blackboard_eqs_locs _blackboard_bforgottarget _blackboard_bstaggered) (break `EnemyBlackboard` (`EnemyBrainComponent.blackboard` _returnvalue)))
  (`/Engine/EditorBlueprintResources/StandardMacros.IsValid` _returnvalue
    (:`Is Valid`
      (set `EnemyBrainComponent.blackboard` (make `EnemyBlackboard` _blackboard_targetactor _blackboard_lastknownlocation _blackboard_lastdamagesource _blackboard_homelocation _blackboard_aggro (`KismetSystemLibrary.GetGameTimeInSeconds` self) _blackboard_bforgottarget _blackboard_bstaggered) _returnvalue))
    (:`Is Not Valid`
      _))
  (`self.FinishHelper`))

(fn `CanExecute`
  (returns (ReturnValue :type Boolean))
  (bind (_blackboard_targetactor _blackboard_targetdistance) (break `EnemyBlackboard` (`EnemyBrainComponent.blackboard` (`self.GetBrain`))))
  (return (and (`parent.CanExecute`) (`KismetSystemLibrary.IsValid` _blackboard_targetactor) (<= _blackboard_targetdistance 300.0))))

(fn `FindDashLoc`
  (`EnemyController.RunEQSQueryHNS` (`EnemyBrainComponent.GetEnemyController` (`self.GetBrain`)) "/Game/Hack-N-Slash/Enemies/EnvQuery/QuerySelf/EQ_GetBack.EQ_GetBack" (`|MakeMap`) "RandomBest25Pct"))