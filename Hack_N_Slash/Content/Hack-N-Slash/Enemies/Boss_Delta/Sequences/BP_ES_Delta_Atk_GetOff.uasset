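; Enemy sequence for Boss Delta's "GetOff" attack, a close-range move against the current target.
; It can execute only when the parent check passes, the target is valid and within close range, and a combat component exists.
; Execution validates references, becomes interruptible, focuses the controller on the target and triggers the attack, finishing early if references are missing.
; Advancing the sequence stamps the current game time into the Brain's blackboard and finishes.
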(event `self.Execute`
  (bind _brain (`self.brain`))
  (`self.EnsureReferences`
    (:`Is Valid`
      (set `self.bInterruptible` true)
      (`EnemyController.SetFocusHNS` (`EnemyBrainComponent.GetEnemyController` _brain) (`.TargetActor` (break `EnemyBlackboard` (`EnemyBrainComponent.blackboard` _brain))))
      (`EnemyCombatComponent.Attack` (`EnemyBrainComponent.GetEnemyCombatComp` (`self.brain`)) (`self.Atk`)))
    (:`Is Not Valid`
      (`self.Finish`))))

(event `self.AdvanceSequence`
  (bind _brain (`self.brain`))
  (bind (_targetactor _targetdistance _targetheightdifference _lastknownlocation _lastdamagesource _homelocation _aggro _lastattacktime _eqs_actors _eqs_locs _blockedon _bforgottarget) (break `EnemyBlackboard` (`EnemyBrainComponent.blackboard` _brain)))
  (`/Engine/EditorBlueprintResources/StandardMacros.IsValid` _brain
    (:`Is Valid`
      (set `EnemyBrainComponent.blackboard` (make `EnemyBlackboard` _targetactor _lastknownlocation _lastdamagesource _homelocation _aggro (`KismetSystemLibrary.GetGameTimeInSeconds` self) _bforgottarget) _brain))
    (:`Is Not Valid`
      _))
  (`self.Finish`))

(fn `CanExecute`
  (returns (ReturnValue :type Boolean))
  (bind _brain (`self.brain`))
  (bind (_targetactor _targetdistance) (break `EnemyBlackboard` (`EnemyBrainComponent.blackboard` _brain)))
  (return (and (`parent.CanExecute`) (`KismetSystemLibrary.IsValid` _targetactor) (<= _targetdistance 400.0) (`KismetSystemLibrary.IsValid` (`EnemyBrainComponent.GetEnemyCombatComp` _brain)))))