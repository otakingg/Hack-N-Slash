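; Delta boss enemy Blueprint that dual-wields katanas and provides dash effects and a giant area attack.
; On BeginPlay it runs parent setup, waits briefly, pauses its brain component, then spawns and attaches a katana to each hand socket.
; Helper functions toggle dash VFX with sound and optional delayed shutoff, and spawn the AOE warning and damage actors at its location.
; Timeline and root-motion movement experiments remain unconnected in the event graph.
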(event `self.ReceiveBeginPlay`
  (`parent.ReceiveBeginPlay`)
  (`KismetSystemLibrary.Delay` 0.5)
  (`EnemyBrainComponent.PauseBrain` (`self.brainComp`))
  (`|ExecutionSequence`
    (:`then_0`
      (bind _returnvalue (`|SpawnActorFromClass` "/Game/Hack-N-Slash/Enemies/Boss_Delta/Weapons/BP_Weapon_Delta_Katana.BP_Weapon_Delta_Katana_C" (`SceneComponent.GetSocketTransform` (`self.Mesh`) "Katana_rSocket" "RTS_World") "Undefined" "MultiplyWithRoot" self self))
      (`self.K2_AttachToComponent` _returnvalue (`self.Mesh`) "Katana_rSocket" "SnapToTarget" "SnapToTarget" "SnapToTarget" true))
    (:`then_1`
      (bind _returnvalue_2 (`|SpawnActorFromClass` "/Game/Hack-N-Slash/Enemies/Boss_Delta/Weapons/BP_Weapon_Delta_Katana.BP_Weapon_Delta_Katana_C" (`SceneComponent.GetSocketTransform` (`self.Mesh`) "Katana_lSocket" "RTS_World") "Undefined" "MultiplyWithRoot" self self))
      (`self.K2_AttachToComponent` _returnvalue_2 (`self.Mesh`) "Katana_lSocket" "SnapToTarget" "SnapToTarget" "SnapToTarget" true))))

(event `EndDashVFX`
  (bind _dashvfx (`self.DashVFX`)
    (:`then`
      (`ActorComponent.Deactivate` _dashvfx))
    (:`else`)))

(fn `ActivateDashFX`
  (`GameplayStatics.PlaySoundAtLocation` "/Game/Hack-N-Slash/Enemies/Boss_Delta/SFX/SQ_SFX_Delta_Dash.SQ_SFX_Delta_Dash" (`self.K2_GetActorLocation`) (struct) 1.0 1.0 0.0 null null null null)
  (bind _dashvfx (`self.DashVFX`)
    (:`then`
      (`ActorComponent.Activate` _dashvfx false))
    (:`else`)))

(fn `DeacticateDashVFX`
  (params (Delay :type "Float (double-precision)"))
  (bind _dashvfx (`self.DashVFX`)
    (:`then`
      (if (`ActorComponent.IsActive` _dashvfx)
        (if (> (`local.Delay`) 0.0)
          (`KismetSystemLibrary.K2_SetTimerDelegate` (`|CreateDelegate` :!event `EndDashVFX`) (`local.Delay`))
          (else
            (`ActorComponent.Deactivate` (`self.DashVFX`))))))
    (:`else`)))

(fn `SpawnGiantAOEAtk`
  (returns (AOE_Atk :type "/Game/Hack-N-Slash/Enemies/Boss_Delta/AOE/BP_AOE_Delta_Atk Object Reference"))
  (bind _returnvalue (`|SpawnActorFromClass` "/Game/Hack-N-Slash/Enemies/Boss_Delta/AOE/BP_AOE_Delta_Atk.BP_AOE_Delta_Atk_C" (`KismetMathLibrary.MakeTransform` (`self.K2_GetActorLocation`)) "Undefined" "MultiplyWithRoot" self 100.0 0.5 1 0.25 1.5 "TraceTypeQuery5" false 0.1 true 1500.0 self self))
  (return _returnvalue))

(fn `SpawnGiantAOEWarning`
  (returns (AOE_Warning :type "/Game/Hack-N-Slash/Enemies/Boss_Delta/AOE/BP_AOE_Delta_Atk_Warning Object Reference"))
  (bind _returnvalue (`|SpawnActorFromClass` "/Game/Hack-N-Slash/Enemies/Boss_Delta/AOE/BP_AOE_Delta_Atk_Warning.BP_AOE_Delta_Atk_Warning_C" (`KismetMathLibrary.MakeTransform` (`self.K2_GetActorLocation`)) "Undefined" "MultiplyWithRoot" self 500.0 4.0 "TraceTypeQuery5" false 0.1 true 1500.0 self self))
  (return _returnvalue))

(fn `UserConstructionScript`
  (`parent.UserConstructionScript`))