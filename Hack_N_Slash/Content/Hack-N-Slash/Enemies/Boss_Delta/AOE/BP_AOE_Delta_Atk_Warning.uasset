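; Warning actor for Boss Delta's giant AOE attack that telegraphs the blast and draws players toward it.
; On spawn it moves below its target, sweeps the player near the owning boss via timeline, then spawns a circle indicator and starts a timer.
; Its sphere applies a radial root-motion pull to unlocked players, cleared on exit or destruction.
; Looping charge sounds ramp volume and pitch over the warning duration, ending with a finish sound.
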(event `self.ReceiveBeginPlay`
  (`parent.ReceiveBeginPlay`)
  (`/Engine/EditorBlueprintResources/StandardMacros.IsValid` (`self.GetOwner`)
    (:`Is Valid`
      (`self.MoveBelowTarget`)
      (bind _asbp_player (cast `/Game/Hack-N-Slash/Player/BP_Player` (`GameplayStatics.GetPlayerCharacter` 0))
        (:`then`
          (bind _lococomp (`Player_Base.locoComp` _asbp_player)
            (:`then`
              (bind (_direction _alpha) (`Timeline|Move Player To Center` :!via `PlayFromStart`)
                (:`Update`
                  (`self.K2_SetActorLocation` _asbp_player (`KismetMathLibrary.VLerp` (`self.K2_GetActorLocation` _asbp_player) (`LocomotionComponent.CalcWarpLocRot` _lococomp (`self.K2_GetActorLocation` (`self.GetOwner`)) 150.0 0.0 true true true false) _alpha) true false))
                (:`Finished`
                  (`self.Spawn Atk Indicator`)
                  (`self.Play Charge Audio`))))
            (:`else`
              (`self.Spawn Atk Indicator` :!label _label)
              (`self.Play Charge Audio`))))
        (:`CastFailed`
          (goto _label))))
    (:`Is Not Valid`
      (`self.K2_DestroyActor`))))

(event `self.Sphere.OnComponentBeginOverlap`
  (params (OverlappedComponent :type "PrimitiveComponent Object Reference") (OtherActor :type "Actor Object Reference") (OtherComp :type "PrimitiveComponent Object Reference") (OtherBodyIndex :type Integer) (bFromSweep :type Boolean) (SweepResult :type "HitResult Structure (by ref)"))
  (bind _asplayer_base (cast `Player_Base` OtherActor))
  (bind _lococomp (`Player_Base.locoComp` _asplayer_base)
    (:`then`
      (set `self.Loco Comp` _lococomp)
      (if (not (`BPFL_Combat.ActorHasTag` _asplayer_base (`BlueprintGameplayTagLibrary.MakeLiteralGameplayTag` (struct :`TagName` "Status.MovementLocked"))))
        (bind (_asynctaskproxy _rootmovement) (`AsyncRootMovement.AsyncRootMovement_RadialForce` (`Character.CharacterMovement` _asplayer_base) (`self.K2_GetActorLocation`) (`self.Radius`) (`self.PullStrength`) -1.0 false null)
          (:`then`
            (bind _output_get (set `self.RootMotion` _asynctaskproxy))
            (`LocomotionComponent.AddRootMotionSource_BP` (`self.Loco Comp`) _output_get true))
          (:`OnComplete`
            (`LocomotionComponent.OnRootMotionComplete` (`self.Loco Comp`) _rootmovement)))))
    (:`else`)))

(event `self.Sphere.OnComponentEndOverlap`
  (params (OverlappedComponent :type "PrimitiveComponent Object Reference") (OtherActor :type "Actor Object Reference") (OtherComp :type "PrimitiveComponent Object Reference") (OtherBodyIndex :type Integer))
  (bind _asplayer_base (cast `Player_Base` OtherActor))
  (bind _lococomp (`Player_Base.locoComp` _asplayer_base)
    (:`then`
      (bind _output_get (set `self.Loco Comp` _lococomp))
      (`LocomotionComponent.ClearRootMotionSource` _output_get (`self.RootMotion`)))
    (:`else`)))

(event `self.ReceiveDestroyed`
  (bind _loco_comp (`self.Loco Comp`)
    (:`then`
      (`LocomotionComponent.ClearRootMotionSource` _loco_comp (`self.RootMotion`)))
    (:`else`
      _))
  (`parent.ReceiveDestroyed`))

(event `Spawn Atk Indicator`
  (bind _returnvalue (`KismetSystemLibrary.K2_SetTimerDelegate` (`|CreateDelegate` :!event `K2_DestroyActor`) (`self.Duration`)))
  (set `self.TH_Destroy` _returnvalue)
  (`|SpawnActorFromClass` "/Game/Hack-N-Slash/Utility/Atk_Indicators/BP_AtkInd_Circle.BP_AtkInd_Circle_C" (`KismetMathLibrary.MakeTransform` (`self.K2_GetActorLocation`) (struct) (* (`KismetMathLibrary.MakeVector` 1.0 1.0 1.0) 6.0)) "Undefined" "MultiplyWithRoot" (`self.GetOwner`) (`self.Duration`) 0.003 (struct :`R` 1.0 :`A` 1.0) (struct :`R` 1.0 :`A` 0.1) (struct :`R` 1.0 :`A` 1.0) (`self.GetInstigator`)))

(event `Play Charge Audio`
  (bind _returnvalue (`GameplayStatics.SpawnSoundAtLocation` "/Game/UltimateCombatFightingSFXBundle/Cues/Superhero_Flight/Flying_Loop_1_Cue.Flying_Loop_1_Cue" (`self.K2_GetActorLocation`) (struct) 1.0 1.0 0.0 null null))
  (bind _output_get (set `self.Wind Audio` _returnvalue))
  (`AudioComponent.SetVolumeMultiplier` _output_get 0.3)
  (`AudioComponent.SetPitchMultiplier` (`self.Wind Audio`) 0.7)
  (bind _returnvalue_2 (`GameplayStatics.SpawnSoundAtLocation` "/Game/Anime_Weap_SFX_Pack/CUEs/Gun/AW_Gun_SKILL_electric_charge_01_LOOP_Cue.AW_Gun_SKILL_electric_charge_01_LOOP_Cue" (`self.K2_GetActorLocation`) (struct) 1.0 1.0 0.0 null null))
  (bind _output_get_2 (set `self.Lasic Audio` _returnvalue_2))
  (`AudioComponent.SetVolumeMultiplier` _output_get_2 0.1)
  (`AudioComponent.SetPitchMultiplier` (`self.Lasic Audio`) 0.5)
  (`TimelineComponent.SetPlayRate` (`self.Charge Over Time`) (/ (`TimelineComponent.GetTimelineLength` (`self.Charge Over Time`)) (`self.Duration`)))
  (bind (_direction _alpha) (`Timeline|Charge Over Time` :!via `PlayFromStart`)
    (:`Update`
      (bind _returnvalue_3 (`KismetMathLibrary.FClamp` (/ _alpha (`self.Duration`))))
      (`AudioComponent.SetVolumeMultiplier` (`self.Wind Audio`) (`KismetMathLibrary.Lerp` 0.3 2.0 _returnvalue_3))
      (`AudioComponent.SetPitchMultiplier` (`self.Wind Audio`) (`KismetMathLibrary.Lerp` 0.7 1.5 _returnvalue_3))
      (`AudioComponent.SetVolumeMultiplier` (`self.Lasic Audio`) (`KismetMathLibrary.Lerp` 0.1 1.0 _returnvalue_3))
      (`AudioComponent.SetPitchMultiplier` (`self.Lasic Audio`) (`KismetMathLibrary.Lerp` 0.5 2.0 _returnvalue_3)))
    (:`Finished`
      (`AudioComponent.FadeOut` (`self.Wind Audio`) 1.0 0.0 "Linear")
      (`AudioComponent.FadeOut` (`self.Lasic Audio`) 1.0 0.0 "Linear")
      (`GameplayStatics.PlaySoundAtLocation` "/Game/Hack-N-Slash/Enemies/Boss_Delta/SFX/SQ_SFX_Delta_GiantAOE_Finish.SQ_SFX_Delta_GiantAOE_Finish" (`self.K2_GetActorLocation`) (struct) 1.0 1.0 0.0 null null null null))))

(fn `UserConstructionScript`
  (`SphereComponent.SetSphereRadius` (`self.Sphere`) (`self.radius`) true)
  (`parent.UserConstructionScript`))