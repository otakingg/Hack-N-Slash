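; Enemy brain module that represents the Stagger state in the hack-n-slash enemy AI.
; It can start only while the brain's blackboard staggered flag is set, and it toggles its module state on enter and exit, printing debug strings.
; While active, it deactivates itself through the brain when a Clear Action State anim notify tag arrives, so animation timing ends the stagger.
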(event `self.OnEnter`
  (set `self.moduleState` "Active")
  (`KismetSystemLibrary.PrintString` null "Stagger: On Enter"))

(event `self.HandleAnimNotify`
  (params (NotifyTag :type "GameplayTag Structure"))
  (if (`|EnumEquality` (`self.moduleState`) "Active")
    (`|SwitchGameplayTag` NotifyTag
      (:`Notify.EnemyBrain.ClearActionState`
        (`EnemyBrainComponent.DeactivateModule` (`self.GetBrain`))))))

(event `self.OnExit`
  (set `self.moduleState` "Inactive")
  (`KismetSystemLibrary.PrintString` null "Stagger: On Exit"))

(fn `CanStart`
  (params (Reason :type String))
  (returns (ReturnValue :type Boolean))
  (bind (_blackboard_targetactor _blackboard_lastknownlocation _blackboard_lastdamagesource _blackboard_homelocation _blackboard_eqs_actors _blackboard_eqs_locs _blackboard_bforgottarget _blackboard_bstaggered) (break `EnemyBlackboard` (`EnemyBrainComponent.blackboard` (`self.GetBrain`))))
  (return _blackboard_bstaggered))