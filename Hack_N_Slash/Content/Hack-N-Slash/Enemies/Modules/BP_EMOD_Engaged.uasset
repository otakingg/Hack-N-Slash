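; Enemy brain module for the Engaged state, startable while the blackboard holds a target that is not forgotten, and interruptible by higher-priority modules or Return.
; A looping timer executes the highest-weight eligible enemy sequence unless the current one is non-interruptible.
; While active, it uses EQS, move-completion and tagged anim notify events to drive that sequence, then finishes it on exit.
; A Chase helper moves toward the target through the state machine, falling back to the controller.
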(event `self.OnEnter`
  (set `self.moduleState` "Active")
  (`KismetSystemLibrary.PrintString` null "Engaged: On Enter")
  (`self.EvaluateSequences`)
  (bind _returnvalue (`KismetSystemLibrary.K2_SetTimer` null "EvaluateSequences" 0.2 true))
  (set `self.TH_Sequences` _returnvalue))

(event `self.HandleEQSFinished`
  (params (Result :type "EnvQueryResult Structure (by ref)"))
  (if (and (`|EnumEquality` (`self.moduleState`) "Active") (`KismetSystemLibrary.IsValid` (`self.sequence`)))
    (`EnemySequence.AdvanceSequence` (`self.sequence`))))

(event `self.HandleMoveCompleted`
  (params (RequestID :type Integer) (Result :type "EPathFollowingResult Enum" :default "Success"))
  (if (and (`|EnumEquality` (`self.moduleState`) "Active") (`KismetSystemLibrary.IsValid` (`self.sequence`)))
    (`EnemySequence.AdvanceSequence` (`self.sequence`))))

(event `self.HandleAnimNotify`
  (params (NotifyTag :type "GameplayTag Structure"))
  (bind _sequence (`self.sequence`))
  (if (`|EnumEquality` (`self.moduleState`) "Active")
    (`|SwitchGameplayTag` NotifyTag
      (:`Default`
        (`/Engine/EditorBlueprintResources/StandardMacros.IsValid` _sequence
          (:`Is Valid`
            (`EnemySequence.HandleAnimNotify` _sequence NotifyTag))))
      (:`Notify.EnemyBrain.AdvanceSequence`
        (`/Engine/EditorBlueprintResources/StandardMacros.IsValid` _sequence
          (:`Is Valid`
            (`EnemySequence.AdvanceSequence` _sequence)))))))

(event `self.OnExit`
  (bind _sequence (`self.sequence`))
  (set `self.moduleState` "Exiting")
  (`KismetSystemLibrary.PrintString` null "Engaged: On Exit")
  (`KismetSystemLibrary.K2_ClearTimer` null "EvaluateSequences")
  (`/Engine/EditorBlueprintResources/StandardMacros.IsValid` _sequence
    (:`Is Valid`
      (`EnemySequence.Finish` _sequence))
    (:`Is Not Valid`
      _))
  (set `self.moduleState` "Inactive"))

(fn `CanBeInterruptedBy`
  (params (Other :type "EnemyBrainModule Object Reference"))
  (returns (ReturnValue :type Boolean))
  (`/Engine/EditorBlueprintResources/StandardMacros.IsValid` Other
    (:`Is Valid`
      (return (or (> (`KismetMathLibrary.Conv_ByteToInt` (`EnemyBrainModule.priority` Other)) (`KismetMathLibrary.Conv_ByteToInt` (`self.priority`))) (== (`EnemyBrainModule.moduleName` Other) "Return"))))
    (:`Is Not Valid`
      (return false))))

(fn `CanStart`
  (params (Reason :type String))
  (returns (ReturnValue :type Boolean))
  (bind (_blackboard_targetactor _blackboard_targetdistance _blackboard_lastknownlocation _blackboard_lastdamagesource _blackboard_homelocation _blackboard_aggro _blackboard_eqs_actors _blackboard_eqs_locs _blackboard_bforgottarget) (break `EnemyBlackboard` (`EnemyBrainComponent.blackboard` (`self.GetBrain`))))
  (return (and (`KismetSystemLibrary.IsValid` _blackboard_targetactor) (not _blackboard_bforgottarget))))

(fn `Chase`
  (bind _returnvalue (`self.GetBrain`))
  (bind _returnvalue_2 (`EnemyBrainComponent.GetEnemyController` _returnvalue))
  (bind _returnvalue_3 (`EnemyBrainComponent.GetStateMachine` _returnvalue))
  (bind (_blackboard_targetactor _blackboard_targetdistance _blackboard_lastknownlocation) (break `EnemyBlackboard` (`EnemyBrainComponent.blackboard` _returnvalue)))
  (`/Engine/EditorBlueprintResources/StandardMacros.IsValid` _returnvalue_3
    (:`Is Valid`
      (`self.SetWalkSpeedAndAcceleration` 500.0 4500.0)
      (`StateMachineComponent.RequestMoveTo` _returnvalue_3 _blackboard_targetactor _blackboard_lastknownlocation 300.0))
    (:`Is Not Valid`
      (`/Engine/EditorBlueprintResources/StandardMacros.IsValid` _returnvalue_2
        (:`Is Valid`
          (`self.SetWalkSpeedAndAcceleration` 500.0 4500.0)
          (`EnemyController.MoveToActorHNS` _returnvalue_2 _blackboard_targetactor 300.0))))))

(fn `EvaluateSequences`
  (locals (BestWeight :type "Float (double-precision)" :default -1.0) (BestSequence :type "EnemySequence Object Reference"))
  (bind _sequence (`self.sequence`)
    (:`then`
      (if (not (not (`EnemySequence.bInterruptible` _sequence)))
        (for _array_element (`EnemyBrainComponent.GetEnemySequences` (`self.GetBrain`)) :!label _label
          (`/Engine/EditorBlueprintResources/StandardMacros.IsValid` _array_element
            (:`Is Valid`
              (bind _weight (`EnemySequence.weight` _array_element))
              (if (and (`EnemySequence.CanExecute` _array_element) (> _weight (`local.BestWeight`)))
                (set `local.BestSequence` _array_element)
                (set `local.BestWeight` _weight)))))
        (bind _output_get (set `self.sequence` (`local.BestSequence`)))
        (`/Engine/EditorBlueprintResources/StandardMacros.IsValid` _output_get
          (:`Is Valid`
            (`EnemySequence.Execute` _output_get))
          (:`Is Not Valid`
            _))))
    (:`else`
      (goto _label)))
  (return))