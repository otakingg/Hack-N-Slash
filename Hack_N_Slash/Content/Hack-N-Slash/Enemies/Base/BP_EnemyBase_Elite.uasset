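; Elite enemy base Blueprint that extends a parent enemy with a health bar widget shown while the enemy is locked on.
; On BeginPlay it casts the bar's widget to WB_ProgressBar_NoCanvas and initializes it from the StatsComp health percentage.
; Lock-on and lock-off events toggle the bar's visibility, StatsComp health updates drive its value, and zero health deactivates and hides it.
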(event `self.ReceiveBeginPlay`
  (`parent.ReceiveBeginPlay`)
  (bind _health_bar (`self.Health Bar`)
    (:`then`
      (bind _aswb_progress_bar_no_canvas (cast `/Game/Hack-N-Slash/UI/WB_ProgressBar_NoCanvas` (`WidgetComponent.GetWidget` _health_bar)))
      (bind _output_get (set `self.WB Health Bar` _aswb_progress_bar_no_canvas))
      (`/Game/Hack-N-Slash/UI/WB_ProgressBar_NoCanvas.Initialize` _output_get (`StatsComponent.GetStatPercentage` (`self.statsComp`) "Health" "HealthMax") (struct :`R` 1.0 :`A` 1.0) (struct :`R` 0.5 :`G` 0.5 :`B` 0.5 :`A` 1.0) (struct :`R` 1.0 :`G` 1.0 :`A` 1.0)))
    (:`else`)))

(event `self.OnLockOn`
  (`parent.OnLockOn`)
  (`SceneComponent.SetVisibility` (`self.Health Bar`) true true))

(event `self.OnLockOff`
  (`parent.OnLockOff`)
  (`SceneComponent.SetVisibility` (`self.Health Bar`) false true))

(event `self.statsComp.OnZeroHealth`
  (bind _health_bar (`self.Health Bar`)
    (:`then`
      (`ActorComponent.SetActive` _health_bar false false)
      (`SceneComponent.SetVisibility` _health_bar false true))
    (:`else`)))

(event `self.statsComp.OnHealthUpdate`
  (params (NewPercent :type "Float (single-precision)") (PrevPercent :type "Float (single-precision)"))
  (bind _wb_health_bar (`self.WB Health Bar`)
    (:`then`
      (`/Game/Hack-N-Slash/UI/WB_ProgressBar_NoCanvas.Update Value` _wb_health_bar NewPercent))
    (:`else`)))

(fn `UserConstructionScript`
  (`parent.UserConstructionScript`))