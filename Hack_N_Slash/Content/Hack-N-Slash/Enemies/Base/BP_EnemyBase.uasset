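; BP_EnemyBase is the base enemy for the hack-n-slash game, handling hit responses, lock-on markers and block visuals.
; OnHitCombat routes block reactions to empty handlers and all others to OnHitStandard, which plays the hit's sound and Niagara effect.
; Lock-on events toggle target icons, tag updates refresh LocoComp movement stats, and blocking swaps a mesh overlay material.
; Health and super-armor events are empty stubs, and GetPatrolRoute exposes the patrol route.
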(event `self.ReceiveBeginPlay`
  (add `self.OnHit` (`|CreateDelegate` :!event `On Hit Combat`))
  (add `self.OnTagsUpdated` (delegate `OnTagsUpdated_Event`)))

(event `OnTagsUpdated_Event`
  (bind _lococomp (`self.locoComp`)
    (:`then`
      (`LocomotionComponent.RefreshMovementStats` _lococomp))
    (:`else`)))

(event `self.statsComp.OnHealthUpdate`
  (params (NewPercent :type "Float (single-precision)") (PrevPercent :type "Float (single-precision)")))

(event `self.statsComp.OnZeroHealth`)

(event `self.combatComp.OnSuperArmorActivated`)

(event `self.combatComp.OnSuperArmorDeactivated`)

(event `self.combatComp.OnSuperArmorBroken`)

(event `self.OnLockOn`
  (bind _lock_on_icon (`self.Lock On Icon`)
    (:`then`
      (`SceneComponent.SetVisibility` _lock_on_icon true true))
    (:`else`)))

(event `self.OnLockOff`
  (bind _lock_on_icon (`self.Lock On Icon`)
    (:`then`
      (`SceneComponent.SetVisibility` _lock_on_icon false true))
    (:`else`)))

(event `self.OnSoftLockOn`
  (bind _soft_target_icon (`self.Soft Target Icon`)
    (:`then`
      (`SceneComponent.SetVisibility` _soft_target_icon true true))
    (:`else`)))

(event `self.OnSoftLockOff`
  (bind _soft_target_icon (`self.Soft Target Icon`)
    (:`then`
      (`SceneComponent.SetVisibility` _soft_target_icon false true))
    (:`else`)))

(event `On Hit Combat`
  (params (HitData :type "AtkHitData Structure (by ref)"))
  (switch `EHitReaction` (`.resolvedReaction` (break `AtkHitData` HitData))
    (:`NoReact`
      (`self.On Hit Standard` HitData :!label _label))
    (:`Air`
      (goto _label))
    (:`BlockBreak`
      (`self.On Block Break` HitData))
    (:`BlockHit`
      (`self.On Block` HitData))
    (:`BlockPerfect`
      (`self.On Block Perfect` HitData))
    (:`BounceGround`
      (goto _label))
    (:`BounceWall`
      (goto _label))
    (:`Countered`
      (goto _label))
    (:`LaunchDown`
      (goto _label))
    (:`LaunchFwdHard`
      (goto _label))
    (:`LaunchFwdSoftBack`
      (goto _label))
    (:`LaunchFwdSoftFront`
      (goto _label))
    (:`LaunchUp`
      (goto _label))
    (:`StaggerBack`
      (goto _label))
    (:`StaggerDownFront1`
      (goto _label))
    (:`StaggerDownFront2`
      (goto _label))
    (:`StaggerDownFront3`
      (goto _label))
    (:`StaggerUpFront1`
      (goto _label))
    (:`StaggerUpFront2`
      (goto _label))
    (:`StaggerUpFront3`
      (goto _label))
    (:`WallSplat`
      (goto _label))))

(event `On Block`
  (params (`Hit Data` :type "AtkHitData Structure (by ref)")))

(event `On Block Break`
  (params (`Hit Data` :type "AtkHitData Structure (by ref)")))

(event `On Block Perfect`
  (params (`Hit Data` :type "AtkHitData Structure (by ref)")))

(event `On Hit Standard`
  (params (`Hit Data` :type "AtkHitData Structure (by ref)"))
  (bind (_attacker _damager _attackmotion _attackreaction _attacktype _barmorbreaker _biscounterfollowup _elements _aggrobuildup _dmg _penetration _poise _knockbacktype _velocityonfinishmode _velocityonfinish _clampvelocityonfinish _duration _badditive _localdir _distance _strengthovertime _brestrictspeedtoexpected _gbextrabounceheight _bgbadditive _gbsot _gbcvof _bkilled _dmgdealt _hitimpactnormal _hitimpactpoint _hitloc _hitsfx _hitvfx _hitvfxscale) (break `AtkHitData` `Hit Data`))
  (`GameplayStatics.PlaySoundAtLocation` _hitsfx _hitloc (struct) 1.0 1.0 0.0 null null null null)
  (`NiagaraFunctionLibrary.SpawnSystemAtLocation` _hitvfx _hitimpactpoint (struct) _hitvfxscale))

(fn `GetPatrolRoute`
  (returns (`Patrol Route` :type "/Game/Hack-N-Slash/Utility/BP_PatrolRoute Object Reference"))
  (return (`self.patrolRoute`)))

(fn `UpdateBlockOverlay`
  (params (`Blocking?` :type Boolean))
  (bind _mesh (`self.Mesh`))
  (if `Blocking?`
    (`MeshComponent.SetOverlayMaterial` _mesh "/Game/Hack-N-Slash/Art/EnemyBlock_Overlay.EnemyBlock_Overlay")
    (else
      (`MeshComponent.SetOverlayMaterial` _mesh null))))

(fn `UserConstructionScript`)