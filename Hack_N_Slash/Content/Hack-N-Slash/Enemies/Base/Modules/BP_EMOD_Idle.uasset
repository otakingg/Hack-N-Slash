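; Enemy brain module for the idle state in the Hack-N-Slash AI, which keeps an enemy standing still.
; It can start only when the owner has no valid patrol route and the brain's blackboard has no target and no forgotten target.
; Entering marks the module active and stops movement, while exiting marks it inactive, with both printing debug strings.
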(event `self.OnEnter`
  (set `self.moduleState` "Active")
  (`KismetSystemLibrary.PrintString` null "Idle: On Enter")
  (`self.StopMovingHNS`))

(event `self.OnExit`
  (set `self.moduleState` "Inactive")
  (`KismetSystemLibrary.PrintString` null "Idle: On Exit"))

(fn `CanStart`
  (params (Reason :type String))
  (returns (ReturnValue :type Boolean))
  (bind _returnvalue (`self.GetBrain`))
  (bind (_targetactor _lastknownlocation _lastdamagesource _homelocation _eqs_actors _eqs_locs _bforgottarget) (break `EnemyBlackboard` (`EnemyBrainComponent.blackboard` _returnvalue)))
  (bind _patrol_route (message `/Game/Hack-N-Slash/Interfaces/BPI_Patroler.GetPatrolRoute` (`ActorComponent.GetOwner` _returnvalue)))
  (return (and (not (`KismetSystemLibrary.IsValid` _patrol_route)) (not (`KismetSystemLibrary.IsValid` _targetactor)) (not _bforgottarget))))