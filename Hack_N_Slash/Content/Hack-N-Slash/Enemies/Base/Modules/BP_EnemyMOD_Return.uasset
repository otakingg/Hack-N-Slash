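; Enemy brain module that sends an enemy back to its home location after it forgets its target.
; It starts only when away from home with no valid target, refuses interruption, and waits on a timer before moving.
; Movement goes through the state machine, falling back to the enemy controller, and makes the enemy immune.
; Arrival deactivates the module, while exit stops movement and restores normal vulnerability.
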(event `self.OnEnter`
  (`KismetSystemLibrary.PrintString` null "Return: On Enter")
  (set `self.moduleState` "Active")
  (`self.Validate Combat Res`
    (:`Is Valid`
      _)
    (:`then`
      _))
  (bind _returnvalue (`KismetSystemLibrary.K2_SetTimerDelegate` (delegate `Return`) 10.0))
  (set `self.TH_Return` _returnvalue))

(event `Return`
  (bind _returnvalue (`self.GetBrain`))
  (bind _returnvalue_2 (`EnemyBrainComponent.GetStateMachine` _returnvalue))
  (bind _returnvalue_3 (`EnemyBrainComponent.GetEnemyController` _returnvalue))
  (bind (_blackboard_targetactor _blackboard_lastknownlocation _blackboard_lastdamagesource _blackboard_homelocation) (break `EnemyBlackboard` (`EnemyBrainComponent.blackboard` _returnvalue)))
  (`/Engine/EditorBlueprintResources/StandardMacros.IsValid` _returnvalue
    (:`Is Valid`
      (`/Engine/EditorBlueprintResources/StandardMacros.IsValid` _returnvalue_2
        (:`Is Valid`
          (`self.SetWalkSpeedAndAcceleration` 500.0 4500.0)
          (`StateMachineComponent.RequestMoveTo` _returnvalue_2 null _blackboard_homelocation 50.0))
        (:`Is Not Valid`
          (`/Engine/EditorBlueprintResources/StandardMacros.IsValid` _returnvalue_3
            (:`Is Valid`
              (`self.SetWalkSpeedAndAcceleration` 500.0 4500.0)
              (`EnemyController.MoveToLocationHNS` _returnvalue_3 _blackboard_homelocation 50.0)))))
      (`self.Validate Combat Res`
        (:`Is Valid`
          (`CombatResolutionComponent.SetVulnerability` (`self.CombatRes`) "Immune"))
        (:`then`)))))

(event `self.HandleMoveCompleted`
  (params (RequestID :type Integer) (Result :type "EPathFollowingResult Enum" :default "Success"))
  (bind _returnvalue (`self.GetBrain`))
  (bind (_blackboard_targetactor _blackboard_lastknownlocation _blackboard_lastdamagesource _blackboard_homelocation _blackboard_eqs_actors _blackboard_eqs_locs _blackboard_bforgottarget _blackboard_bstaggered) (break `EnemyBlackboard` (`EnemyBrainComponent.blackboard` _returnvalue)))
  (if (`|EnumEquality` (`self.moduleState`) "Active")
    (set `EnemyBrainComponent.blackboard` (make `EnemyBlackboard` _blackboard_targetactor _blackboard_lastknownlocation _blackboard_lastdamagesource _blackboard_homelocation false _blackboard_bstaggered) _returnvalue)
    (set `self.moduleState` "Inactive")))

(event `self.OnExit`
  (bind _returnvalue (`self.GetBrain`))
  (bind (_blackboard_targetactor _blackboard_lastknownlocation _blackboard_lastdamagesource _blackboard_homelocation _blackboard_eqs_actors _blackboard_eqs_locs _blackboard_bforgottarget _blackboard_bstaggered) (break `EnemyBlackboard` (`EnemyBrainComponent.blackboard` _returnvalue)))
  (`KismetSystemLibrary.PrintString` null "Return: On Exit")
  (set `self.moduleState` "Inactive")
  (`KismetSystemLibrary.K2_ClearAndInvalidateTimerHandle` self (`self.TH_Return`))
  (`self.StopMovingHNS`)
  (`self.Validate Combat Res`
    (:`Is Valid`
      (`CombatResolutionComponent.SetVulnerability` (`self.CombatRes`) "Normal"))
    (:`then`
      _))
  (set `EnemyBrainComponent.blackboard` (make `EnemyBlackboard` _blackboard_targetactor _blackboard_lastknownlocation _blackboard_lastdamagesource _blackboard_homelocation false _blackboard_bstaggered) _returnvalue))

(fn `CanBeInterruptedBy`
  (params (Other :type "EnemyBrainModule Object Reference"))
  (returns (ReturnValue :type Boolean))
  (return false))

(fn `CanStart`
  (params (Reason :type String))
  (returns (ReturnValue :type Boolean))
  (bind _returnvalue (`self.GetBrain`))
  (bind _returnvalue_2 (`ActorComponent.GetOwner` _returnvalue))
  (bind (_blackboard_targetactor _blackboard_lastknownlocation _blackboard_lastdamagesource _blackboard_homelocation _blackboard_eqs_actors _blackboard_eqs_locs _blackboard_bforgottarget) (break `EnemyBlackboard` (`EnemyBrainComponent.blackboard` _returnvalue)))
  (return (and (`KismetSystemLibrary.IsValid` _returnvalue_2) (> (`KismetMathLibrary.Vector_Distance` (`Actor.K2_GetActorLocation` _returnvalue_2) _blackboard_homelocation) 150.0) (not (`KismetSystemLibrary.IsValid` _blackboard_targetactor)) _blackboard_bforgottarget)))