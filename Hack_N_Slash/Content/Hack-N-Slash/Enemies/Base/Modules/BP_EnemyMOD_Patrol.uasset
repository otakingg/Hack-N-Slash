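; Enemy brain module that walks an enemy along its spline patrol route in the hack-n-slash game.
; It can start only when a route exists, the blackboard has no target actor and ForgotTarget is false.
; Patrol moves at walk speed via the state machine, falling back to the enemy controller.
; Each completed move advances the route index and schedules the next after a random pause; exiting stops movement and timer.
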(event `self.OnEnter`
  (`KismetSystemLibrary.PrintString` null "Patrol: OnEnter")
  (set `self.moduleState` "Active")
  (`self.Patrol`))

(event `self.HandleMoveCompleted`
  (params (RequestID :type Integer) (Result :type "EPathFollowingResult Enum" :default "Success"))
  (if (`|EnumEquality` (`self.moduleState`) "Active")
    (`KismetSystemLibrary.K2_ClearAndInvalidateTimerHandle` self (`self.TH_Wait`))
    (bind _patrol_route (message `/Game/Hack-N-Slash/Interfaces/BPI_Patroler.GetPatrolRoute` (`ActorComponent.GetOwner` (`self.GetBrain`))))
    (`/Engine/EditorBlueprintResources/StandardMacros.IsValid` _patrol_route
      (:`Is Valid`
        (`/Game/Hack-N-Slash/Utility/BP_PatrolRoute.IncrementPatrolIndex` _patrol_route)
        (bind _returnvalue (`KismetSystemLibrary.K2_SetTimer` null "Patrol" (`KismetMathLibrary.RandomFloatInRange` 2.0 5.0)))
        (set `self.TH_Wait` _returnvalue)))))

(event `self.OnExit`
  (`KismetSystemLibrary.PrintString` null "Patrol: OnExit")
  (set `self.moduleState` "Inactive")
  (`KismetSystemLibrary.K2_ClearAndInvalidateTimerHandle` self (`self.TH_Wait`))
  (`self.StopMovingHNS`))

(fn `CanStart`
  (params (Reason :type String))
  (returns (ReturnValue :type Boolean))
  (bind _returnvalue (`self.GetBrain`))
  (bind (_targetactor _lastknownlocation _lastdamagesource _homelocation _eqs_actors _eqs_locs _bforgottarget) (break `EnemyBlackboard` (`EnemyBrainComponent.blackboard` _returnvalue)))
  (bind _patrol_route (message `/Game/Hack-N-Slash/Interfaces/BPI_Patroler.GetPatrolRoute` (`ActorComponent.GetOwner` _returnvalue)))
  (return (and (`KismetSystemLibrary.IsValid` _patrol_route) (not (`KismetSystemLibrary.IsValid` _targetactor)) (not _bforgottarget))))

(fn `Patrol`
  (bind _returnvalue (`self.GetBrain`))
  (bind _returnvalue_2 (`self.GetBrain`))
  (bind _returnvalue_3 (`EnemyBrainComponent.GetStateMachine` _returnvalue_2))
  (bind _returnvalue_4 (`EnemyBrainComponent.GetEnemyController` _returnvalue_2))
  (`/Engine/EditorBlueprintResources/StandardMacros.IsValid` _returnvalue
    (:`Is Valid`
      (bind _patrol_route (message `/Game/Hack-N-Slash/Interfaces/BPI_Patroler.GetPatrolRoute` (`ActorComponent.GetOwner` _returnvalue)))
      (`/Engine/EditorBlueprintResources/StandardMacros.IsValid` _patrol_route
        (:`Is Valid`
          (`/Engine/EditorBlueprintResources/StandardMacros.IsValid` _returnvalue_3
            (:`Is Valid`
              (`self.SetWalkSpeedAndAcceleration` 200.0 4500.0)
              (bind _patrolpoint (`/Game/Hack-N-Slash/Utility/BP_PatrolRoute.GetSplinePointAsWorldLocation` _patrol_route))
              (`StateMachineComponent.RequestMoveTo` _returnvalue_3 null _patrolpoint 50.0))
            (:`Is Not Valid`
              (`/Engine/EditorBlueprintResources/StandardMacros.IsValid` _returnvalue_4
                (:`Is Valid`
                  (`self.SetWalkSpeedAndAcceleration` 200.0 4500.0)
                  (`EnemyController.MoveToLocationHNS` _returnvalue_4 _patrolpoint 50.0))))))))))