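; Enemy brain module that runs the stagger state for hack-n-slash enemies.
; It can start only while the brain's blackboard flags the enemy as staggered.
; Entering and exiting toggle the module state between active and inactive with debug prints.
; A Clear Action State anim notify tag tells the brain to deactivate the module, so the animation drives when it ends.
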(event `self.OnEnter`
  (`KismetSystemLibrary.PrintString` null "Stagger: On Enter")
  (set `self.moduleState` "Active"))

(event `self.HandleAnimNotify`
  (params (NotifyTag :type "GameplayTag Structure"))
  (`|SwitchGameplayTag` NotifyTag
    (:`Notify.EnemyBrain.ClearActionState`
      (`EnemyBrainComponent.DeactivateModule` (`self.GetBrain`)))))

(event `self.OnExit`
  (`KismetSystemLibrary.PrintString` null "Stagger: On Exit")
  (set `self.moduleState` "Inactive"))

(fn `CanStart`
  (params (Reason :type String))
  (returns (ReturnValue :type Boolean))
  (bind (_blackboard_targetactor _blackboard_lastknownlocation _blackboard_lastdamagesource _blackboard_homelocation _blackboard_eqs_actors _blackboard_eqs_locs _blackboard_bforgottarget _blackboard_bstaggered) (break `EnemyBlackboard` (`EnemyBrainComponent.blackboard` (`self.GetBrain`))))
  (return _blackboard_bstaggered))