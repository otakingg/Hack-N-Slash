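; Enemy attack sequence that zips the enemy through three high-speed dashes around its focused target, then requests a far attack.
; An indexed step machine alternates EQS location queries, uninterruptible move-to dashes and interruptible random timed pauses.
; Distance to the target picks the query, switching to a close-to-target dash beyond a threshold.
; Invalid references end the sequence, and finishing resets it and starts any cooldown.
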(event `self.Execute`
  (bind _returnvalue (`self.GetBrain`))
  (bind _returnvalue_2 (`self.GetBrain`))
  (bind _blackboard_targetactor (break `EnemyBlackboard` (`EnemyBrainComponent.blackboard` _returnvalue_2)))
  (bind _blackboard_targetactor_2 (break `EnemyBlackboard` (`EnemyBrainComponent.blackboard` _returnvalue)))
  (`self.EnsureReferences`
    (:`Is Valid`
      (set `self.bExecuting` true)
      (if (<= (`KismetMathLibrary.Vector_Distance` (`Actor.K2_GetActorLocation` (`ActorComponent.GetOwner` _returnvalue)) (`Actor.K2_GetActorLocation` _blackboard_targetactor_2)) (`self.dashDirThreshold`))
        (`self.FindDashLoc` null)
        (else
          (`self.FindDashLoc` "/Game/Hack-N-Slash/Enemies/EQS/EQS_DashCloseToTarget.EQS_DashCloseToTarget")))
      (`EnemyController.SetFocusHNS` (`EnemyBrainComponent.GetEnemyController` _returnvalue_2) _blackboard_targetactor)
      (`self.SetWalkSpeedAndAcceleration` 9000.0 10000.0))
    (:`Is Not Valid`
      (`self.Finish`))))

(event `self.AdvanceSequence`
  (bind _returnvalue (`self.GetBrain`))
  (bind _returnvalue_2 (`self.GetBrain`))
  (bind _blackboard_targetactor (break `EnemyBlackboard` (`EnemyBrainComponent.blackboard` _returnvalue_2)))
  (`self.EnsureReferences`
    (:`Is Valid`
      (bind _output_get (set `self.sequenceIndex` (+ (`self.sequenceIndex`) 1)))
      (switch `int` _output_get
        (:`Default`
          (`self.Finish`))
        (:`2`
          (set `self.bInterruptible` false :!label _label)
          (bind _dashlocvalid_ (`self.Dash`))
          (if (not _dashlocvalid_)
            (`self.AdvanceSequence`)))
        (:`3`
          (set `self.bInterruptible` true :!label _label_2)
          (bind _returnvalue_3 (`KismetSystemLibrary.K2_SetTimer` null "Advance Sequence" (`KismetMathLibrary.RandomFloatInRange` 0.0 2.0)))
          (set `self.TH_AdvSeq` _returnvalue_3))
        (:`4`
          (if (<= (`KismetMathLibrary.Vector_Distance` (`Actor.K2_GetActorLocation` (`ActorComponent.GetOwner` _returnvalue_2)) (`Actor.K2_GetActorLocation` _blackboard_targetactor)) (`self.dashDirThreshold`)) :!label _label_3
            (`self.FindDashLoc` null)
            (else
              (`self.FindDashLoc` "/Game/Hack-N-Slash/Enemies/EQS/EQS_DashCloseToTarget.EQS_DashCloseToTarget"))))
        (:`5`
          (goto _label))
        (:`6`
          (goto _label_2))
        (:`7`
          (goto _label_3))
        (:`8`
          (goto _label))
        (:`9`
          (`AIController.K2_ClearFocus` (`EnemyBrainComponent.GetEnemyController` _returnvalue))
          (set `self.bInterruptible` false)
          (`StateMachineComponent.RequestAttackEnemy` (`EnemyBrainComponent.GetStateMachine` _returnvalue) (`self.atkFar`)))))
    (:`Is Not Valid`
      (`self.Finish`))))

(event `self.Finish`
  (`self.EnsureReferences`
    (:`Is Valid`
      (`AIController.K2_ClearFocus` (`EnemyBrainComponent.GetEnemyController` (`self.GetBrain`))))
    (:`Is Not Valid`
      _))
  (`KismetSystemLibrary.K2_ClearAndInvalidateTimerHandle` self (`self.TH_AdvSeq`))
  (if (> (`self.cooldown`) 0.0)
    (set `self.bOnCooldown` true)
    (`KismetSystemLibrary.K2_ClearAndInvalidateTimerHandle` self (`self.TH_Cooldown`))
    (bind _returnvalue (`KismetSystemLibrary.K2_SetTimer` self "EndCooldown" (`self.cooldown`)))
    (set `self.TH_Cooldown` _returnvalue))
  (set `self.sequenceIndex` 1)
  (set `self.bExecuting` false))

(fn `Dash`
  (returns (`dashLocValid?` :type Boolean))
  (bind _returnvalue (`self.GetBrain`))
  (bind (_targetactor _lastknownlocation _lastdamagesource _homelocation _eqs_actors _eqs_locs) (break `EnemyBlackboard` (`EnemyBrainComponent.blackboard` _returnvalue)))
  (`StateMachineComponent.RequestMoveTo` (`EnemyBrainComponent.GetStateMachine` _returnvalue) null (`|GetArrayItem` _eqs_locs) 100.0)
  (return (`KismetArrayLibrary.Array_IsEmpty` _eqs_locs)))

(fn `FindDashLoc`
  (params (`Query Temp` :type "EnvQuery Object Reference"))
  (`EnemyController.RunEQSQueryHNS` (`EnemyBrainComponent.GetEnemyController` (`self.GetBrain`)) `Query Temp` "RandomBest5Pct"))