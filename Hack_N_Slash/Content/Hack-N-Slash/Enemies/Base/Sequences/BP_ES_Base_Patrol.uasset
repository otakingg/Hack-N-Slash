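; Base enemy AI sequence that walks an enemy along its patrol route while the blackboard has no target actor.
; It runs only when a route and the movement and locomotion components are valid, then sets a slower walk speed, marks itself interruptible and moves to the current spline point.
; On move completion it advances the route index and calls Patrol again after a random pause of a few seconds.
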(event `self.Initialize`
  (params (InBrain :type "EnemyBrainComponent Object Reference"))
  (`parent.Initialize` InBrain)
  (bind _brain (`self.brain`)
    (:`then`
      (bind _returnvalue (`ActorComponent.GetOwner` _brain))
      (`/Engine/EditorBlueprintResources/StandardMacros.IsValid` _returnvalue
        (:`Is Valid`
          (set `self.MoveComp` (`Actor.GetComponentByClass` _returnvalue "/Script/Engine.CharacterMovementComponent"))
          (set `self.LocoComp` (`Actor.GetComponentByClass` _returnvalue "/Script/Hack_N_Slash.LocomotionComponent")))))
    (:`else`)))

(event `self.Execute`
  (`self.Is Active?`
    (:`Yes`
      (`self.EnsureReferences`
        (:`Valid`
          (set `self.bInterruptibleProactive` true)
          (`self.Is Active?`
            (:`Yes`
              (`self.SetMaxWalkSpeedAndAcceleration` 200.0 4500.0)
              (`self.Patrol`))))
        (:`Invalid`
          (`self.Finish`))))))

(event `self.HandleMoveCompleted`
  (params (RequestID :type Integer) (Result :type "EPathFollowingResult Enum" :default "Success"))
  (`self.Is Active?`
    (:`Yes`
      (`self.EnsureReferences`
        (:`Valid`
          (`KismetSystemLibrary.K2_ClearTimer` null "Wait")
          (`self.Is Active?`
            (:`Yes`
              (bind _patrol_route (message `/Game/Hack-N-Slash/Interfaces/BPI_Patroler.GetPatrolRoute` (`ActorComponent.GetOwner` (`self.brain`))))
              (`/Engine/EditorBlueprintResources/StandardMacros.IsValid` _patrol_route
                (:`Is Valid`
                  (`/Game/Hack-N-Slash/Utility/BP_PatrolRoute.IncrementPatrolIndex` _patrol_route)
                  (bind _returnvalue (`KismetSystemLibrary.K2_SetTimer` null "Patrol" (`KismetMathLibrary.RandomFloatInRange` 2.0 5.0)))
                  (set `self.TH_Wait` _returnvalue))
                (:`Is Not Valid`
                  (`self.Finish`))))))
        (:`Invalid`
          (`self.Finish`))))))

(fn `CanExecute`
  (returns (ReturnValue :type Boolean))
  (bind _brain (`self.brain`))
  (bind _blackboard_targetactor (break `EnemyBlackboard` (`EnemyBrainComponent.blackboard` _brain)))
  (bind _patrol_route (message `/Game/Hack-N-Slash/Interfaces/BPI_Patroler.GetPatrolRoute` (`ActorComponent.GetOwner` _brain)))
  (return (and (`parent.CanExecute`) (`KismetSystemLibrary.IsValid` _patrol_route) (`KismetSystemLibrary.IsValid` (`self.MoveComp`)) (`KismetSystemLibrary.IsValid` (`self.LocoComp`)) (not (`KismetSystemLibrary.IsValid` _blackboard_targetactor)))))

(fn `Patrol`
  (`self.Is Active?`
    (:`Yes`
      (bind _brain (`self.brain`)
        (:`then`
          (bind _patrol_route (message `/Game/Hack-N-Slash/Interfaces/BPI_Patroler.GetPatrolRoute` (`ActorComponent.GetOwner` _brain)))
          (`/Engine/EditorBlueprintResources/StandardMacros.IsValid` _patrol_route
            (:`Is Valid`
              (bind _lococomp (`self.LocoComp`)
                (:`then`
                  (`LocomotionComponent.MoveTo` _lococomp null (`/Game/Hack-N-Slash/Utility/BP_PatrolRoute.GetSplinePointAsWorldLocation` _patrol_route) 50.0))
                (:`else`
                  (`self.Finish` :!label _label))))
            (:`Is Not Valid`
              (goto _label))))
        (:`else`
          (`self.Finish`))))))

(fn `SetMaxWalkSpeedAndAcceleration`
  (params (Speed :type "Float (double-precision)") (Acceleration :type "Float (double-precision)"))
  (set `CharacterMovementComponent.MaxWalkSpeed` Speed (`self.MoveComp`))
  (set `CharacterMovementComponent.MaxAcceleration` (`local.Acceleration`) (`self.MoveComp`)))