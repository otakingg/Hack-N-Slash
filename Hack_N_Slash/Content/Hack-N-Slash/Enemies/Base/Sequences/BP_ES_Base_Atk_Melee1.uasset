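; Enemy action sequence for a basic melee attack: close in on the target actor, then attack.
; Execute boosts walk speed and acceleration and asks the brain's state machine to move near the blackboard target.
; AdvanceSequence steps the action index, requesting the attack until the action count is reached, then finishing.
; A reference check on brain, state machine, controller and target guards both events, finishing early on failure; CanExecute always passes.
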(event `self.Execute`
  (bind _returnvalue (`self.GetBrain`))
  (set `self.bExecuting` true)
  (`self.EnsureReferences`
    (:`Is Valid`
      (`self.SetWalkSpeedAndAcceleration` 500.0 4500.0)
      (`StateMachineComponent.RequestMoveTo` (`EnemyBrainComponent.GetStateMachine` _returnvalue) null (`Actor.K2_GetActorLocation` (`.TargetActor` (break `EnemyBlackboard` (`EnemyBrainComponent.blackboard` _returnvalue)))) 300.0))
    (:`Is Not Valid`
      (`self.Finish`))))

(event `self.AdvanceSequence`
  (`self.EnsureReferences`
    (:`Is Valid`
      (bind _output_get (set `self.sequenceIndex` (+ (`self.sequenceIndex`) 1)))
      (if (>= _output_get (`self.numActions`))
        (`self.Finish`)
        (else
          (`StateMachineComponent.RequestAttackEnemy` (`EnemyBrainComponent.GetStateMachine` (`self.GetBrain`)) (`self.Atk`)))))
    (:`Is Not Valid`
      (`self.Finish`))))

(fn `CanExecute`
  (returns (ReturnValue :type Boolean))
  (return true))