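; Enemy behavior sequence that has an AI strafe at walking speed while keeping focus on its target actor.
; Execute sets focus and speed and runs an EQS strafe query, then AdvanceSequence steps through a fixed cycle of moving, randomly timed pauses and new queries.
; EnsureReferences guards the brain, controller, state machine and target.
; Finish clears focus and timers, starts any cooldown and resets the sequence as interruptible.
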(event `self.Execute`
  (bind _returnvalue (`self.GetBrain`))
  (bind _blackboard_targetactor (break `EnemyBlackboard` (`EnemyBrainComponent.blackboard` _returnvalue)))
  (`self.EnsureReferences`
    (:`Is Valid`
      (`self.FindStrafeLoc`)
      (`EnemyController.SetFocusHNS` (`EnemyBrainComponent.GetEnemyController` _returnvalue) _blackboard_targetactor)
      (`self.SetWalkSpeedAndAcceleration` 300.0 2048.0))
    (:`Is Not Valid`
      (`self.Finish`))))

(event `self.AdvanceSequence`
  (`self.EnsureReferences`
    (:`Is Valid`
      (bind _output_get (set `self.sequenceIndex` (+ (`self.sequenceIndex`) 1)))
      (switch `int` _output_get
        (:`Default`
          (`self.Finish`))
        (:`2`
          (bind _movelocvalid_ (`self.Move` :!label _label))
          (if (not _movelocvalid_)
            (`self.Finish`)))
        (:`3`
          (bind _returnvalue (`KismetSystemLibrary.K2_SetTimer` null "Advance Sequence" (`KismetMathLibrary.RandomFloatInRange` 0.0 2.0) :!label _label_2))
          (set `self.TH_AdvSeq` _returnvalue))
        (:`4`
          (`self.FindStrafeLoc` :!label _label_3))
        (:`5`
          (goto _label))
        (:`6`
          (goto _label_2))
        (:`7`
          (goto _label_3))
        (:`8`
          (goto _label))
        (:`9`
          (goto _label_2))
        (:`10`
          (goto _label_3))
        (:`11`
          (goto _label))))
    (:`Is Not Valid`
      (`self.Finish`))))

(event `self.Finish`
  (`self.EnsureReferences`
    (:`Is Valid`
      (`AIController.K2_ClearFocus` (`EnemyBrainComponent.GetEnemyController` (`self.GetBrain`))))
    (:`Is Not Valid`
      _))
  (`KismetSystemLibrary.K2_ClearAndInvalidateTimerHandle` self (`self.TH_AdvSeq`))
  (if (> (`self.cooldown`) 0.0)
    (set `self.bOnCooldown` true)
    (`KismetSystemLibrary.K2_ClearAndInvalidateTimerHandle` self (`self.TH_Cooldown`))
    (bind _returnvalue (`KismetSystemLibrary.K2_SetTimer` self "EndCooldown" (`self.cooldown`)))
    (set `self.TH_Cooldown` _returnvalue))
  (set `self.sequenceIndex` 1)
  (set `self.bInterruptible` true))

(fn `FindStrafeLoc`
  (`EnemyController.RunEQSQueryHNS` (`EnemyBrainComponent.GetEnemyController` (`self.GetBrain`)) "/Game/Hack-N-Slash/Enemies/EQS/QueryTarget/EQ_StrafeTarget.EQ_StrafeTarget" (`|MakeMap` "None" :!type "Name" :!valuetype "Float (single-precision)") "RandomBest5Pct"))

(fn `Move`
  (returns (`MoveLocValid?` :type Boolean))
  (bind _returnvalue (`self.GetBrain`))
  (bind (_targetactor _targetdistance _lastknownlocation _lastdamagesource _homelocation _aggro _eqs_actors _eqs_locs) (break `EnemyBlackboard` (`EnemyBrainComponent.blackboard` _returnvalue)))
  (`StateMachineComponent.RequestMoveTo` (`EnemyBrainComponent.GetStateMachine` _returnvalue) null (`|GetArrayItem` _eqs_locs) 10.0)
  (return (`KismetArrayLibrary.Array_IsEmpty` _eqs_locs)))