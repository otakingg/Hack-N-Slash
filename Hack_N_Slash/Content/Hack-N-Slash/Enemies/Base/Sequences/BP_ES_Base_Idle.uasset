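; Enemy behavior sequence for idling, used when the parent check passes and the enemy has neither a valid patrol route nor a target actor.
; On execute it stops the enemy controller's movement and flags itself interruptible, both proactively and reactively, re-checking that it is still active between steps.
; It then starts a looping, randomized-delay timer bound to a Wait event, which is empty here.
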(event `self.Execute`
  (`self.Is Active?`
    (:`Yes`
      (`Controller.StopMovement` (`EnemyBrainComponent.GetEnemyController` (`self.brain`)))
      (`self.Is Active?`
        (:`Yes`
          (set `self.bInterruptibleProactive` true)
          (set `self.bInterruptibleReactive` true)
          (`self.Is Active?`
            (:`Yes`
              (bind _returnvalue (`KismetSystemLibrary.K2_SetTimerDelegate` (delegate `Wait`) (`KismetMathLibrary.RandomFloatInRange` 2.0 5.0) true))
              (set `self.TH_Wait` _returnvalue))))))))

(event `Wait`)

(fn `CanExecute`
  (returns (ReturnValue :type Boolean))
  (bind _brain (`self.brain`))
  (bind _blackboard_targetactor (break `EnemyBlackboard` (`EnemyBrainComponent.blackboard` _brain)))
  (bind _patrol_route (message `/Game/Hack-N-Slash/Interfaces/BPI_Patroler.GetPatrolRoute` (`ActorComponent.GetOwner` _brain)))
  (return (and (`parent.CanExecute`) (not (`KismetSystemLibrary.IsValid` _patrol_route)) (not (`KismetSystemLibrary.IsValid` _blackboard_targetactor)))))