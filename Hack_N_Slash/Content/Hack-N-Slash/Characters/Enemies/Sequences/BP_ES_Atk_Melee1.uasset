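; Enemy action sequence that closes on the target and performs a melee attack, driven through the AI brain's state machine.
; Execute sets walk speed and acceleration, then requests a move to the Blackboard's target actor within an acceptance radius.
; Each AdvanceSequence call increments the step and requests the configured attack, finishing once the action count is reached or the state machine is invalid.
; CanExecute always returns true.
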(event `self.Execute`
  (bind _returnvalue (`self.GetBrain`))
  (bind _returnvalue_2 (`EnemyBrainComponent.GetStateMachine` _returnvalue))
  (set `self.bExecuting` true)
  (`/Engine/EditorBlueprintResources/StandardMacros.IsValid` _returnvalue_2
    (:`Is Valid`
      (`self.SetWalkSpeedAndAcceleration` 500.0 4500.0)
      (`StateMachineComponent.RequestMoveTo` _returnvalue_2 (`.TargetActor` (break `EnemyBlackboard` (`EnemyBrainComponent.blackboard` _returnvalue))) (0.0 0.0 0.0) 300.0))
    (:`Is Not Valid`
      (`self.Finish`))))

(event `self.AdvanceSequence`
  (bind _returnvalue (`EnemyBrainComponent.GetStateMachine` (`self.GetBrain`)))
  (bind _output_get (set `self.sequenceIndex` (+ (`self.sequenceIndex`) 1)))
  (if (>= _output_get (`self.numActions`))
    (`self.Finish`)
    (else
      (`/Engine/EditorBlueprintResources/StandardMacros.IsValid` _returnvalue
        (:`Is Valid`
          (`StateMachineComponent.RequestAttackEnemy` _returnvalue (`self.Atk`)))
        (:`Is Not Valid`
          (`self.Finish`))))))

(fn `CanExecute`
  (returns (ReturnValue :type Boolean))
  (return true))