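; BP_Player is the hack-n-slash player character, which spawns a katana attached to its hand socket.
; Enhanced Input events funnel into InputComp.HandlePlayerInput as enum-tagged calls, while chakra nature keys call CombatComp directly.
; CombatComp events toggle base and wind aura VFX, and hits play SFX/VFX except block reactions, which route to empty stubs.
; It also has dash VFX, a sphere-trace lightning strike on nearby living actors, and debug slow-motion and trace keys.
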(event `self.ReceiveBeginPlay`
  (add `self.OnHit` (`|CreateDelegate` :!event `On Hit Combat`))
  (add `self.OnTagsUpdated` (delegate `OnTagsUpdated_Event`))
  (bind _returnvalue (`|SpawnActorFromClass` "/Game/Hack-N-Slash/Player/Weapons/BP_Weapon_Player_Katana.BP_Weapon_Player_Katana_C" (`SceneComponent.GetSocketTransform` (`self.Mesh`) "weaponBaseR_Socket" "RTS_World") "Undefined" "MultiplyWithRoot" self self))
  (`self.K2_AttachToComponent` _returnvalue (`self.Mesh`) "weaponBaseR_Socket" "SnapToTarget" "SnapToTarget" "SnapToTarget" true))

(event `OnTagsUpdated_Event`
  (bind _lococomp (`self.locoComp`)
    (:`then`
      (`LocomotionComponent.RefreshMovementStats` _lococomp))
    (:`else`)))

(event `Key|Tab`
  (params (Key :type "Key Structure"))
  ;[0 1 0 0.5] Debug Testing
  (:`Pressed`
    (`GameplayStatics.SetGlobalTimeDilation` 0.2))
  (:`Released`
    (`GameplayStatics.SetGlobalTimeDilation` 1.0)))

(event `EnhancedInput|/Game/Hack-N-Slash/Player/Input/IA_LookMouse_HNS`
  (params (ActionValue :type "Vector2D Structure") (ElapsedSeconds :type "Float (double-precision)") (TriggeredSeconds :type "Float (double-precision)") (InputAction :type "InputAction Object Reference" :default "/Game/Hack-N-Slash/Player/Input/IA_LookMouse_HNS.IA_LookMouse_HNS"))
  ;[1 1 1 0.5] Look/Lock On
  (:`Triggered`
    (`PlayerInputComponent.HandlePlayerInput` (`self.inputComp`) "LookMouseTrigger" ActionValue (0.0 0.0))))

(event `EnhancedInput|/Game/Hack-N-Slash/Player/Input/IA_SwitchTargetLeft`
  (params (ActionValue :type Boolean) (ElapsedSeconds :type "Float (double-precision)") (TriggeredSeconds :type "Float (double-precision)") (InputAction :type "InputAction Object Reference" :default "/Game/Hack-N-Slash/Player/Input/IA_SwitchTargetLeft.IA_SwitchTargetLeft"))
  ;[1 1 1 0.5] Look/Lock On
  (:`Started`
    (`PlayerInputComponent.HandlePlayerInput` (`self.inputComp`) "SwitchTargetLeftStart" (0.0 0.0) (0.0 0.0))))

(event `EnhancedInput|/Game/Hack-N-Slash/Player/Input/IA_AttackHeavy`
  (params (ActionValue :type Boolean) (ElapsedSeconds :type "Float (double-precision)") (TriggeredSeconds :type "Float (double-precision)") (InputAction :type "InputAction Object Reference" :default "/Game/Hack-N-Slash/Player/Input/IA_AttackHeavy.IA_AttackHeavy"))
  ;[1 1 1 0.5] Attack
  (:`Triggered`
    (`PlayerInputComponent.HandlePlayerInput` (`self.inputComp`) "AttackHeavyTrigger" (0.0 0.0) (`|GetInputActionValue`)))
  (:`Started`
    (`PlayerInputComponent.HandlePlayerInput` (`self.inputComp`) "AttackHeavyStart" (0.0 0.0) (`|GetInputActionValue`)))
  (:`Completed`
    (`PlayerInputComponent.HandlePlayerInput` (`self.inputComp`) "AttackHeavyComplete" (0.0 0.0) (`|GetInputActionValue`))))

(event `EnhancedInput|/Game/Hack-N-Slash/Player/Input/IA_AttackLight`
  (params (ActionValue :type Boolean) (ElapsedSeconds :type "Float (double-precision)") (TriggeredSeconds :type "Float (double-precision)") (InputAction :type "InputAction Object Reference" :default "/Game/Hack-N-Slash/Player/Input/IA_AttackLight.IA_AttackLight"))
  ;[1 1 1 0.5] Attack
  (:`Triggered`
    (`PlayerInputComponent.HandlePlayerInput` (`self.inputComp`) "AttackLightTrigger" (0.0 0.0) (`|GetInputActionValue`)))
  (:`Started`
    (`PlayerInputComponent.HandlePlayerInput` (`self.inputComp`) "AttackLightStart" (0.0 0.0) (`|GetInputActionValue`)))
  (:`Completed`
    (`PlayerInputComponent.HandlePlayerInput` (`self.inputComp`) "AttackLightComplete" (0.0 0.0) (`|GetInputActionValue`))))

(event `EnhancedInput|/Game/Hack-N-Slash/Player/Input/IA_AttackNinjutsu`
  (params (ActionValue :type Boolean) (ElapsedSeconds :type "Float (double-precision)") (TriggeredSeconds :type "Float (double-precision)") (InputAction :type "InputAction Object Reference" :default "/Game/Hack-N-Slash/Player/Input/IA_AttackNinjutsu.IA_AttackNinjutsu"))
  ;[1 1 1 0.5] Attack
  (:`Triggered`
    (`PlayerInputComponent.HandlePlayerInput` (`self.inputComp`) "AttackNinjutsuTrigger" (0.0 0.0) (`|GetInputActionValue`)))
  (:`Started`
    (`PlayerInputComponent.HandlePlayerInput` (`self.inputComp`) "AttackNinjutsuStart" (0.0 0.0) (`|GetInputActionValue`)))
  (:`Completed`
    (`PlayerInputComponent.HandlePlayerInput` (`self.inputComp`) "AttackNinjutsuComplete" (0.0 0.0) (`|GetInputActionValue`))))

(event `Key|B`
  (params (Key :type "Key Structure"))
  ;[0 1 0 0.5] Debug Testing
  (:`Pressed`
    (`self.TestDistanceFwd`)))

(event `EnhancedInput|/Game/Hack-N-Slash/Player/Input/IA_LookStick_HNS`
  (params (ActionValue :type "Vector2D Structure") (ElapsedSeconds :type "Float (double-precision)") (TriggeredSeconds :type "Float (double-precision)") (InputAction :type "InputAction Object Reference" :default "/Game/Hack-N-Slash/Player/Input/IA_LookStick_HNS.IA_LookStick_HNS"))
  ;[1 1 1 0.5] Look/Lock On
  (:`Triggered`
    (`PlayerInputComponent.HandlePlayerInput` (`self.inputComp`) "LookStickTrigger" ActionValue (0.0 0.0))))

(event `Key|N`
  (params (Key :type "Key Structure"))
  ;[0 1 0 0.5] Debug Testing
  (:`Pressed`
    (`self.TestDistanceUp`)))

(event `EnhancedInput|/Game/Hack-N-Slash/Player/Input/IA_SwitchTargetRight`
  (params (ActionValue :type Boolean) (ElapsedSeconds :type "Float (double-precision)") (TriggeredSeconds :type "Float (double-precision)") (InputAction :type "InputAction Object Reference" :default "/Game/Hack-N-Slash/Player/Input/IA_SwitchTargetRight.IA_SwitchTargetRight"))
  ;[1 1 1 0.5] Look/Lock On
  (:`Started`
    (`PlayerInputComponent.HandlePlayerInput` (`self.inputComp`) "SwitchTargetRightStart" (0.0 0.0) (0.0 0.0))))

(event `EnhancedInput|/Game/Hack-N-Slash/Player/Input/IA_ToggleLockOn`
  (params (ActionValue :type Boolean) (ElapsedSeconds :type "Float (double-precision)") (TriggeredSeconds :type "Float (double-precision)") (InputAction :type "InputAction Object Reference" :default "/Game/Hack-N-Slash/Player/Input/IA_ToggleLockOn.IA_ToggleLockOn"))
  ;[1 1 1 0.5] Look/Lock On
  (:`Started`
    (`PlayerInputComponent.HandlePlayerInput` (`self.inputComp`) "LockOnOffStart" (0.0 0.0) (0.0 0.0))))

(event `Key|O`
  (params (Key :type "Key Structure"))
  ;[0 1 0 0.5] Debug Testing
)

(event `Key|P`
  (params (Key :type "Key Structure"))
  ;[0 1 0 0.5] Debug Testing
)

(event `EnhancedInput|/Game/Input/Actions/IA_Move`
  (params (ActionValue :type "Vector2D Structure") (ElapsedSeconds :type "Float (double-precision)") (TriggeredSeconds :type "Float (double-precision)") (InputAction :type "InputAction Object Reference" :default "/Game/Input/Actions/IA_Move.IA_Move"))
  ;[1 1 1 0.5] Locomotion
  (:`Triggered`
    (`PlayerInputComponent.HandlePlayerInput` (`self.inputComp`) "MoveTrigger" (0.0 0.0) ActionValue)))

(event `EnhancedInput|/Game/Hack-N-Slash/Player/Input/IA_ChakraNatureBase`
  (params (ActionValue :type Boolean) (ElapsedSeconds :type "Float (double-precision)") (TriggeredSeconds :type "Float (double-precision)") (InputAction :type "InputAction Object Reference" :default "/Game/Hack-N-Slash/Player/Input/IA_ChakraNatureBase.IA_ChakraNatureBase"))
  ;[1 1 1 0.5] Chakra
  (:`Started`
    (`PlayerCombatComponent.ChangeChakraNature` (`self.combatComp`) "None")))

(event `EnhancedInput|/Game/Hack-N-Slash/Player/Input/IA_RegenChakra`
  (params (ActionValue :type Boolean) (ElapsedSeconds :type "Float (double-precision)") (TriggeredSeconds :type "Float (double-precision)") (InputAction :type "InputAction Object Reference" :default "/Game/Hack-N-Slash/Player/Input/IA_RegenChakra.IA_RegenChakra"))
  ;[1 1 1 0.5] Chakra
  (:`Triggered`
    (`PlayerInputComponent.HandlePlayerInput` (`self.inputComp`) "RegenChakraTrigger" (0.0 0.0) (0.0 0.0)))
  (:`Completed`
    (`PlayerInputComponent.HandlePlayerInput` (`self.inputComp`) "RegenChakraComplete" (0.0 0.0) (0.0 0.0))))

(event `EnhancedInput|/Game/Hack-N-Slash/Player/Input/IA_ChakraNatureAir`
  (params (ActionValue :type Boolean) (ElapsedSeconds :type "Float (double-precision)") (TriggeredSeconds :type "Float (double-precision)") (InputAction :type "InputAction Object Reference" :default "/Game/Hack-N-Slash/Player/Input/IA_ChakraNatureAir.IA_ChakraNatureAir"))
  ;[1 1 1 0.5] Chakra
  (:`Started`
    (`PlayerCombatComponent.ChangeChakraNature` (`self.combatComp`) "Wind")))

(event `EnhancedInput|/Game/Hack-N-Slash/Player/Input/IA_Dodge`
  (params (ActionValue :type Boolean) (ElapsedSeconds :type "Float (double-precision)") (TriggeredSeconds :type "Float (double-precision)") (InputAction :type "InputAction Object Reference" :default "/Game/Hack-N-Slash/Player/Input/IA_Dodge.IA_Dodge"))
  ;[1 1 1 0.5] Block/Dodge
  (:`Started`
    (`PlayerInputComponent.HandlePlayerInput` (`self.inputComp`) "DodgeStart" (0.0 0.0) (`|GetInputActionValue`))))

(event `EnhancedInput|/Game/Hack-N-Slash/Player/Input/IA_Block`
  (params (ActionValue :type Boolean) (ElapsedSeconds :type "Float (double-precision)") (TriggeredSeconds :type "Float (double-precision)") (InputAction :type "InputAction Object Reference" :default "/Game/Hack-N-Slash/Player/Input/IA_Block.IA_Block"))
  ;[1 1 1 0.5] Block/Dodge
  (:`Triggered`
    (`PlayerInputComponent.HandlePlayerInput` (`self.inputComp`) "BlockTrigger" (0.0 0.0) (0.0 0.0)))
  (:`Started`
    (`PlayerInputComponent.HandlePlayerInput` (`self.inputComp`) "BlockStart" (0.0 0.0) (0.0 0.0)))
  (:`Completed`
    (`PlayerInputComponent.HandlePlayerInput` (`self.inputComp`) "BlockComplete" (0.0 0.0) (0.0 0.0))))

(event `EnhancedInput|/Game/Hack-N-Slash/Player/Input/IA_BlockDodge`
  (params (ActionValue :type Boolean) (ElapsedSeconds :type "Float (double-precision)") (TriggeredSeconds :type "Float (double-precision)") (InputAction :type "InputAction Object Reference" :default "/Game/Hack-N-Slash/Player/Input/IA_BlockDodge.IA_BlockDodge"))
  ;[1 1 1 0.5] Block/Dodge
  (:`Triggered`
    (`PlayerInputComponent.HandlePlayerInput` (`self.inputComp`) "BlockDodgeTrigger" (0.0 0.0) (`|GetInputActionValue`)))
  (:`Started`
    (`PlayerInputComponent.HandlePlayerInput` (`self.inputComp`) "BlockDodgeStart" (0.0 0.0) (`|GetInputActionValue`)))
  (:`Completed`
    (`PlayerInputComponent.HandlePlayerInput` (`self.inputComp`) "BlockDodgeComplete" (0.0 0.0) (`|GetInputActionValue`))))

(event `EnhancedInput|/Game/Input/Actions/IA_Jump`
  (params (ActionValue :type Boolean) (ElapsedSeconds :type "Float (double-precision)") (TriggeredSeconds :type "Float (double-precision)") (InputAction :type "InputAction Object Reference" :default "/Game/Input/Actions/IA_Jump.IA_Jump"))
  (bind _inputcomp (`self.inputComp`))
  ;[1 1 1 0.5] Locomotion
  (:`Started`
    (`PlayerInputComponent.HandlePlayerInput` _inputcomp "JumpStart" (0.0 0.0) (0.0 0.0)))
  (:`Canceled`
    (`PlayerInputComponent.HandlePlayerInput` _inputcomp "JumpComplete" (0.0 0.0) (0.0 0.0) :!label _label))
  (:`Completed`
    (goto _label)))

(event `EnhancedInput|/Game/Hack-N-Slash/Player/Input/IA_ChakraNatureLightning`
  (params (ActionValue :type Boolean) (ElapsedSeconds :type "Float (double-precision)") (TriggeredSeconds :type "Float (double-precision)") (InputAction :type "InputAction Object Reference" :default "/Game/Hack-N-Slash/Player/Input/IA_ChakraNatureLightning.IA_ChakraNatureLightning"))
  ;[1 1 1 0.5] Chakra
  (:`Started`
    (`PlayerCombatComponent.ChangeChakraNature` (`self.combatComp`) "Lightning")))

(event `On Hit Combat`
  (params (`Hit Data` :type "AtkHitData Structure"))
  ;[1 0 0 0.5] Receive Hit
  (switch `EHitReaction` (`.resolvedReaction` (break `AtkHitData` `Hit Data`))
    (:`NoReact`
      (`self.On Hit Standard` `Hit Data` :!label _label))
    (:`Air`
      (goto _label))
    (:`BlockBreak`
      (`self.On Block Break` `Hit Data`))
    (:`BlockHit`
      (`self.On Block` `Hit Data`))
    (:`BlockPerfect`
      (`self.On Block Perfect` `Hit Data`))
    (:`BounceGround`
      (goto _label))
    (:`BounceWall`
      (goto _label))
    (:`Countered`
      (goto _label))
    (:`LaunchDown`
      (goto _label))
    (:`LaunchFwdHard`
      (goto _label))
    (:`LaunchFwdSoftBack`
      (goto _label))
    (:`LaunchFwdSoftFront`
      (goto _label))
    (:`LaunchUp`
      (goto _label))
    (:`StaggerBack`
      (goto _label))
    (:`StaggerDownFront1`
      (goto _label))
    (:`StaggerDownFront2`
      (goto _label))
    (:`StaggerDownFront3`
      (goto _label))
    (:`StaggerUpFront1`
      (goto _label))
    (:`StaggerUpFront2`
      (goto _label))
    (:`StaggerUpFront3`
      (goto _label))
    (:`WallSplat`
      (goto _label))))

(event `self.statsComp.OnHealthUpdate`
  (params (NewPercent :type "Float (single-precision)") (PrevPercent :type "Float (single-precision)"))
  ;[0 1 0 0.5] Health
)

(event `self.statsComp.OnZeroHealth`
  ;[0 1 0 0.5] Health
)

(event `On Block`
  (params (`Hit Data` :type "AtkHitData Structure (by ref)"))
  ;[1 0 0 0.5] Receive Hit
)

(event `self.combatComp.OnChakraModeUpdate`
  ;[0 1 1 0.5] Chakra
  (`PlayerCombatComponent.bChakraMode` (`self.combatComp`)
    (:`then`
      (switch `EChakraNature` (`PlayerCombatComponent.chakraNatureActive` (`self.combatComp`))
        (:`None`
          (`/Game/Hack-N-Slash/Player/VFX/BC_Aura21.Start Aura Effect` (`self.VFX_CM_Base`)))
        (:`Wind`
          (`/Game/Hack-N-Slash/Player/VFX/BC_Aura05.Start Aura Effect` (`self.VFX_CM_Air`)))))
    (:`else`
      (switch `EChakraNature` (`PlayerCombatComponent.chakraNatureActive` (`self.combatComp`))
        (:`None`
          (`/Game/Hack-N-Slash/Player/VFX/BC_Aura21.Stop Aura Effect` (`self.VFX_CM_Base`)))
        (:`Wind`
          (`/Game/Hack-N-Slash/Player/VFX/BC_Aura05.Stop Aura Effect` (`self.VFX_CM_Air`)))))))

(event `On Block Break`
  (params (`Hit Data` :type "AtkHitData Structure (by ref)"))
  ;[1 0 0 0.5] Receive Hit
)

(event `self.combatComp.OnChakraNatureChange`
  (params (NewNature :type "EChakraNature Enum" :default "None"))
  (bind _combatcomp (`self.combatComp`))
  ;[0 1 1 0.5] Chakra
  (switch `EChakraNature` (`PlayerCombatComponent.chakraNaturePrevious` (`self.combatComp`))
    (:`None`
      (`/Game/Hack-N-Slash/Player/VFX/BC_Aura21.Stop Aura Effect` (`self.VFX_CM_Base`)))
    (:`Wind`
      (`/Game/Hack-N-Slash/Player/VFX/BC_Aura05.Stop Aura Effect` (`self.VFX_CM_Air`))))
  (`PlayerCombatComponent.bChakraMode` _combatcomp
    (:`then`
      (switch `EChakraNature` (`PlayerCombatComponent.chakraNatureActive` _combatcomp)
        (:`None`
          (`/Game/Hack-N-Slash/Player/VFX/BC_Aura21.Start Aura Effect` (`self.VFX_CM_Base`)))
        (:`Wind`
          (`/Game/Hack-N-Slash/Player/VFX/BC_Aura05.Start Aura Effect` (`self.VFX_CM_Air`)))))
    (:`else`)))

(event `On Block Perfect`
  (params (`Hit Data` :type "AtkHitData Structure (by ref)"))
  ;[1 0 0 0.5] Receive Hit
)

(event `Atk: Rain Lightning`
  (bind _returnvalue (`self.K2_GetActorLocation`))
  ;[1 0.2502 0] Atk: Rain Lightning
  (bind _outhits (`KismetSystemLibrary.SphereTraceMulti` _returnvalue _returnvalue 3000.0 "TraceTypeQuery3" false (`|MakeArray` self :!type "Actor Object Reference") (select `bool` (`self.Debug?`) :`true` "ForDuration" :!type "EDrawDebugTrace Enum") true (struct :`R` 1.0 :`A` 1.0) (struct :`G` 1.0 :`A` 1.0) 2.0))
  (for _array_element _outhits
    (bind (_bblockinghit _binitialoverlap _time _distance _location _impactpoint _normal _impactnormal _physmat _hitactor) (`GameplayStatics.BreakHitResult` _array_element))
    (if (and _bblockinghit (`BPFL_Combat.IsActorAlive` _hitactor))
      (`|SpawnActorFromClass` "/Game/Hack-N-Slash/Player/AOEs/BP_AOE_LightningStrike.BP_AOE_LightningStrike_C" (`KismetMathLibrary.MakeTransform` (`self.K2_GetActorLocation` _hitactor)) "Undefined" "MultiplyWithRoot" self "TraceTypeQuery3" (`self.Debug?`) 3.0 true 200.0 _hitactor self))))

(event `On Hit Standard`
  (params (`Hit Data` :type "AtkHitData Structure (by ref)"))
  (bind (_attacker _damager _attackmotion _attackreaction _attacktype _barmorbreaker _biscounterfollowup _bisfinalhit _elements _aggrobuildup _dmg _penetration _poise _knockbacktype _velocityonfinishmode _velocityonfinish _clampvelocityonfinish _duration _badditive _localdir _distance _strengthovertime _brestrictspeedtoexpected _gbextrabounceheight _bgbadditive _gbsot _gbcvof _bkilled _dmgdealt _hitimpactnormal _hitimpactpoint _hitloc _hitsfx _hitvfx _hitvfxscale) (break `AtkHitData` `Hit Data`))
  ;[1 0 0 0.5] Receive Hit
  (`GameplayStatics.PlaySoundAtLocation` _hitsfx _hitloc (struct) 1.0 1.0 0.0 null null null null)
  (`NiagaraFunctionLibrary.SpawnSystemAtLocation` _hitvfx _hitimpactpoint (struct) _hitvfxscale))

(event `Dash Start`
  ;[1 0.2502 0] Dodge
  (bind _vfx_dash (`self.VFX_Dash`)
    (:`then`
      (`/Game/Hack-N-Slash/Player/VFX/BC_Aura24.Start Aura Effect` _vfx_dash))
    (:`else`)))

(event `Dash End`
  ;[1 0.2502 0] Dodge
  (bind _vfx_dash (`self.VFX_Dash`)
    (:`then`
      (`/Game/Hack-N-Slash/Player/VFX/BC_Aura24.Stop Aura Effect` _vfx_dash))
    (:`else`)))

(fn `CheckForGroundUnderSelf`
  (params (Distance :type "Float (double-precision)"))
  (returns (OutHit :type "HitResult Structure") (`Hit?` :type Boolean))
  (bind _returnvalue (`self.K2_GetActorLocation`))
  (bind (_outhit _returnvalue_2) (`KismetSystemLibrary.LineTraceSingle` _returnvalue (+ _returnvalue (* (`self.GetActorUpVector`) (`local.Distance`) -1.0)) "TraceTypeQuery1" false (`|MakeArray` self :!type "Actor Object Reference") (select `bool` (`self.Debug?`) :`true` "ForDuration" :!type "EDrawDebugTrace Enum")))
  (return _outhit _returnvalue_2))

(fn `TestDistanceFwd`
  (bind _returnvalue (`self.K2_GetActorLocation`))
  (bind (_outradius _outhalfheight) (`CapsuleComponent.GetUnscaledCapsuleSize` (`self.CapsuleComponent`)))
  (bind _outhits (`KismetSystemLibrary.CapsuleTraceMultiForObjects` _returnvalue (+ _returnvalue (* (`self.GetActorForwardVector`) (`self.DistanceTest`))) _outradius _outhalfheight (`|MakeArray` "ObjectTypeQuery1" "ObjectTypeQuery2" "ObjectTypeQuery5" "ObjectTypeQuery6" :!type "EObjectTypeQuery Enum") false (`|MakeArray` self :!type "Actor Object Reference") "ForDuration" true (struct :`R` 1.0 :`A` 1.0) (struct :`G` 1.0 :`A` 1.0) 3.0))
  (for _array_element _outhits
    (`KismetSystemLibrary.PrintString` (`KismetSystemLibrary.GetDisplayName` (`.HitActor` (`GameplayStatics.BreakHitResult` _array_element))))))

(fn `TestDistanceUp`
  (bind _returnvalue (+ (`self.K2_GetActorLocation`) (* (`self.GetActorUpVector`) (`self.DistanceTest`))))
  (`KismetSystemLibrary.SphereTraceMultiForObjects` _returnvalue _returnvalue 25.0 (`|MakeArray` "ObjectTypeQuery1" "ObjectTypeQuery2" "ObjectTypeQuery5" "ObjectTypeQuery6" :!type "EObjectTypeQuery Enum") false (`|MakeArray` self :!type "Actor Object Reference") "ForDuration" true (struct :`R` 1.0 :`A` 1.0) (struct :`G` 1.0 :`A` 1.0) 3.0))

(fn `UserConstructionScript`)