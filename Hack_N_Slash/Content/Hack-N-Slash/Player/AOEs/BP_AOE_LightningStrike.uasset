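; Lightning strike AOE for the hack-n-slash player that damages overlapped actors.
; On BeginPlay it builds hit data from its owner, damage, penetration and poise, then activates the lightning effect and triggers the AOE.
; A grounded-tag check on the target either moves the strike below it or disables the floor impact and scorch visuals for non-grounded targets.
; Each overlap adds impact point and normal to the hit data before handling damage.
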(event `self.ReceiveBeginPlay`
  (bind (_hit_data_attacker _hit_data_damager _hit_data_attackmotion _hit_data_attackreaction _hit_data_attacktype _hit_data_barmorbreaker _hit_data_biscounterfollowup _hit_data_elements _hit_data_aggrobuildup _hit_data_dmg _hit_data_penetration _hit_data_poise _hit_data_knockbacktype _hit_data_velocityonfinishmode _hit_data_velocityonfinish _hit_data_clampvelocityonfinish _hit_data_duration _hit_data_badditive _hit_data_localdir _hit_data_distance _hit_data_strengthovertime _hit_data_brestrictspeedtoexpected _hit_data_gbextrabounceheight _hit_data_bgbadditive _hit_data_gbsot _hit_data_gbcvof _hit_data_bkilled _hit_data_dmgdealt _hit_data_hitimpactnormal _hit_data_hitimpactpoint _hit_data_hitloc _hit_data_hitsfx _hit_data_hitvfx _hit_data_hitvfxscale _hit_data_resolvedreaction) (break `AtkHitData` (`self.Hit Data`)))
  (`parent.ReceiveBeginPlay`)
  (set `self.Hit Data` (make `AtkHitData` (`self.GetOwner`) null _hit_data_attackmotion _hit_data_attackreaction _hit_data_attacktype _hit_data_barmorbreaker _hit_data_biscounterfollowup _hit_data_elements _hit_data_aggrobuildup (`self.Damage`) (`self.Penetration`) (`self.Poise`) _hit_data_knockbacktype _hit_data_velocityonfinishmode _hit_data_velocityonfinish _hit_data_clampvelocityonfinish _hit_data_duration _hit_data_badditive _hit_data_localdir _hit_data_distance _hit_data_strengthovertime _hit_data_brestrictspeedtoexpected _hit_data_gbextrabounceheight _hit_data_bgbadditive _hit_data_gbsot _hit_data_gbcvof _hit_data_bkilled _hit_data_dmgdealt _hit_data_hitimpactnormal _hit_data_hitimpactpoint _hit_data_hitloc _hit_data_hitsfx _hit_data_hitvfx _hit_data_hitvfxscale _hit_data_resolvedreaction))
  (if (`BPFL_Combat.ActorHasTag` (`self.target`) (struct :`TagName` "State.Movement.Grounded"))
    (`self.MoveBelowTarget`)
    (else
      (`NiagaraComponent.SetVariableBool` (`self.Lightning`) "Activate Floor Impact" false)
      (`NiagaraComponent.SetVariableBool` (`self.Lightning`) "Activate Floor Scorch" false)
      (`NiagaraComponent.SetVariableBool` (`self.Lightning`) "Activate Lightning Floo" false)))
  (`ActorComponent.Activate` (`self.Lightning`) true)
  (`self.Trigger`))

(event `self.OnAOEOverlap`
  (params (Actor :type "Actor Object Reference") (HitResult :type "HitResult Structure (by ref)"))
  (bind (_bblockinghit _binitialoverlap _time _distance _location _impactpoint _normal _impactnormal) (`GameplayStatics.BreakHitResult` HitResult))
  (bind (_hit_data_attacker _hit_data_damager _hit_data_attackmotion _hit_data_attackreaction _hit_data_attacktype _hit_data_barmorbreaker _hit_data_biscounterfollowup _hit_data_elements _hit_data_aggrobuildup _hit_data_dmg _hit_data_penetration _hit_data_poise _hit_data_knockbacktype _hit_data_velocityonfinishmode _hit_data_velocityonfinish _hit_data_clampvelocityonfinish _hit_data_duration _hit_data_badditive _hit_data_localdir _hit_data_distance _hit_data_strengthovertime _hit_data_brestrictspeedtoexpected _hit_data_gbextrabounceheight _hit_data_bgbadditive _hit_data_gbsot _hit_data_gbcvof _hit_data_bkilled _hit_data_dmgdealt _hit_data_hitimpactnormal _hit_data_hitimpactpoint _hit_data_hitloc _hit_data_hitsfx _hit_data_hitvfx _hit_data_hitvfxscale _hit_data_resolvedreaction) (break `AtkHitData` (`self.Hit Data`)))
  (`parent.OnAOEOverlap` Actor HitResult)
  (bind _output_get (set `self.Hit Data` (make `AtkHitData` _hit_data_attacker _hit_data_damager _hit_data_attackmotion _hit_data_attackreaction _hit_data_attacktype _hit_data_barmorbreaker _hit_data_biscounterfollowup _hit_data_elements _hit_data_aggrobuildup _hit_data_dmg _hit_data_penetration _hit_data_poise _hit_data_knockbacktype _hit_data_velocityonfinishmode _hit_data_velocityonfinish _hit_data_clampvelocityonfinish _hit_data_duration _hit_data_badditive _hit_data_localdir _hit_data_distance _hit_data_strengthovertime _hit_data_brestrictspeedtoexpected _hit_data_gbextrabounceheight _hit_data_bgbadditive _hit_data_gbsot _hit_data_gbcvof _hit_data_bkilled _hit_data_dmgdealt _impactnormal _impactpoint (0.0 0.0 0.0) _hit_data_hitsfx _hit_data_hitvfx _hit_data_hitvfxscale _hit_data_resolvedreaction)))
  (`self.HandleDamage` Actor _output_get))

(fn `UserConstructionScript`
  (`parent.UserConstructionScript`))