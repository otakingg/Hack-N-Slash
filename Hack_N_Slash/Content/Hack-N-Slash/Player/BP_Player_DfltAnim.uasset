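; Hack-N-Slash player Blueprint that sets up Enhanced Input and offers a hold-to-slow-time key.
; On BeginPlay, it clears existing mappings on the local player's input subsystem and applies the hack-and-slash mapping context.
; Holding Tab lowers global time dilation for slow motion, and releasing it restores normal speed.
; Attack, block/dodge, jump, move and look input events are empty stubs here.
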(event `self.ReceiveBeginPlay`
  (bind _asplayer_controller (cast `PlayerController` (`self.GetController`)))
  (bind _returnvalue (pcsubsystem `EnhancedInputLocalPlayerSubsystem` _asplayer_controller))
  (`/Engine/EditorBlueprintResources/StandardMacros.IsValid` _returnvalue
    (:`Is Valid`
      (`EnhancedInputSubsystemInterface.ClearAllMappings` _returnvalue)
      (`EnhancedInputSubsystemInterface.AddMappingContext` _returnvalue "/Game/Hack-N-Slash/Input/IMC_HackNSlash.IMC_HackNSlash" 0 (struct)))))

(event `self.ReceiveTick`
  (params (DeltaSeconds :type "Float (single-precision)")))

(event `EnhancedInput|/Game/Hack-N-Slash/Input/IA_AttackHeavy`
  (params (ActionValue :type Boolean) (ElapsedSeconds :type "Float (double-precision)") (TriggeredSeconds :type "Float (double-precision)") (InputAction :type "InputAction Object Reference" :default "/Game/Hack-N-Slash/Input/IA_AttackHeavy.IA_AttackHeavy"))
  ;[1 1 1 0.5] Inputs
)

(event `EnhancedInput|/Game/Hack-N-Slash/Input/IA_AttackLight`
  (params (ActionValue :type Boolean) (ElapsedSeconds :type "Float (double-precision)") (TriggeredSeconds :type "Float (double-precision)") (InputAction :type "InputAction Object Reference" :default "/Game/Hack-N-Slash/Input/IA_AttackLight.IA_AttackLight"))
  ;[1 1 1 0.5] Inputs
)

(event `EnhancedInput|/Game/Hack-N-Slash/Input/IA_BlockDodge`
  (params (ActionValue :type Boolean) (ElapsedSeconds :type "Float (double-precision)") (TriggeredSeconds :type "Float (double-precision)") (InputAction :type "InputAction Object Reference" :default "/Game/Hack-N-Slash/Input/IA_BlockDodge.IA_BlockDodge"))
  ;[1 1 1 0.5] Inputs
)

(event `Key|Tab`
  (params (Key :type "Key Structure"))
  ;[1 1 1 0.5] Inputs
  (:`Pressed`
    (`GameplayStatics.SetGlobalTimeDilation` 0.2))
  (:`Released`
    (`GameplayStatics.SetGlobalTimeDilation` 1.0)))

(event `EnhancedInput|/Game/Input/Actions/IA_Jump`
  (params (ActionValue :type Boolean) (ElapsedSeconds :type "Float (double-precision)") (TriggeredSeconds :type "Float (double-precision)") (InputAction :type "InputAction Object Reference" :default "/Game/Input/Actions/IA_Jump.IA_Jump"))
  ;[1 1 1 0.5] Inputs
)

(event `EnhancedInput|/Game/Hack-N-Slash/Input/IA_LookMouse_HNS`
  (params (ActionValue :type "Vector2D Structure") (ElapsedSeconds :type "Float (double-precision)") (TriggeredSeconds :type "Float (double-precision)") (InputAction :type "InputAction Object Reference" :default "/Game/Hack-N-Slash/Input/IA_LookMouse_HNS.IA_LookMouse_HNS"))
  ;[1 1 1 0.5] Inputs
)

(event `EnhancedInput|/Game/Input/Actions/IA_Move`
  (params (ActionValue :type "Vector2D Structure") (ElapsedSeconds :type "Float (double-precision)") (TriggeredSeconds :type "Float (double-precision)") (InputAction :type "InputAction Object Reference" :default "/Game/Input/Actions/IA_Move.IA_Move"))
  ;[1 1 1 0.5] Inputs
)

(event `EnhancedInput|/Game/Hack-N-Slash/Input/IA_Look_HNS`
  (params (ActionValue :type "Vector2D Structure") (ElapsedSeconds :type "Float (double-precision)") (TriggeredSeconds :type "Float (double-precision)") (InputAction :type "InputAction Object Reference" :default "/Game/Hack-N-Slash/Input/IA_Look_HNS.IA_Look_HNS"))
  ;[1 1 1 0.5] Inputs
)

(fn `UserConstructionScript`)