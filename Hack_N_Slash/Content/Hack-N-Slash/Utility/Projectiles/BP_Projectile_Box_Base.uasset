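; Base projectile Blueprint with box collision that passes hits on to damage handling and plays spawn and destruction effects.
; On BeginPlay it optionally makes the box ignore the owning actor while moving, plays a spawn sound and binds its destroyed event.
; Box hits route through HandleImpact, which only forwards the actor and hit result to HandleDamage.
; Destruction spawns VFX and plays a sound at the projectile's location.
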(event `self.ReceiveBeginPlay`
  (`PrimitiveComponent.IgnoreActorWhenMoving` (`self.Box`) (`self.GetOwner`) (`self.bIgnoreSelf`))
  (`GameplayStatics.PlaySoundAtLocation` (`self.spawnSFX`) (`self.K2_GetActorLocation`) (struct) 1.0 1.0 0.0 null null null null)
  (add `self.OnDestroyed` (`|CreateDelegate` :!event `On Projectile Destroyed`)))

(event `self.Box.OnComponentHit`
  (params (HitComponent :type "PrimitiveComponent Object Reference") (OtherActor :type "Actor Object Reference") (OtherComp :type "PrimitiveComponent Object Reference") (NormalImpulse :type "Vector Structure") (Hit :type "HitResult Structure (by ref)"))
  (`self.HandleImpact` OtherActor Hit))

(event `On Projectile Destroyed` :!signature `self.OnDestroyed`
  (params (DestroyedActor :type "Actor Object Reference"))
  (`NiagaraFunctionLibrary.SpawnSystemAtLocation` (`self.destroyedVFX`) (`self.K2_GetActorLocation`))
  (`GameplayStatics.PlaySoundAtLocation` (`self.destroyedSFX`) (`self.K2_GetActorLocation`) (struct) 1.0 1.0 0.0 null null null null))

(fn `HandleImpact`
  (params (HitActor :type "Actor Object Reference") (`Hit Result` :type "HitResult Structure (by ref)"))
  (locals (`Impact Point` :type "Vector Structure" :default (0.0 0.0 0.0)) (`Impact Normal` :type "Vector Structure" :default (0.0 0.0 0.0)))
  (`self.HandleDamage` HitActor `Hit Result`))

(fn `UserConstructionScript`)