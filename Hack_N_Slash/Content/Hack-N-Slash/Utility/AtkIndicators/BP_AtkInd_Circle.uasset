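; BP_AtkInd_Circle is a circular attack indicator actor that shows an area filling up over a set duration, then removes itself.
; On BeginPlay it creates dynamic materials for its Outer and Inner components, assigning each a color and an outer/inner switch parameter.
; After a short delay, a timeline rescaled to Duration drives the inner material's AreaValue, and the actor destroys itself shortly after it finishes.
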(event `self.ReceiveBeginPlay`
  (`|ExecutionSequence`
    (:`then_0`
      (bind _returnvalue (`DecalComponent.CreateDynamicMaterialInstance` (`self.Outer`)))
      (set `self.OuterRef` _returnvalue)
      (`MaterialInstanceDynamic.SetScalarParameterValue` (`self.OuterRef`) "Outer1Inner0" 1.0)
      (`MaterialInstanceDynamic.SetVectorParameterValue` (`self.OuterRef`) "Color" (`self.Outer Color`)))
    (:`then_1`
      (bind _returnvalue_2 (`DecalComponent.CreateDynamicMaterialInstance` (`self.Inner`)))
      (set `self.InnerRef` _returnvalue_2)
      (`MaterialInstanceDynamic.SetScalarParameterValue` (`self.InnerRef`) "Outer1Inner0" 0.0)
      (`MaterialInstanceDynamic.SetVectorParameterValue` (`self.InnerRef`) "Color" (`self.Inner Color`)))
    (:`then_2`
      (`MaterialInstanceDynamic.SetScalarParameterValue` (`self.InnerRef`) "AreaValue" 0.0)
      (`KismetSystemLibrary.Delay` 1.0)
      (`TimelineComponent.SetPlayRate` (`self.AreaFillOverTime`) (/ (`TimelineComponent.GetTimelineLength` (`self.AreaFillOverTime`)) (`self.Duration`)))
      (bind (_direction _alpha) (`Timeline|AreaFillOverTime` :!via `PlayFromStart`)
        (:`Update`
          (`MaterialInstanceDynamic.SetScalarParameterValue` (`self.InnerRef`) "AreaValue" _alpha))
        (:`Finished`
          (`KismetSystemLibrary.Delay` 0.1)
          (`self.K2_DestroyActor`))))))

(fn `UserConstructionScript`)