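; Circular attack indicator actor that shows an area filling up over a set Duration, then destroys itself.
; On BeginPlay it creates dynamic material instances for the Border, Outer and Inner components, using one material parameter to select border, fill or progress mode, each with its own color.
; A timeline, rate-scaled to Duration, drives the Progress parameter, and the actor destroys itself shortly after it finishes.
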(event `self.ReceiveBeginPlay`
  (`|ExecutionSequence`
    (:`then_0`
      (bind _returnvalue (`DecalComponent.CreateDynamicMaterialInstance` (`self.Border`)))
      (bind _output_get (set `self.Border Ref` _returnvalue))
      (`MaterialInstanceDynamic.SetScalarParameterValue` _output_get "Border1Progress0Fill0.5" 1.0)
      (`MaterialInstanceDynamic.SetVectorParameterValue` (`self.Border Ref`) "Color" (`self.Border Color`))
      (`MaterialInstanceDynamic.SetScalarParameterValue` (`self.Border Ref`) "Intensity" 1.0))
    (:`then_1`
      (bind _returnvalue_2 (`DecalComponent.CreateDynamicMaterialInstance` (`self.Outer`)))
      (bind _output_get_2 (set `self.Fill Ref` _returnvalue_2))
      (`MaterialInstanceDynamic.SetScalarParameterValue` _output_get_2 "Border1Progress0Fill0.5" 0.5)
      (`MaterialInstanceDynamic.SetVectorParameterValue` (`self.Fill Ref`) "Color" (`self.Fill Color`))
      (`MaterialInstanceDynamic.SetScalarParameterValue` (`self.Fill Ref`) "Intensity" 1.0))
    (:`then_2`
      (bind _returnvalue_3 (`DecalComponent.CreateDynamicMaterialInstance` (`self.Inner`)))
      (bind _output_get_3 (set `self.Progress Ref` _returnvalue_3))
      (`MaterialInstanceDynamic.SetScalarParameterValue` _output_get_3 "Border1Progress0Fill0.5" 0.0)
      (`MaterialInstanceDynamic.SetVectorParameterValue` (`self.Progress Ref`) "Color" (`self.Progress Color`))
      (`MaterialInstanceDynamic.SetScalarParameterValue` (`self.Progress Ref`) "Intensity" 1.0))
    (:`then_3`
      (`MaterialInstanceDynamic.SetScalarParameterValue` (`self.Progress Ref`) "Progress" 0.0)
      (`TimelineComponent.SetPlayRate` (`self.AreaFillOverTime`) (/ (`TimelineComponent.GetTimelineLength` (`self.AreaFillOverTime`)) (`self.Duration`)))
      (bind (_direction _alpha) (`Timeline|AreaFillOverTime` :!via `PlayFromStart`)
        (:`Update`
          (`MaterialInstanceDynamic.SetScalarParameterValue` (`self.Progress Ref`) "Progress" _alpha))
        (:`Finished`
          (`KismetSystemLibrary.Delay` 0.1)
          (`self.K2_DestroyActor`))))))

(fn `UserConstructionScript`)