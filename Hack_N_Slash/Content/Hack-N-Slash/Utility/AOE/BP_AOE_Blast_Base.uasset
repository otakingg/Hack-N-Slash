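; Base Blueprint for a blast area-of-effect that damages overlapped actors and destroys itself when its visuals end.
; Both parent AOE spawn events also trigger the blast sound and an attached particle system.
; Overlaps build hit data from instigator, target location, damage and penetration, then pass it to HandleHit.
; The actor is destroyed when the effect finishes, or after a fallback lifespan if none spawns.
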(event `self.SpawnAOE_C`
  (`parent.SpawnAOE_C`)
  (`self.PlaySFX`)
  (`self.PlayVFX`))

(event `self.SpawnAOE_O`
  (`parent.SpawnAOE_O`)
  (`self.PlaySFX`)
  (`self.PlayVFX`))

(event `PlaySFX`
  (`GameplayStatics.PlaySoundAtLocation` (`self.BlastSFX`) (`self.K2_GetActorLocation`) (struct) 1.0 1.0 0.0 null null null null))

(event `PlayVFX`
  (bind _blastvfx (`self.BlastVFX`)
    (:`then`
      (bind _returnvalue (`NiagaraFunctionLibrary.SpawnSystemAttached` _blastvfx (`self.DefaultSceneRoot`) "None" (0.0 0.0 0.0) (struct) "KeepRelativeOffset" true))
      (`/Engine/EditorBlueprintResources/StandardMacros.IsValid` _returnvalue
        (:`Is Valid`
          (add `NiagaraComponent.OnSystemFinished` _returnvalue (delegate `OnSystemFinished_Event`)))
        (:`Is Not Valid`
          (`KismetSystemLibrary.Delay` (`self.FallbackLifeSpan`))
          (`self.K2_DestroyActor`))))
    (:`else`
      (`KismetSystemLibrary.Delay` (`self.FallbackLifeSpan`))
      (`self.K2_DestroyActor`))))

(event `OnSystemFinished_Event`
  (params (PSystem :type "NiagaraComponent Object Reference"))
  (`self.K2_DestroyActor`))

(event `self.OnAOEOverlap`
  (params (Actor :type "Actor Object Reference"))
  (`parent.OnAOEOverlap` Actor)
  (`/Engine/EditorBlueprintResources/StandardMacros.IsValid` Actor
    (:`Is Valid`
      (bind _output_get (set `self.AtkHitData` (make `AtkHitData` (`self.GetInstigator`) (`self.K2_GetActorLocation` Actor) (`self.Damage`) (`self.Penetration`))))
      (`self.HandleHit` _output_get Actor))))

(fn `UserConstructionScript`
  (`parent.UserConstructionScript`))