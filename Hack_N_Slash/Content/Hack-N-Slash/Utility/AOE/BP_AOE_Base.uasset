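; BP_AOE_Base is a base area-of-effect Blueprint for the Hack-N-Slash utilities.
; Trigger calls SpawnAOE, which sphere-traces at the actor's location, optionally ignoring the instigator, and passes each hit to OnAOEOverlap.
; OnAOEOverlap only prints debug names here, with no gameplay effect.
; MoveBelowTarget teleports the actor to a line-trace hit from Target, whose end point multiplies Target's Z by -5000 rather than offsetting it.
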(event `self.ReceiveBeginPlay`)

(event `MoveBelowTarget`
  (bind _target (`self.target`)
    (:`then`
      (bind _returnvalue (`self.K2_GetActorLocation` _target))
      (bind (_outhit _returnvalue_2) (`KismetSystemLibrary.LineTraceSingle` _returnvalue (* _returnvalue (1.0 1.0 -5000.0)) "TraceTypeQuery1" false (`|MakeArray` _target self :!type "Actor Object Reference") (select `bool` (`self.bDebug`) :`true` "ForDuration" :!type "EDrawDebugTrace Enum") true (struct :`R` 1.0 :`A` 1.0) (struct :`G` 1.0 :`A` 1.0) 3.0))
      (if _returnvalue_2
        (`self.K2_SetActorLocation` (`.Location` (`GameplayStatics.BreakHitResult` _outhit)) false true)))
    (:`else`)))

(event `Trigger`
  (`self.SpawnAOE`))

(event `SpawnAOE`
  (bind _outhits (`KismetSystemLibrary.SphereTraceMulti` (`self.K2_GetActorLocation`) (`self.K2_GetActorLocation`) (`self.radius`) (`self.TraceChannel`) false (select `bool` (`self.bIgnoreSelf`) :`false` (`|MakeArray` self :!type "Actor Object Reference") :`true` (`|MakeArray` self (`self.GetInstigator`) :!type "Actor Object Reference")) (select `bool` (`self.bDebug`) :`true` "ForDuration" :!type "EDrawDebugTrace Enum") true (struct :`R` 1.0 :`A` 1.0) (struct :`G` 1.0 :`A` 1.0) 0.1))
  (for _array_element _outhits
    (`self.OnAOEOverlap` (`.HitActor` (`GameplayStatics.BreakHitResult` _array_element)) _array_element)))

(event `self.OnAOEOverlap`
  (params (Actor :type "Actor Object Reference") (HitResult :type "HitResult Structure (by ref)"))
  (`self.bDebug`
    (:`then`
      (`/Engine/EditorBlueprintResources/StandardMacros.IsValid` Actor
        (:`Is Valid`
          (`KismetSystemLibrary.PrintString` (`KismetStringLibrary.Concat_StrStr` " OnOverlapAOE: " (`KismetSystemLibrary.GetDisplayName` Actor))))))
    (:`else`)))

(fn `UserConstructionScript`)