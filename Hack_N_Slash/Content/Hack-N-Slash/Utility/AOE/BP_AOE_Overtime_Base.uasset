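; BP_AOE_Overtime_Base is a base Blueprint for area-of-effect actors that act over time, with Trigger as the extension point for VFX and SFX.
; Trigger starts a looping timer at SpawnInterval and, when Duration is positive, a second one-shot timer for that Duration.
; The events bound to both timers are not defined in this graph, and BeginPlay is disabled.
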(event `self.Trigger`
  ;[1 1 1 0.5] Extend this if you want to spawn VFX, SFX, etc.
  (`KismetSystemLibrary.K2_SetTimerDelegate` (`|CreateDelegate` :!event `SpawnAOE`) (`self.SpawnInterval`) true)
  (if (> (`self.Duration`) 0.0)
    (`KismetSystemLibrary.K2_SetTimerDelegate` (`|CreateDelegate` :!event `K2_DestroyActor`) (`self.Duration`))))

(fn `UserConstructionScript`
  (`parent.UserConstructionScript`))