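; BP_AOE_Dmg_Base is a base actor for area-of-effect damage centered on its own location.
; SpawnAOESphereC uses a multi-sphere channel trace, while SpawnAOESphereO uses an object-type sphere overlap, both sized by Radius.
; Each actor found goes through OnAOEOverlap to HandleDamage, whose body is not in this graph.
; IgnoreSelf excludes the instigator, and Debug controls sphere drawing.
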(event `SpawnAOESphereC`
  (bind _outhits (`KismetSystemLibrary.SphereTraceMulti` (`self.K2_GetActorLocation`) (`self.K2_GetActorLocation`) (`self.Radius`) "TraceTypeQuery3" false (select `bool` (`self.IgnoreSelf?`) :`false` (`|MakeArray` null :!type "Actor Object Reference") :`true` (`|MakeArray` (`self.GetInstigator`) :!type "Actor Object Reference")) (select `bool` (`self.Debug?`) :`true` "ForDuration" :!type "EDrawDebugTrace Enum") true (struct :`R` 1.0 :`A` 1.0) (struct :`G` 1.0 :`A` 1.0) 3.0))
  (for _array_element _outhits
    (`self.OnAOEOverlap` (`.HitActor` (`GameplayStatics.BreakHitResult` _array_element)))))

(event `SpawnAOESphereO`
  (`self.Debug?`
    (:`then`
      (`KismetSystemLibrary.DrawDebugSphere` (`self.K2_GetActorLocation`) (`self.Radius`) 12 (struct :`R` 1.0 :`G` 0.83353 :`A` 1.0) 3.0 5.0))
    (:`else`
      _))
  (bind _outactors (`KismetSystemLibrary.SphereOverlapActors` (`self.K2_GetActorLocation`) (`self.Radius`) (`self.ObjectTypes`) null (select `bool` (`self.IgnoreSelf?`) :`false` (`|MakeArray` null :!type "Actor Object Reference") :`true` (`|MakeArray` (`self.GetInstigator`) :!type "Actor Object Reference"))))
  (for _array_element _outactors
    (`self.OnAOEOverlap` _array_element)))

(event `self.OnAOEOverlap`
  (params (actor :type "Actor Object Reference"))
  (`self.HandleDamage` actor))

(fn `UserConstructionScript`)