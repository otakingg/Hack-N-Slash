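; Patrol route Blueprint that exposes the points of a Route spline as world-space waypoints.
; GetSplinePointAsWorldLocation returns the location of the spline point at the current Index.
; IncrementPatrolIndex sets up ping-pong traversal, turning Direction negative when Index plus Direction hits the last point and positive when Index is zero.
; Despite its name, IncrementPatrolIndex shows no write to Index itself, only to Direction.
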(fn `GetSplinePointAsWorldLocation`
  (returns (PatrolPoint :type "Vector Structure"))
  (return (`SplineComponent.GetLocationAtSplinePoint` (`self.Route`) (`self.index`) "World")))

(fn `IncrementPatrolIndex`
  (if (== (+ (`self.index`) (`self.direction`)) (- (`SplineComponent.GetNumberOfSplinePoints` (`self.Route`)) 1))
    (set `self.direction` -1)
    (elif (== (`self.index`) 0)
      (set `self.direction` 1))))

(fn `UserConstructionScript`)